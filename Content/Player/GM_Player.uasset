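; Game mode that manages player login, character creation, persistence and disconnection in multiplayer.
; PostLogin spawns a hidden BP_Character, kicks duplicate names, then restores saved data and local UI/control settings, or opens character creation.
; New characters start from DT_Entities "human" defaults; all share one name-keyed SG_SAVE slot, with writes guarded by a lock flag.
; When the host disconnects, other players are saved and kicked before the host.
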(event `DisconnectHost`
  (params (Host :type "/Game/Player/PC_Player Object Reference"))
  (bind _mycharacter (`/Game/Player/PC_Player.MyCharacter` Host))
  (bind _outactors (`GameplayStatics.GetAllActorsOfClass` "/Game/Player/PC_Player.PC_Player_C"))
  (for _array_element _outactors
    (bind _mycharacter_2 (`/Game/Player/PC_Player.MyCharacter` _array_element))
    (if (not (`KismetStringLibrary.EqualEqual_StrStr` (`/Game/Player/BP_Character.Player Name` _mycharacter_2) (`/Game/Player/BP_Character.Player Name` _mycharacter)))
      (`self.SavePlayer` _mycharacter_2)
      (`self.DisconnectPlayer` _array_element)))
  (`self.SavePlayer` _mycharacter)
  (`self.DisconnectPlayer` Host))

(event `DisconnectPlayer`
  (params (Controller :type "PlayerController Object Reference"))
  (bind _aspc_player (cast `/Game/Player/PC_Player` Controller))
  (`BlueprintSetLibrary.Set_Remove` (`self.Current Players`) (`KismetStringLibrary.Conv_StringToName` (`/Game/Player/BP_Character.Player Name` (`/Game/Player/PC_Player.MyCharacter` _aspc_player))))
  (`/Game/Player/PC_Player.CLIENT_SaveLocalSettings` _aspc_player)
  (`AdvancedSessionsLibrary.KickPlayer` Controller))

(event `CreatePlayer`
  (params (Data :type "/Game/Blueprints/SaveLoad/Components/S_SAVE_BODY_PARTS_COMP Structure") (Controller :type "PlayerController Object Reference (by ref)"))
  (bind _slot_name (`self.Slot Name`))
  (bind _aspc_player (cast `/Game/Player/PC_Player` Controller))
  (bind _asbp_character (cast `/Game/Player/BP_Character` (`Controller.K2_GetPawn` Controller)))
  (bind _slot (`self.GetLockedSlot` _slot_name)
    (:`SlotFound`
      (set `self.is_slot_locked` true)
      (bind _assg_save (cast `/Game/Blueprints/SaveLoad/SG_SAVE` _slot))
      (bind _result (`self.PutStartCharacterToSlot` Data _asbp_character _assg_save (`/Game/Player/BP_Character.Player Name` _asbp_character)))
      (`GameplayStatics.SaveGameToSlot` _result _slot_name)
      (set `self.is_slot_locked` false)
      (`WidgetBlueprintLibrary.SetInputMode_GameOnly` Controller)
      (set `PlayerController.bShowMouseCursor` false Controller)
      (`self.LoadPlayer` _aspc_player)
      (`/Game/Player/BP_Character.RemoveStartRoom` _asbp_character))))

(event `LoadPlayerLocal`
  (params (Character :type "/Game/Player/BP_Character Object Reference") (Data :type "/Game/Blueprints/SaveLoad/S_SAVE_PLAYER Structure"))
  (bind _ac_uimanager (`/Game/Player/BP_Character.AC_UIManager` Character))
  (`/Game/UI/AC_UIManager.Init` _ac_uimanager)
  (`KismetSystemLibrary.Delay` 0.1)
  (bind _returnvalue (`GameplayStatics.DoesSaveGameExist` "PLAYER_LOCAL"))
  (if _returnvalue
    (bind _returnvalue_2 (`GameplayStatics.LoadGameFromSlot` "PLAYER_LOCAL"))
    (bind _assg_local_settings (cast `/Game/Blueprints/SaveLoad/SG_LocalSettings` _returnvalue_2))
    (`/Game/Blueprints/SaveLoad/BFL_SaveLoad.LoadUI` (`/Game/Blueprints/SaveLoad/SG_LocalSettings.UI` _assg_local_settings) _ac_uimanager)
    (`/Game/Blueprints/SaveLoad/BFL_SaveLoad.LoadControls` (`/Game/Blueprints/SaveLoad/SG_LocalSettings.Controls` _assg_local_settings) Character)
    (else
      (bind _returnvalue_3 (`GameplayStatics.CreateSaveGameObject` "/Game/Blueprints/SaveLoad/SG_LocalSettings.SG_LocalSettings_C"))
      (`GameplayStatics.SaveGameToSlot` _returnvalue_3 "PLAYER_LOCAL")))
  (`/Game/UI/AC_UIManager.UpdateUI` _ac_uimanager "NewEnumerator2"))

(event `LoadPlayer`
  (params (Controller :type "Controller Object Reference"))
  (`KismetSystemLibrary.Delay` 0.1)
  (bind _aspc_player (cast `/Game/Player/PC_Player` Controller))
  (bind _asbp_character (cast `/Game/Player/BP_Character` (`Controller.K2_GetPawn` Controller)))
  (bind _returnvalue (`GameplayStatics.LoadGameFromSlot` (`self.Slot Name`)))
  (bind _assg_save (cast `/Game/Blueprints/SaveLoad/SG_SAVE` _returnvalue))
  (bind (_value _returnvalue_2) (`BlueprintMapLibrary.Map_Find` (`/Game/Blueprints/SaveLoad/SG_SAVE.Players` _assg_save) (`KismetStringLibrary.Conv_StringToName` (`/Game/Player/BP_Character.Player Name` _asbp_character))))
  (if _returnvalue_2
    (bind _asbp_character_2 (cast `/Game/Player/BP_Character` (`Controller.K2_GetPawn` Controller)))
    (`/Game/Blueprints/SaveLoad/BFL_SaveLoad.LoadPlayer` _asbp_character_2 _value)
    (`self.LoadPlayerLocal` _asbp_character_2 _value)
    (`KismetSystemLibrary.Delay` 0.2)
    (`/Game/Blueprints/StorageSystem/AC_BaseStorage.SERVER_UpdateData` (`/Game/Player/BP_Character.AC_ItemStorage` _asbp_character_2))
    (`/Game/Blueprints/StorageSystem/Panel/AC_Panel.SERVER_UpdatePanel` (`/Game/Player/BP_Character.AC_Panel` _asbp_character_2))
    (bind _ac_bodypart (`/Game/Player/BP_Character.AC_BodyPart` _asbp_character_2))
    (`/Game/Blueprints/Animations/AC_BodyPart.SERVER_UpdateData` _ac_bodypart)
    (`/Game/Blueprints/StorageSystem/AC_BaseStorage.SERVER_UpdateData` (`/Game/Player/BP_Character.AC_Equipment` _asbp_character_2))
    (`/Game/Blueprints/Animations/AC_BodyPart.SetEmotion` _ac_bodypart "NewEnumerator0" "NewEnumerator0" "NewEnumerator0")
    (bind _ac_skills (`/Game/Player/BP_Character.AC_Skills` _asbp_character_2))
    (bind _keypin (`|MapForEach` (`/Game/Blueprints/SkillSystem/AC_SkillComponent.AttributeSet` _ac_skills))
      (:`then`
        (`/Game/Blueprints/SkillSystem/AC_SkillComponent.ReCalculateAttribute` _ac_skills _keypin))
      (:`CompletedPin`
        (`self.SetActorHiddenInGame` _asbp_character_2 false)
        (`KismetSystemLibrary.Delay` 0.1)
        (set `/Game/Player/PC_Player.isLocked` false _aspc_player)
        (`/Game/Player/PC_Player.CLIENT_StartPlay` _aspc_player)))
    (else
      (`self.PrepareToCreateCharacter` _aspc_player))))

(event `self.K2_PostLogin`
  (params (NewPlayer :type "PlayerController Object Reference"))
  (bind _current_players (`self.Current Players`))
  (bind _returnvalue (`GameplayStatics.GetCurrentLevelName` true))
  (if (not (`KismetStringLibrary.EqualEqual_StrStr` _returnvalue "Test"))
    (bind _aspc_player (cast `/Game/Player/PC_Player` NewPlayer))
    (set `/Game/Player/PC_Player.isLocked` true _aspc_player)
    (bind _returnvalue_2 (`|SpawnActorFromClass` "/Game/Player/BP_Character.BP_Character_C" (`KismetMathLibrary.MakeTransform` (0.0 0.0 50.0)) "Undefined" "MultiplyWithRoot" null null))
    (`/Game/Player/BP_Character.SetupLocal` _returnvalue_2)
    (`Controller.Possess` NewPlayer _returnvalue_2)
    (set `/Game/Player/PC_Player.MyCharacter` _returnvalue_2 _aspc_player)
    (`self.SetActorHiddenInGame` _returnvalue_2 true)
    (`KismetSystemLibrary.Delay` 0.5)
    (bind _returnvalue_3 (`KismetStringLibrary.Conv_StringToName` (`/Game/Player/BP_Character.Player Name` _returnvalue_2)))
    (if (`BlueprintSetLibrary.Set_Contains` _current_players _returnvalue_3)
      (`AdvancedSessionsLibrary.KickPlayer` NewPlayer)
      (else
        (`BlueprintSetLibrary.Set_Add` _current_players _returnvalue_3)
        (`self.LoadPlayer` NewPlayer)))))

(event `SavePlayer`
  (params (Character :type "/Game/Player/BP_Character Object Reference"))
  (bind _slot (`self.GetLockedSlot` (`self.Slot Name`))
    (:`SlotFound`
      (set `self.is_slot_locked` true)
      (bind _assg_save (cast `/Game/Blueprints/SaveLoad/SG_SAVE` _slot))
      (bind _slotresult (`self.SavePlayerToSlot` Character _assg_save))
      (`GameplayStatics.SaveGameToSlot` _slotresult (`self.Slot Name`))
      (set `self.is_slot_locked` false))))

(event `self.K2_OnSetMatchState`
  (params (NewState :type Name))
  (bind _asgi_main (cast `/Game/Player/GI_Main` (`GameplayStatics.GetGameInstance`)))
  (`/Engine/EditorBlueprintResources/StandardMacros.DoOnce` false
    (:`Completed`
      (bind _slotname (`/Game/Player/GI_Main.SlotName` _asgi_main))
      (set `self.Slot Name` _slotname)
      (`KismetSystemLibrary.PrintString` (`KismetStringLibrary.Concat_StrStr` "SET GAME NAME " _slotname)))))

(fn `PrepareToCreateCharacter`
  (params (Controller :type "/Game/Player/PC_Player Object Reference"))
  (locals (Location :type "Vector Structure"))
  (bind _mycharacter (`/Game/Player/PC_Player.MyCharacter` Controller))
  (`self.SetActorHiddenInGame` _mycharacter false)
  (`/Game/Player/BP_Character.CreateStartRoom` _mycharacter)
  (`/Game/Blueprints/StorageSystem/Panel/AC_Panel.InitPanels` (`/Game/Player/BP_Character.AC_Panel` _mycharacter) 1 0)
  (bind _returnvalue (`|GetDataTableRow` "/Game/Data/Enitites/DT_Entities.DT_Entities" "human")
    (:`then`
      (`/Game/Blueprints/SkillSystem/BFL_SkillsHelper.SetSkillComp` (make `/Game/Data/Enitites/S_SkillCompData` (break `/Game/Data/Enitites/S_SkillCompData` (`.SkillCompData_62_FAE5C04747C2625E7987C386D8520124` (break `/Game/Data/Enitites/S_Entity` _returnvalue))) (`.Effect_9_FA60C20A41CB932F3BB127845D8F9E6A` (break `/Game/Data/Enitites/S_SkillCompData` (`.SkillCompData_62_FAE5C04747C2625E7987C386D8520124` (break `/Game/Data/Enitites/S_Entity` _returnvalue)))) (`.Buffs_12_E745184945F56A1901C01199CF87EE8E` (break `/Game/Data/Enitites/S_SkillCompData` (`.SkillCompData_62_FAE5C04747C2625E7987C386D8520124` (break `/Game/Data/Enitites/S_Entity` _returnvalue)))) (`.Bars_16_726B218742F45B2D872226BA9FE6E750` (break `/Game/Data/Enitites/S_SkillCompData` (`.SkillCompData_62_FAE5C04747C2625E7987C386D8520124` (break `/Game/Data/Enitites/S_Entity` _returnvalue))))) (`/Game/Player/BP_Character.AC_Skills` _mycharacter)))))

(fn `PutStartCharacterToSlot`
  (params (BodyDAta :type "/Game/Blueprints/SaveLoad/Components/S_SAVE_BODY_PARTS_COMP Structure") (Character :type "/Game/Player/BP_Character Object Reference (by ref)") (Slot :type "/Game/Blueprints/SaveLoad/SG_SAVE Object Reference") (name :type String))
  (returns (Result :type "/Game/Blueprints/SaveLoad/SG_SAVE Object Reference"))
  (locals (NewPlayerData :type "/Game/Blueprints/SaveLoad/S_SAVE_PLAYER Structure") (Attributes :type "Map of GameplayTag Structure to Float (double-precision)") (EmptyInventory :type "Array of /Game/Blueprints/SaveLoad/Base/S_SAVE_DATA_ITEM Structure") (SlotBase :type "/Game/Blueprints/SaveLoad/SG_SAVE Object Reference") (Players :type "Map of Name to /Game/Blueprints/SaveLoad/S_SAVE_PLAYER Structure") (EmptyPanel :type "Array of /Game/Blueprints/SaveLoad/Base/S_SAVE_DATA_ITEM Structure"))
  (bind _returnvalue (`KismetStringLibrary.Conv_StringToName` name))
  (bind _slotbase (`local.SlotBase`))
  (set `local.SlotBase` Slot)
  (bind _returnvalue_2 (`|GetDataTableRow` "/Game/Data/Enitites/DT_Entities.DT_Entities" "human")
    (:`then`
      (bind (_keypin _valuepin) (`|MapForEach` (break `/Game/Data/Enitites/S_SkillCompData` (`.SkillCompData_62_FAE5C04747C2625E7987C386D8520124` (break `/Game/Data/Enitites/S_Entity` _returnvalue_2))))
        (:`then`
          (`BlueprintMapLibrary.Map_Add` (`local.Attributes`) _keypin (`.Base_27_6D5926F0445AB5B78ECF7D85052FB2B0` (break `/Game/Blueprints/SkillSystem/S_Attribute` _valuepin))))
        (:`CompletedPin`
          (bind _result (`/Game/Blueprints/SaveLoad/BFL_SaveLoad.SavePlayer` Character))
          (for _ (range 1 41)
            (`KismetArrayLibrary.Array_Add` (`local.EmptyInventory`) (make `/Game/Blueprints/SaveLoad/Base/S_SAVE_DATA_ITEM` "air")))
          (for _ (range 1 11)
            (`KismetArrayLibrary.Array_Add` (`local.EmptyPanel`) (make `/Game/Blueprints/SaveLoad/Base/S_SAVE_DATA_ITEM` "air")))
          (bind _output_get (set `local.NewPlayerData` (make `/Game/Blueprints/SaveLoad/S_SAVE_PLAYER` _returnvalue (make `/Game/Blueprints/SaveLoad/Components/S_SAVE_SKILL_COMP` (`local.Attributes`)) (`.Equip_14_E9B699BB4B5AEF8FFD0F65923AA6C0F5` (break `/Game/Blueprints/SaveLoad/S_SAVE_PLAYER` _result)) (struct :`OwnedSkills` (struct :`(TagName` "TagName"))) (make `/Game/Blueprints/SaveLoad/Components/S_SAVE_STORAGE_COMP` (`local.EmptyInventory`)) (make `/Game/Blueprints/SaveLoad/Components/S_SAVE_PANEL_COMP` (`|MakeArray` (make `/Game/Blueprints/SaveLoad/Base/S_SAVE_ITEM_PANEL` (make `/Game/Blueprints/StorageSystem/Panel/S_SlotsOnPanel` 0) (`local.EmptyPanel`)) :!type "/Game/Blueprints/SaveLoad/Base/S_SAVE_ITEM_PANEL Structure") (`|MakeArray` (make `/Game/Blueprints/SaveLoad/Base/S_SAVE_SKILL_PANEL` (struct) (`|MakeArray` (struct) (struct) (struct) (struct) (struct) (struct) (struct) (struct) (struct) :!type "GameplayTag Structure")) :!type "/Game/Blueprints/SaveLoad/Base/S_SAVE_SKILL_PANEL Structure")) BodyDAta (`NavigationSystemV1.K2_GetRandomReachablePointInRadius` (0.0 0.0 0.0) 1000.0 null null))))
          (bind _output_get_2 (set `local.Players` (`/Game/Blueprints/SaveLoad/SG_SAVE.Players` _slotbase)))
          (`BlueprintMapLibrary.Map_Add` _output_get_2 _returnvalue _output_get)
          (set `/Game/Blueprints/SaveLoad/SG_SAVE.Players` (`local.Players`) _slotbase)
          (return _slotbase))))))

(fn `SavePlayerToSlot`
  (params (Player :type "/Game/Player/BP_Character Object Reference") (Slot :type "/Game/Blueprints/SaveLoad/SG_SAVE Object Reference"))
  (returns (SlotResult :type "/Game/Blueprints/SaveLoad/SG_SAVE Object Reference"))
  (locals (NewSlot :type "/Game/Blueprints/SaveLoad/SG_SAVE Object Reference") (NewLocalVar :type "Map of Name to /Game/Blueprints/SaveLoad/S_SAVE_PLAYER Structure"))
  (bind _output_get (set `local.NewSlot` Slot))
  (bind _result (`/Game/Blueprints/SaveLoad/BFL_SaveLoad.SavePlayer` Player))
  (bind _output_get_2 (set `local.NewLocalVar` (`/Game/Blueprints/SaveLoad/SG_SAVE.Players` Slot)))
  (`BlueprintMapLibrary.Map_Add` _output_get_2 (`KismetStringLibrary.Conv_StringToName` (`/Game/Player/BP_Character.Player Name` Player)) _result)
  (set `/Game/Blueprints/SaveLoad/SG_SAVE.Players` _output_get_2 (`local.NewSlot`))
  (return _output_get))

(fn `UserConstructionScript`)