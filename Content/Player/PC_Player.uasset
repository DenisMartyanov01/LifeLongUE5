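; Player controller that turns Enhanced Input into character movement, skills, interaction, inventory and UI actions in a networked game.
; Movement, jumping, sphere-trace interaction, hotbar and storage changes route through SERVER events to the character's components and a movement skill.
; Mouse buttons drive per-hand skills from the held panel slot, passing modifier keys as string metadata; throwing charges a bar effect until release.
; It also saves local UI/camera settings, handles disconnects and retains test hooks.
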(event `TEST_MULTICAST`)

(event `TEST_ON_SERVER`
  (`self.TEST_MULTICAST`))

(event `self.ReceiveBeginPlay`
  (bind _returnvalue (subsystem `EnhancedInputLocalPlayerSubsystem`))
  (`KismetSystemLibrary.Delay` 0.1)
  (bind _asbp_character (cast `/Game/Player/BP_Character` (`self.K2_GetPawn`)))
  (set `self.MyCharacter` _asbp_character)
  (`KismetSystemLibrary.K2_SetTimerDelegate` (`|CreateDelegate` :!event `BreakFarInteraction`) 0.2 true)
  (set `self.bShowMouseCursor` false)
  (`/Engine/EditorBlueprintResources/StandardMacros.IsValid` _returnvalue
    (:`Is Valid`
      (`EnhancedInputSubsystemInterface.AddMappingContext` _returnvalue "/Game/Player/Input/IMP_Player.IMP_Player" 0 (struct)))
    (:`Is Not Valid`
      _))
  (set `self.Target` (`self.GetComponentByClass` (`self.K2_GetPawn`) "/Game/Blueprints/Animations/AC_Target.AC_Target_C"))
  (bind _skill (`/Game/Blueprints/SkillSystem/AC_SkillComponent.ActivateAnySkill` :`self` (`self.GetComponentByClass` (`self.K2_GetPawn`) "/Game/Blueprints/SkillSystem/AC_SkillComponent.AC_SkillComponent_C") :`Class` "/Game/Blueprints/SkillSystem/Skills/Movement/AS_MoveInterface.AS_MoveInterface_C"))
  (bind _asas_move_interface (cast `/Game/Blueprints/SkillSystem/Skills/Movement/AS_MoveInterface` _skill))
  (set `self.Moving` _asas_move_interface))

(event `EnhancedInput|/Game/Player/Input/Actions/IA_Test`
  (params (ActionValue :type Boolean) (ElapsedSeconds :type "Float (double-precision)") (TriggeredSeconds :type "Float (double-precision)") (InputAction :type "InputAction Object Reference" :default "/Game/Player/Input/Actions/IA_Test.IA_Test"))
  (:`Started`
    (bind _returnvalue (`GameplayStatics.GetActorOfClass` "/Game/Blueprints/Entities/A_EntityManager.A_EntityManager_C"))
    (`/Game/Blueprints/Entities/A_EntityManager.SpawnEntity` _returnvalue "skeleton" (0.0 0.0 50.0))))

(event `EnhancedInput|/Game/Player/Input/Actions/IA_Jump`
  (params (ActionValue :type Boolean) (ElapsedSeconds :type "Float (double-precision)") (TriggeredSeconds :type "Float (double-precision)") (InputAction :type "InputAction Object Reference" :default "/Game/Player/Input/Actions/IA_Jump.IA_Jump"))
  ; Movement
  (:`Started`
    (`self.SERVER_Jump`)))

(event `EnhancedInput|/Game/Player/Input/Actions/IA_MovePlayer`
  (params (ActionValue :type "Vector2D Structure") (ElapsedSeconds :type "Float (double-precision)") (TriggeredSeconds :type "Float (double-precision)") (InputAction :type "InputAction Object Reference" :default "/Game/Player/Input/Actions/IA_MovePlayer.IA_MovePlayer"))
  ; Movement
  (:`Triggered`
    (`self.SERVER_Move` ActionValue_X ActionValue_Y))
  (:`Started`
    (`self.SERVER_StartMoving`))
  (:`Canceled`
    (`self.SERVER_StopMoving` :!label _label))
  (:`Completed`
    (goto _label)))

(event `EnhancedInput|/Game/Player/Input/Actions/IA_Run`
  (params (ActionValue :type Boolean) (ElapsedSeconds :type "Float (double-precision)") (TriggeredSeconds :type "Float (double-precision)") (InputAction :type "InputAction Object Reference" :default "/Game/Player/Input/Actions/IA_Run.IA_Run"))
  (bind _mycharacter (`self.MyCharacter`))
  ; Movement
  (:`Triggered`
    (`self.SERVER_Run`))
  (:`Started`
    (`/Game/Player/BP_Character.MoveCameraWhileRun` _mycharacter)
    (`self.SERVER_StartRun`))
  (:`Canceled`
    (`/Game/Player/BP_Character.ReturnCameraAfterRun` _mycharacter :!label _label_2)
    (`self.SERVER_StopRun`))
  (:`Completed`
    (goto _label_2)))

(event `SERVER_Jump`
  ; Movement
  (`/Game/Blueprints/SkillSystem/AC_SkillComponent.ActivateSkill` (`/Game/Player/BP_Character.AC_Skills` (`self.MyCharacter`)) null "/Game/Blueprints/SkillSystem/Skills/Movement/AS_Jump.AS_Jump_C" ""))

(event `SERVER_Run`
  ; Movement
  (`/Game/Blueprints/SkillSystem/Skills/Movement/AS_MoveInterface.Run` (`self.Moving`)))

(event `SERVER_StartRun`
  ; Movement
  (`/Game/Blueprints/SkillSystem/Skills/Movement/AS_MoveInterface.StartRun` (`self.Moving`)))

(event `SERVER_Move`
  (params (X :type "Float (double-precision)") (Y :type "Float (double-precision)"))
  ; Movement
  (`/Game/Blueprints/SkillSystem/Skills/Movement/AS_MoveInterface.Move` (`self.Moving`) X Y))

(event `SERVER_StopRun`
  ; Movement
  (`/Game/Blueprints/SkillSystem/Skills/Movement/AS_MoveInterface.StopRun` (`self.Moving`)))

(event `SERVER_StartMoving`
  ; Movement
  (`/Game/Blueprints/SkillSystem/Skills/Movement/AS_MoveInterface.Start` (`self.Moving`)))

(event `SERVER_StopMoving`
  ; Movement
  (`/Game/Blueprints/SkillSystem/Skills/Movement/AS_MoveInterface.End` (`self.Moving`)))

(event `InputVectorAxis|Mouse2D`
  (params (AxisValue :type "Vector Structure"))
  (bind _mycharacter (`self.MyCharacter`))
  ; Movement
  (if (not (or (`self.bShowMouseCursor`) (`self.isLocked`)))
    (`Pawn.AddControllerYawInput` _mycharacter (* AxisValue_X 0.75))
    (`Pawn.AddControllerPitchInput` _mycharacter (* AxisValue_Y 0.75))))

(event `EnhancedInput|/Game/Player/Input/Actions/IA_OpenInventory`
  (params (ActionValue :type Boolean) (ElapsedSeconds :type "Float (double-precision)") (TriggeredSeconds :type "Float (double-precision)") (InputAction :type "InputAction Object Reference" :default "/Game/Player/Input/Actions/IA_OpenInventory.IA_OpenInventory"))
  (bind _ac_uimanager (`/Game/Player/BP_Character.AC_UIManager` (`self.MyCharacter`)))
  ; UI
  (:`Started`
    (if (not (`self.isLocked`))
      (`/Game/UI/AC_UIManager.SwitchUIVisibility` _ac_uimanager "NewEnumerator0")
      (`/Game/UI/AC_UIManager.UpdateUI` _ac_uimanager "NewEnumerator0"))))

(event `EnhancedInput|/Game/Player/Input/Actions/IA_OpenSkills`
  (params (ActionValue :type Boolean) (ElapsedSeconds :type "Float (double-precision)") (TriggeredSeconds :type "Float (double-precision)") (InputAction :type "InputAction Object Reference" :default "/Game/Player/Input/Actions/IA_OpenSkills.IA_OpenSkills"))
  ; UI
  (:`Started`
    (`/Game/UI/AC_UIManager.SwitchUIVisibility` (`/Game/Player/BP_Character.AC_UIManager` (`self.MyCharacter`)) "NewEnumerator5")))

(event `SERVER_SwitchPanel`
  (bind _ac_panel (`/Game/Player/BP_Character.AC_Panel` (`self.MyCharacter`)))
  ; UI
  (`/Game/Blueprints/StorageSystem/Panel/AC_Panel.SwapPanel` _ac_panel)
  (`/Game/Blueprints/StorageSystem/AC_Equipment.UpdateHands` (`/Game/Player/BP_Character.AC_Equipment` (`self.MyCharacter`)))
  (`/Game/Blueprints/StorageSystem/Panel/AC_Panel.SERVER_UpdatePanel` _ac_panel))

(event `SERVER_BreakInteraction`
  (bind _mycharacter (`self.MyCharacter`))
  ; Actions
  (message `/Game/Blueprints/Entities/BPI_Interact.OnBreakInteraction` (`/Game/Player/BP_Character.InteractionActor` _mycharacter))
  (message `/Game/Blueprints/Entities/BPI_Interact.OnBreakInteraction` _mycharacter))

(event `EnhancedInput|/Game/Player/Input/Actions/IA_Interact`
  (params (ActionValue :type Boolean) (ElapsedSeconds :type "Float (double-precision)") (TriggeredSeconds :type "Float (double-precision)") (InputAction :type "InputAction Object Reference" :default "/Game/Player/Input/Actions/IA_Interact.IA_Interact"))
  ; Actions
  (:`Started`
    (`/Engine/EditorBlueprintResources/StandardMacros.IsValid` (`/Game/Player/BP_Character.InteractionActor` (`self.MyCharacter`))
      (:`Is Valid`
        (`self.SERVER_BreakInteraction`))
      (:`Is Not Valid`
        (`self.SERVER_TryToInteract`)))))

(event `SERVER_TryToInteract`
  ; Actions
  (`self.TraceToInteract`))

(event `OnGoingLArm`
  (params (Keys :type String))
  (bind _leftarmskill (`self.LeftArmSkill`))
  ; Actions
  (`/Engine/EditorBlueprintResources/StandardMacros.IsValid` _leftarmskill
    (:`Is Valid`
      (`/Game/Blueprints/SkillSystem/Skills/A_Skill.OnGoingBase` _leftarmskill Keys))))

(event `EnhancedInput|/Game/Player/Input/Actions/IA_SwitchPanel`
  (params (ActionValue :type Boolean) (ElapsedSeconds :type "Float (double-precision)") (TriggeredSeconds :type "Float (double-precision)") (InputAction :type "InputAction Object Reference" :default "/Game/Player/Input/Actions/IA_SwitchPanel.IA_SwitchPanel"))
  ; UI
  (:`Started`
    (`self.SERVER_SwitchPanel`)
    (`/Game/UI/AC_UIManager.UpdateUI` (`/Game/Player/BP_Character.AC_UIManager` (`self.MyCharacter`)) "NewEnumerator2")))

(event `EnhancedInput|/Game/Player/Input/Actions/IA_Equipment`
  (params (ActionValue :type Boolean) (ElapsedSeconds :type "Float (double-precision)") (TriggeredSeconds :type "Float (double-precision)") (InputAction :type "InputAction Object Reference" :default "/Game/Player/Input/Actions/IA_Equipment.IA_Equipment"))
  (bind _ac_uimanager (`/Game/Player/BP_Character.AC_UIManager` (`self.MyCharacter`)))
  ; UI
  (:`Started`
    (if (not (`self.isLocked`))
      (`/Game/UI/AC_UIManager.SwitchUIVisibility` _ac_uimanager "NewEnumerator1")
      (`/Game/UI/AC_UIManager.UpdateUI` _ac_uimanager "NewEnumerator1"))))

(event `EnhancedInput|/Game/Player/Input/Actions/IA_LeftMouseBtn`
  (params (ActionValue :type Boolean) (ElapsedSeconds :type "Float (double-precision)") (TriggeredSeconds :type "Float (double-precision)") (InputAction :type "InputAction Object Reference" :default "/Game/Player/Input/Actions/IA_LeftMouseBtn.IA_LeftMouseBtn"))
  (bind _returnvalue (`self.GetKeys`))
  (bind _returnvalue_2 (== (`/Game/UI/AC_UIManager.WidgetsCount` (`/Game/Player/BP_Character.AC_UIManager` (`self.MyCharacter`))) 0))
  ; Actions
  (:`Triggered`
    (if _returnvalue_2
      (`self.OnGoingLArm` _returnvalue)))
  (:`Started`
    (if _returnvalue_2
      (`self.ActivateLArm` _returnvalue)))
  (:`Canceled`
    (`self.ReleaseLArm` :!label _label_3))
  (:`Completed`
    (goto _label_3)))

(event `ActivateLArm`
  (params (MetaData :type String))
  (bind _mycharacter (`self.MyCharacter`))
  ; Actions
  (bind (_source _holder _skill) (`/Game/Blueprints/StorageSystem/Panel/AC_Panel.GetSkillInHand` (`/Game/Player/BP_Character.AC_Panel` _mycharacter) true))
  (bind _returnvalue (`/Game/Blueprints/SkillSystem/AC_SkillComponent.ActivateSkill` (`/Game/Player/BP_Character.AC_Skills` _mycharacter) _holder _skill (`KismetStringLibrary.Concat_StrStr` (`|GetEnumeratorNameAsString` _source) "|" MetaData)))
  (set `self.LeftArmSkill` _returnvalue))

(event `EnhancedInput|/Game/Player/Input/Actions/IA_Numbers`
  (params (ActionValue :type "Float (double-precision)") (ElapsedSeconds :type "Float (double-precision)") (TriggeredSeconds :type "Float (double-precision)") (InputAction :type "InputAction Object Reference" :default "/Game/Player/Input/Actions/IA_Numbers.IA_Numbers"))
  ; UI
  (:`Started`
    (if (not (`self.isLocked`))
      (`self.SERVER_Numbers` (`KismetMathLibrary.FTrunc` (- ActionValue 1.0)) (not (`self.IsInputKeyDown` "LeftControl"))))))

(event `SERVER_Numbers`
  (params (Val :type Integer) (RButton :type Boolean))
  (bind _ac_equipment (`/Game/Player/BP_Character.AC_Equipment` (`self.MyCharacter`)))
  (bind _ac_panel (`/Game/Player/BP_Character.AC_Panel` (`self.MyCharacter`)))
  ; UI
  (bind (_result _has_changes) (`/Game/Blueprints/StorageSystem/Panel/AC_Panel.SetActiveSlots` _ac_panel Val RButton))
  (if _has_changes
    (`/Game/Blueprints/StorageSystem/AC_Equipment.UpdateHands` _ac_equipment)
    (`/Game/Blueprints/StorageSystem/Panel/AC_Panel.SERVER_UpdatePanel` _ac_panel)
    (`/Game/Blueprints/StorageSystem/AC_BaseStorage.SERVER_UpdateData` _ac_equipment)))

(event `EnhancedInput|/Game/Player/Input/Actions/IA_Save`
  (params (ActionValue :type Boolean) (ElapsedSeconds :type "Float (double-precision)") (TriggeredSeconds :type "Float (double-precision)") (InputAction :type "InputAction Object Reference" :default "/Game/Player/Input/Actions/IA_Save.IA_Save"))
  (bind _creativeui (`self.CreativeUI`))
  ; Actions
  (:`Started`
    (`/Engine/EditorBlueprintResources/StandardMacros.IsValid` _creativeui
      (:`Is Valid`
        (`Widget.RemoveFromParent` _creativeui)
        (set `self.CreativeUI` null))
      (:`Is Not Valid`
        (bind _returnvalue (`|CreateWidget` "/Game/UI/Storage/UW_CreativeBar.UW_CreativeBar_C"))
        (set `self.CreativeUI` _returnvalue)
        (`UserWidget.AddToViewport` _returnvalue 0)))))

(event `ReleaseLArm`
  (bind _leftarmskill (`self.LeftArmSkill`))
  ; Actions
  (`/Engine/EditorBlueprintResources/StandardMacros.IsValid` _leftarmskill
    (:`Is Valid`
      (`/Game/Blueprints/SkillSystem/Skills/A_Skill.OnRelease` _leftarmskill))))

(event `EnhancedInput|/Game/Player/Input/Actions/IA_ChangeActiveSlot`
  (params (ActionValue :type "Float (double-precision)") (ElapsedSeconds :type "Float (double-precision)") (TriggeredSeconds :type "Float (double-precision)") (InputAction :type "InputAction Object Reference" :default "/Game/Player/Input/Actions/IA_ChangeActiveSlot.IA_ChangeActiveSlot"))
  ; UI
  (:`Triggered`
    (if (not (`self.isLocked`))
      (`self.SERVER_ChangeSlot` ActionValue (not (`self.IsInputKeyDown` "LeftControl"))))))

(event `CLIENT_UpdateSlots`
  ; UI
  (`/Game/UI/AC_UIManager.UpdateActiveSlots` (`/Game/Player/BP_Character.AC_UIManager` (`self.MyCharacter`))))

(event `SERVER_ChangeSlot`
  (params (A :type "Float (double-precision)") (RButton :type Boolean))
  (bind _ac_equipment (`/Game/Player/BP_Character.AC_Equipment` (`self.MyCharacter`)))
  (bind _ac_panel (`/Game/Player/BP_Character.AC_Panel` (`self.MyCharacter`)))
  ; UI
  (`/Game/Blueprints/StorageSystem/Panel/AC_Panel.ChangeActiveSlot` _ac_panel (`KismetMathLibrary.FTrunc` A) RButton)
  (`/Game/Blueprints/StorageSystem/AC_Equipment.UpdateHands` _ac_equipment)
  (`/Game/Blueprints/StorageSystem/Panel/AC_Panel.SERVER_UpdatePanel` _ac_panel)
  (`/Game/Blueprints/StorageSystem/AC_BaseStorage.SERVER_UpdateData` _ac_equipment))

(event `OnGoingRArm`
  (params (Keys :type String))
  (bind _rightarmskill (`self.RightArmSkill`))
  ; Actions
  (`/Engine/EditorBlueprintResources/StandardMacros.IsValid` _rightarmskill
    (:`Is Valid`
      (`/Game/Blueprints/SkillSystem/Skills/A_Skill.OnGoingBase` _rightarmskill Keys))))

(event `EnhancedInput|/Game/Player/Input/Actions/IA_RightMouseBtn`
  (params (ActionValue :type Boolean) (ElapsedSeconds :type "Float (double-precision)") (TriggeredSeconds :type "Float (double-precision)") (InputAction :type "InputAction Object Reference" :default "/Game/Player/Input/Actions/IA_RightMouseBtn.IA_RightMouseBtn"))
  (bind _returnvalue (`self.GetKeys`))
  (bind _returnvalue_2 (== (`/Game/UI/AC_UIManager.WidgetsCount` (`/Game/Player/BP_Character.AC_UIManager` (`self.MyCharacter`))) 0))
  ; Actions
  (:`Triggered`
    (if _returnvalue_2
      (`self.OnGoingRArm` _returnvalue)))
  (:`Started`
    (if _returnvalue_2
      (`self.ActivareRArm` _returnvalue)))
  (:`Canceled`
    (`self.ReleaseRArm` :!label _label_4))
  (:`Completed`
    (goto _label_4)))

(event `EnhancedInput|/Game/Player/Input/Actions/IA_Esc`
  (params (ActionValue :type Boolean) (ElapsedSeconds :type "Float (double-precision)") (TriggeredSeconds :type "Float (double-precision)") (InputAction :type "InputAction Object Reference" :default "/Game/Player/Input/Actions/IA_Esc.IA_Esc"))
  ; UI
  (:`Started`
    (if (not (`self.isLocked`))
      (`/Game/UI/AC_UIManager.RemoveTopUI` (`/Game/Player/BP_Character.AC_UIManager` (`self.MyCharacter`))))))

(event `ActivareRArm`
  (params (Data :type String))
  (bind _mycharacter (`self.MyCharacter`))
  ; Actions
  (bind (_source _holder _skill) (`/Game/Blueprints/StorageSystem/Panel/AC_Panel.GetSkillInHand` (`/Game/Player/BP_Character.AC_Panel` _mycharacter) false))
  (bind _returnvalue (`/Game/Blueprints/SkillSystem/AC_SkillComponent.ActivateSkill` (`/Game/Player/BP_Character.AC_Skills` _mycharacter) _holder _skill (`KismetStringLibrary.Concat_StrStr` (`|GetEnumeratorNameAsString` _source) "|" Data)))
  (set `self.RightArmSkill` _returnvalue))

(event `SERVER_DropItemToSlot`
  (params (Data :type "/Game/Blueprints/StorageSystem/S_DragData Structure") (Index :type Integer))
  (bind (_aindex _data _infinite _baseactor _type) (break `/Game/Blueprints/StorageSystem/S_DragData` Data))
  (bind _storage (`/Game/Blueprints/StorageSystem/BFL_Storage.GetStorageByType` _baseactor _type))
  ; UI
  (`/Game/Blueprints/StorageSystem/AC_BaseStorage.DropToSlot` _storage Data Index)
  (`/Game/Blueprints/StorageSystem/AC_BaseStorage.SERVER_UpdateData` _storage)
  (if (== _type (`KismetSystemLibrary.MakeLiteralByte` (enumliteral `/Game/Blueprints/StorageSystem/E_StorageType` "NewEnumerator2")))
    (`/Game/Blueprints/StorageSystem/AC_Equipment.UpdateHands` (`/Game/Player/BP_Character.AC_Equipment` (`self.MyCharacter`)))))

(event `SERVER_SwapItems`
  (params (ActorA :type "Actor Object Reference") (TypeA :type "/Game/Blueprints/StorageSystem/E_StorageType Enum" :default "NewEnumerator3") (IndexA :type Integer) (ActorB :type "Actor Object Reference") (TypeB :type "/Game/Blueprints/StorageSystem/E_StorageType Enum" :default "NewEnumerator3") (IndexB :type Integer))
  (bind _storage (`/Game/Blueprints/StorageSystem/BFL_Storage.GetStorageByType` ActorB TypeB))
  (bind _storage_2 (`/Game/Blueprints/StorageSystem/BFL_Storage.GetStorageByType` ActorA TypeA))
  (bind _returnvalue (`KismetSystemLibrary.MakeLiteralByte` (enumliteral `/Game/Blueprints/StorageSystem/E_StorageType` "NewEnumerator2")))
  (bind _returnvalue_2 (`KismetSystemLibrary.MakeLiteralByte` (enumliteral `/Game/Blueprints/StorageSystem/E_StorageType` "NewEnumerator1")))
  ; UI
  (`/Game/Blueprints/StorageSystem/AC_BaseStorage.Swap` _storage _storage_2 IndexA IndexB)
  (`/Game/Blueprints/StorageSystem/AC_BaseStorage.SERVER_UpdateData` _storage_2)
  (`/Game/Blueprints/StorageSystem/AC_BaseStorage.SERVER_UpdateData` _storage)
  (if (and (or (== TypeA _returnvalue) (== TypeB _returnvalue)) (not (or (== TypeA _returnvalue_2) (== TypeB _returnvalue_2))))
    (`/Game/Blueprints/StorageSystem/AC_Equipment.UpdateHands` (`/Game/Player/BP_Character.AC_Equipment` (`self.MyCharacter`)))
    (`/Game/Blueprints/StorageSystem/AC_BaseStorage.SERVER_UpdateData` (`/Game/Player/BP_Character.AC_Equipment` (`self.MyCharacter`)))))

(event `ReleaseRArm`
  (bind _rightarmskill (`self.RightArmSkill`))
  ; Actions
  (`/Engine/EditorBlueprintResources/StandardMacros.IsValid` _rightarmskill
    (:`Is Valid`
      (`/Game/Blueprints/SkillSystem/Skills/A_Skill.OnRelease` _rightarmskill))))

(event `SERVER_SetItemToSlot`
  (params (Index :type Integer) (Data :type "/Game/Blueprints/SaveLoad/Base/S_SAVE_DATA_ITEM Structure") (Actor :type "Actor Object Reference") (Type :type "/Game/Blueprints/StorageSystem/E_StorageType Enum" :default "NewEnumerator0"))
  (bind _storage (`/Game/Blueprints/StorageSystem/BFL_Storage.GetStorageByType` Actor Type))
  ; UI
  (bind _result (`/Game/Blueprints/SaveLoad/BFL_SaveLoad.DeSerializeItem` Data))
  (`/Game/Blueprints/StorageSystem/AC_BaseStorage.SetSlot` _storage Index _result false)
  (`/Game/Blueprints/StorageSystem/AC_BaseStorage.SERVER_UpdateData` _storage))

(event `EnhancedInput|/Game/Player/Input/Actions/IA_LockTarget`
  (params (ActionValue :type Boolean) (ElapsedSeconds :type "Float (double-precision)") (TriggeredSeconds :type "Float (double-precision)") (InputAction :type "InputAction Object Reference" :default "/Game/Player/Input/Actions/IA_LockTarget.IA_LockTarget"))
  (bind _ac_target (`/Game/Player/BP_Character.AC_Target` (`self.MyCharacter`)))
  ; Actions
  (:`Started`
    (if (`/Game/Blueprints/Animations/AC_Target.is_locked` _ac_target)
      (`/Game/Blueprints/Animations/AC_Target.ReleaseTarget` _ac_target)
      (else
        (bind _output_get (`/Game/Blueprints/Animations/AC_Target.LockTarget` _ac_target))))))

(event `SwitchToBaseCamera`
  ; NET
  (`self.SetViewTargetWithBlend` self (`self.MyCharacter`) 0.0 "VTBlend_Linear" 0.0 false))

(event `EnhancedInput|/Game/Player/Input/Actions/IA_Throw`
  (params (ActionValue :type Boolean) (ElapsedSeconds :type "Float (double-precision)") (TriggeredSeconds :type "Float (double-precision)") (InputAction :type "InputAction Object Reference" :default "/Game/Player/Input/Actions/IA_Throw.IA_Throw"))
  (bind _returnvalue (`self.IsInputKeyDown` "LeftControl"))
  (bind _returnvalue_2 (not _returnvalue))
  (bind _ac_panel (`/Game/Player/BP_Character.AC_Panel` (`self.MyCharacter`)))
  (bind _ac_animhumanoid (`/Game/Player/BP_Character.AC_AnimHumanoid` (`self.MyCharacter`)))
  ; Actions
  (:`Started`
    (bind (_index _item) (`/Game/Blueprints/StorageSystem/Panel/AC_Panel.GetHandItem` _ac_panel true))
    (bind (_index_2 _item_2) (`/Game/Blueprints/StorageSystem/Panel/AC_Panel.GetHandItem` _ac_panel false))
    (bind _itemdata_id (break `/Game/Data/S_CompBase` (`/Game/Data/O_Item.ItemData` _item_2)))
    (bind _itemdata_id_2 (break `/Game/Data/S_CompBase` (`/Game/Data/O_Item.ItemData` _item)))
    (bind _returnvalue_3 (== _index _index_2))
    (bind _returnvalue_4 (+ (`KismetMathLibrary.Conv_BoolToByte` _returnvalue_2) (* (`KismetMathLibrary.Conv_BoolToByte` _returnvalue_3) 2)))
    (if (not (== (select `byte` _returnvalue_4 :`0` _itemdata_id :`1` _itemdata_id_2 :`2` _itemdata_id_2 :`3` _itemdata_id_2) "air"))
      (`/Game/Blueprints/Animations/AC_AnimHumanoid.SetHandsPos` _ac_animhumanoid "NewEnumerator6" _returnvalue_2 _returnvalue_3)
      (if _returnvalue_3
        (`/Game/Blueprints/Animations/AC_AnimHumanoid.SetHandsPos` _ac_animhumanoid "NewEnumerator6" _returnvalue true))
      (bind _scaleeffect (`/Game/Blueprints/SkillSystem/AC_SkillComponent.ApplyBarEffect` (`/Game/Player/BP_Character.AC_Skills` (`self.MyCharacter`)) "/Game/Blueprints/SkillSystem/Skills/Attack/Throw/AS_ThrowBase.AS_ThrowBase_C" 1.0 (select `byte` _returnvalue_4 :`0` "Left" :`1` "Right" :`2` "Two" :`3` "Two")))
      (bind _asas_throw_base (cast `/Game/Blueprints/SkillSystem/Skills/Attack/Throw/AS_ThrowBase` _scaleeffect))
      (set `/Game/Blueprints/SkillSystem/Skills/Attack/Throw/AS_ThrowBase.Item` (select `byte` _returnvalue_4 :`0` _item_2 :`1` _item :`2` _item :`3` _item) _asas_throw_base)
      (set `/Game/Blueprints/SkillSystem/Skills/Attack/Throw/AS_ThrowBase.throw_full` (`self.IsInputKeyDown` "LeftAlt") _asas_throw_base)))
  (:`Canceled`
    (`/Engine/EditorBlueprintResources/StandardMacros.IsValid` _scaleeffect :!label _label_5
      (:`Is Valid`
        (`/Game/Blueprints/SkillSystem/Skills/Attack/Throw/AS_ThrowBase.Throw` _asas_throw_base))))
  (:`Completed`
    (goto _label_5)))

(event `CLIENT_StartPlay`
  ; NET
  (`WidgetBlueprintLibrary.SetInputMode_GameOnly` self)
  (set `self.bShowMouseCursor` false))

(event `SERVER_ExitGame`
  ; NET
  (bind _asgm_player (cast `/Game/Player/GM_Player` (`GameplayStatics.GetGameMode`)))
  (switch `ENetRole` (`self.GetRemoteRole`)
    (:`ROLE_SimulatedProxy`
      (`/Game/Player/GM_Player.DisconnectHost` _asgm_player self :!label _label_6))
    (:`ROLE_AutonomousProxy`
      (`/Game/Player/GM_Player.DisconnectPlayer` _asgm_player self))
    (:`ROLE_Authority`
      (goto _label_6))))

(event `CLIENT_SaveLocalSettings`
  ; Actions
  (`self.SaveLocal`))

(fn `BreakFarInteraction`
  (bind _mycharacter (`self.MyCharacter`))
  (`/Engine/EditorBlueprintResources/StandardMacros.IsValid` null
    (:`Is Valid`
      (if (> (`KismetMathLibrary.Vector_Distance` (`self.K2_GetActorLocation` (`self.MyCharacter`)) (`self.K2_GetActorLocation`)) 500.0)
        (message `/Game/Blueprints/Entities/BPI_Interact.OnBreakInteraction` (`/Game/Player/BP_Character.InteractionActor` _mycharacter))
        (message `/Game/Blueprints/Entities/BPI_Interact.OnBreakInteraction` _mycharacter)))))

(fn `GetKeys`
  (returns (ReturnValue :type String))
  (return (`KismetStringLibrary.Concat_StrStr` (`KismetMathLibrary.SelectString` "ctrl|" "" (`self.IsInputKeyDown` "LeftControl")) (`KismetMathLibrary.SelectString` "shift|" "" (`self.IsInputKeyDown` "LeftShift")) (`KismetMathLibrary.SelectString` "alt|" "" (`self.IsInputKeyDown` "LeftAlt")))))

(fn `SaveLocal`
  (locals (Save :type "/Game/Blueprints/SaveLoad/SG_LocalSettings Object Reference"))
  (bind _mycharacter (`self.MyCharacter`))
  (bind _save (`local.Save`))
  (bind (_relativelocation_x _relativelocation_y _relativelocation_z) (`KismetMathLibrary.BreakVector` (`SceneComponent.RelativeLocation` (`/Game/Player/BP_Character.Camera` _mycharacter))))
  (bind _returnvalue (`GameplayStatics.DoesSaveGameExist` "PLAYER_LOCAL"))
  (if _returnvalue
    (bind _returnvalue_2 (`GameplayStatics.LoadGameFromSlot` "PLAYER_LOCAL"))
    (bind _assg_local_settings (cast `/Game/Blueprints/SaveLoad/SG_LocalSettings` _returnvalue_2))
    (set `local.Save` _assg_local_settings)
    (else
      (bind _returnvalue_3 (`GameplayStatics.CreateSaveGameObject` "/Game/Blueprints/SaveLoad/SG_LocalSettings.SG_LocalSettings_C"))
      (set `local.Save` _returnvalue_3)))
  (bind _data (`/Game/Blueprints/SaveLoad/BFL_SaveLoad.SaveUI` (`/Game/Player/BP_Character.AC_UIManager` _mycharacter)))
  (set `/Game/Blueprints/SaveLoad/SG_LocalSettings.UI` _data _save)
  (set `/Game/Blueprints/SaveLoad/SG_LocalSettings.Controls` (make `/Game/Blueprints/SaveLoad/Components/Local/S_SAVE_Controls` (`/Game/Player/BP_Character.defaultSpringArmLength` _mycharacter) _relativelocation_z) _save)
  (`GameplayStatics.SaveGameToSlot` (`local.Save`) "PLAYER_LOCAL"))

(fn `TraceToInteract`
  (bind _mycharacter (`self.MyCharacter`))
  (bind _mycharacter_2 (`self.MyCharacter`))
  (bind _ac_target (`/Game/Player/BP_Character.AC_Target` _mycharacter))
  (bind (_outhit _returnvalue) (`KismetSystemLibrary.SphereTraceSingle` (`SceneComponent.K2_GetComponentLocation` (`/Game/Blueprints/Animations/AC_Target.StartLookPoint` _ac_target)) (`SceneComponent.K2_GetComponentLocation` (`/Game/Blueprints/Animations/AC_Target.FinalTarget` _ac_target)) 10.0 "TraceTypeQuery1" false (`|MakeArray` _mycharacter :!type "Actor Object Reference")))
  (if _returnvalue
    (bind (_bblockinghit _binitialoverlap _time _distance _location _impactpoint _normal _impactnormal _physmat _hitactor) (`GameplayStatics.BreakHitResult` _outhit))
    (if (< (`KismetMathLibrary.Vector_Distance` (`self.K2_GetActorLocation` (`self.K2_GetPawn`)) (`self.K2_GetActorLocation` _hitactor)) 300.0)
      (message `/Game/Blueprints/Entities/BPI_Interact.OnInteract` _mycharacter_2 _hitactor _impactpoint _normal)
      (message `/Game/Blueprints/Entities/BPI_Interact.OnInteract` _hitactor _mycharacter_2 _impactpoint _normal))))

(fn `UserConstructionScript`)