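; Player character that handles movement, interaction, replicated name display, death and respawn near the death point.
; Landing stops the jump skill and converts fall velocity into damage through ACSkills, which also restores health on respawn.
; Character creation loads a level instance at a random high-altitude location, with an invisible spawned floor and its own camera.
; Per-tick sphere traces smoothly adjust spring arm length, while timers and timelines shift the camera for running and targeting.
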(event `CLIENT_Move`
  (params (WorldDirectionX :type "Vector Structure") (WorldDirectionY :type "Vector Structure") (X :type "Float (single-precision)") (Y :type "Float (single-precision)"))
  (`self.AddMovementInput` WorldDirectionY Y)
  (`self.AddMovementInput` WorldDirectionX X))

(event `CLIENT_Jump`
  (`self.Jump`))

(event `TeleportCharacter`
  (params (NewLocation :type "Vector Structure"))
  (`self.K2_SetActorLocation` NewLocation)
  (bind _returnvalue (`|SpawnActorFromClass` "/Script/Engine.StaticMeshActor" (`KismetMathLibrary.MakeTransform` (- NewLocation (0.0 0.0 100.0))) "Undefined" "MultiplyWithRoot" self null))
  (`StaticMeshActor.SetMobility` _returnvalue "Movable")
  (bind _staticmeshcomponent (`StaticMeshActor.StaticMeshComponent` _returnvalue))
  (`StaticMeshComponent.SetStaticMesh` _staticmeshcomponent "/Engine/BasicShapes/Cube.Cube")
  (`SceneComponent.SetVisibility` _staticmeshcomponent false false))

(event `RemoveStartRoom`
  (`LevelStreaming.SetIsRequestingUnloadAndRemoval` (stale `CreateStartRoom` _returnvalue_2) true)
  (`/Engine/EditorBlueprintResources/StandardMacros.IsValid` (stale `TeleportCharacter` _returnvalue)
    (:`Is Valid`
      (`self.K2_DestroyActor` (stale `TeleportCharacter` _returnvalue)))))

(event `CreateStartRoom`
  (bind _deathpoint (`self.DeathPoint`))
  (bind _returnvalue (+ _deathpoint (0.0 0.0 50.0)))
  (set `self.DeathPoint` (`KismetMathLibrary.MakeVector` (`KismetMathLibrary.Conv_IntToDouble` (* (`KismetMathLibrary.RandomIntegerInRange` 0 100) 100)) (`KismetMathLibrary.Conv_IntToDouble` (* (`KismetMathLibrary.RandomIntegerInRange` 0 100) 100)) 10000.0))
  (bind (_boutsuccess _returnvalue_2) (`LevelStreamingDynamic.LoadLevelInstanceBySoftObjectPtr` "/Game/Levels/L_CharacterCreation.L_CharacterCreation" _deathpoint (struct :`Yaw` 180.0) "" null))
  (`self.K2_SetActorLocation` _returnvalue)
  (`self.TeleportCharacter` _returnvalue)
  (`KismetSystemLibrary.Delay` 1.0)
  (`/Game/Blueprints/Animations/AC_BodyPart.UpdateBodyType` (`self.AC_BodyPart`))
  (bind _outactors (`GameplayStatics.GetAllActorsOfClassWithTag` "/Script/Engine.CameraActor" "CreationCamera"))
  (bind _aspc_player (cast `/Game/Player/PC_Player` (`self.GetController`)))
  (`PlayerController.SetViewTargetWithBlend` _aspc_player (`|GetArrayItem` _outactors) 0.0 "VTBlend_Linear" 0.0 false))

(event `self.OnLanded`
  (params (Hit :type "HitResult Structure (by ref)"))
  (`self.SERVER_StopJump`))

(event `SERVER_StopJump`
  (bind _ac_skills (`self.AC_Skills`))
  (bind _returnvalue (`KismetMathLibrary.FClamp` (/ (+ (.z (`self.GetVelocity`)) 1000.0) -20.0) 0.0 99999.0))
  (`/Game/Blueprints/SkillSystem/AC_SkillComponent.StopSkillByTag` _ac_skills (struct :`TagName` "Skills.Base.Movement.Jump"))
  (if (> _returnvalue 5.0)
    (`/Game/Blueprints/SkillSystem/AC_SkillComponent.ActivateSkill` _ac_skills null "/Game/Blueprints/SkillSystem/Skills/Base/AS_TakeDamage.AS_TakeDamage_C" (`/Game/Blueprints/SkillSystem/BFL_SkillsHelper.SerializeDamage` (struct :`TagName` "Attributes.Base.Health") (`|MakeMap` (struct :`TagName` "Attributes.Attack.FallDamage") _returnvalue :!type "GameplayTag Structure") true))))

(event `self.ReceiveBeginPlay`
  (`self.SetupLocal`))

(event `self.ReceiveTick`
  (params (DeltaSeconds :type "Float (single-precision)"))
  (`/Game/UI/AC_UIManager.UpdateUI` (`self.AC_UIManager`) "NewEnumerator3")
  (`self.CameraCollision`))

(event `Respawn`
  (`self.RestoreStats`)
  (`self.K2_SetActorLocation` (`NavigationSystemV1.K2_GetRandomReachablePointInRadius` (stale `/Game/Blueprints/Entities/BPI_Damage.Die` _output_get) 1000.0 null null))
  (`ActorComponent.Activate` (`self.CharacterMovement`) false)
  (set `SkeletalMeshComponent.bPauseAnims` false (`self.Mesh`))
  (`/Game/UI/AC_UIManager.OnRespawn` (`self.AC_UIManager`)))

(event `/Game/Blueprints/Entities/BPI_Damage.Die`
  (bind _output_get (set `self.DeathPoint` (`self.K2_GetActorLocation`)))
  (`ActorComponent.Deactivate` (`self.CharacterMovement`))
  (`/Game/UI/AC_UIManager.OnDeath` (`self.AC_UIManager`))
  (set `SkeletalMeshComponent.bPauseAnims` true (`self.Mesh`)))

(event `SERVER_BreakInteraction`
  (set `self.InteractionActor` null))

(event `/Game/Blueprints/Entities/BPI_Interact.OnBreakInteraction`
  (`self.SERVER_BreakInteraction`))

(event `/Game/Blueprints/Entities/BPI_Interact.OnInteract`
  (params (Insignator :type "Actor Object Reference") (Location :type "Vector Structure") (Normal :type "Vector Structure"))
  (`self.SERVER_Ineract` Insignator))

(event `SERVER_Ineract`
  (params (InteractionActor :type "Actor Object Reference"))
  (set `self.InteractionActor` InteractionActor))

(event `CameraCollision`
  (bind _array (`|MakeArray` "ObjectTypeQuery1" "ObjectTypeQuery2" "ObjectTypeQuery4" :!type "EObjectTypeQuery Enum"))
  (bind _springarm (`self.SpringArm`))
  (bind _springarm_2 (`self.SpringArm`))
  (bind _defaultspringarmlength (`self.defaultSpringArmLength`))
  (bind _returnvalue (`SceneComponent.K2_GetComponentLocation` (`self.SpringArm`)))
  (bind _returnvalue_2 (`KismetMathLibrary.FInterpTo` (`SpringArmComponent.TargetArmLength` _springarm_2) _defaultspringarmlength (`GameplayStatics.GetWorldDeltaSeconds`) (`self.GetInterpSpeed`)))
  (bind _returnvalue_3 (`KismetMathLibrary.Normal` (- (`SceneComponent.K2_GetComponentLocation` (`self.Camera`)) (`SceneComponent.K2_GetComponentLocation` (`self.SpringArm`)))))
  (bind _returnvalue_4 (* (`KismetMathLibrary.Normal` (- (`SceneComponent.K2_GetComponentLocation` (`self.Camera`)) (`SceneComponent.K2_GetComponentLocation` (`self.SpringArm`)))) _returnvalue_2))
  (bind (_outhit _returnvalue_5) (`KismetSystemLibrary.SphereTraceSingleForObjects` (+ _returnvalue (* _returnvalue_3 30.0)) (+ _returnvalue (* _returnvalue_3 (`self.SpringArmLength`))) 30.0 _array))
  (if _returnvalue_5
    (bind _output_get (set `self.Impact Point` (`.ImpactPoint` (`GameplayStatics.BreakHitResult` _outhit))))
    (set `SpringArmComponent.TargetArmLength` (`KismetMathLibrary.FInterpTo` (`SpringArmComponent.TargetArmLength` _springarm) (- (`KismetMathLibrary.Vector_Distance` (`SceneComponent.K2_GetComponentLocation` (`self.SpringArm`)) _output_get) 10.0) (`GameplayStatics.GetWorldDeltaSeconds`) (`self.GetInterpSpeed`)) _springarm)
    (elif (not (`KismetMathLibrary.NearlyEqual_FloatFloat` (`SpringArmComponent.TargetArmLength` (`self.SpringArm`)) _defaultspringarmlength 10.0))
      (bind (_outhit_2 _returnvalue_6) (`KismetSystemLibrary.SphereTraceSingleForObjects` (+ (`SceneComponent.K2_GetComponentLocation` (`self.SpringArm`)) _returnvalue_4) _returnvalue_4 25.0 _array))
      (if (not _returnvalue_6)
        (set `SpringArmComponent.TargetArmLength` _returnvalue_2 _springarm_2)))))

(event `SetPlayerNameOnServer`
  (params (PlayerName :type String))
  (set `self.Player Name` PlayerName))

(event `MoveCameraWhileRun`
  (if (not (`self.is_running`))
    (set `self.is_running` true)
    (bind _returnvalue (`KismetSystemLibrary.K2_SetTimerDelegate` (delegate `MoveCamBack`) 0.01 true))
    (`KismetSystemLibrary.Delay` 0.5)
    (`KismetSystemLibrary.K2_ClearAndInvalidateTimerHandle` _returnvalue)))

(event `MoveCameraToTarget`
  (bind _returnvalue (`KismetMathLibrary.MakeVector` 100.0 40.0))
  (if (not (`self.is_camera_on_target`))
    (set `self.is_camera_on_target` true)
    (bind (_direction _newtrack_0) (`Timeline|Timeline` :!via `PlayFromStart`)
      (:`Update`
        (`SceneComponent.K2_SetRelativeLocation` (`self.Camera`) (`KismetMathLibrary.VLerp` _returnvalue (+ _returnvalue (50.0 70.0 0.0)) _newtrack_0) false false)
        (`SceneComponent.K2_SetRelativeLocation` (`self.Camera`) (`KismetMathLibrary.VLerp` _returnvalue (+ _returnvalue (50.0 70.0 0.0)) _newtrack_0) false false)))))

(event `MoveCamBack`
  (`SceneComponent.K2_SetRelativeLocation` (`self.Camera`) (+ (`SceneComponent.RelativeLocation` (`self.Camera`)) (-1.0 0.0 0.0)) false false)
  (`SceneComponent.K2_SetRelativeLocation` (`self.Camera`) (+ (`SceneComponent.RelativeLocation` (`self.Camera`)) (-1.0 0.0 0.0)) false false))

(event `ReturnCameraAfterRun`
  (if (`self.is_running`)
    (set `self.is_running` false)
    (bind _returnvalue (`KismetSystemLibrary.K2_SetTimerDelegate` (delegate `MoveCamForward`) 0.01 true))
    (`KismetSystemLibrary.Delay` 0.5)
    (`KismetSystemLibrary.K2_ClearAndInvalidateTimerHandle` _returnvalue)))

(event `ReleaseCamera`
  (if (`self.is_camera_on_target`)
    (set `self.is_camera_on_target` false)
    (bind (_direction _newtrack_0) (`Timeline|Timeline_0` :!via `PlayFromStart`)
      (:`Update`
        (`SceneComponent.K2_SetRelativeLocation` (`self.Camera`) (`KismetMathLibrary.VLerp` (`SceneComponent.RelativeLocation` (`self.Camera`)) (`KismetMathLibrary.MakeVector` 100.0 40.0) _newtrack_0) false false)
        (`SceneComponent.K2_SetRelativeLocation` (`self.Camera`) (`KismetMathLibrary.VLerp` (`SceneComponent.RelativeLocation` (`self.Camera`)) (`KismetMathLibrary.MakeVector` 100.0 40.0) _newtrack_0) false false)))))

(event `MoveCamForward`
  (`SceneComponent.K2_SetRelativeLocation` (`self.Camera`) (+ (`SceneComponent.RelativeLocation` (`self.Camera`)) (1.0 0.0 0.0)) false false)
  (`SceneComponent.K2_SetRelativeLocation` (`self.Camera`) (+ (`SceneComponent.RelativeLocation` (`self.Camera`)) (1.0 0.0 0.0)) false false))

(fn `CanJumpInternal`
  (returns (ReturnValue :type Boolean))
  (bind (_returnvalue_x _returnvalue_y _returnvalue_z) (`KismetMathLibrary.BreakVector` (`self.K2_GetActorLocation`)))
  (if (`NavMovementComponent.IsSwimming` (`self.CharacterMovement`))
    (return (> _returnvalue_z 0.0))
    (else
      (bind _returnvalue (`parent.CanJumpInternal`))
      (return _returnvalue))))

(fn `GetInterpSpeed`
  (returns (ReturnValue :type "Float (double-precision)"))
  (locals (InterpSpeed :type "Float (double-precision)" :default 10.0))
  (bind _interpspeed (`local.InterpSpeed`))
  (return (`KismetMathLibrary.MapRangeClamped` (`KismetMathLibrary.Vector_Distance` (`SceneComponent.K2_GetComponentLocation` (`self.Camera`)) (`self.Impact Point`)) 50.0 (`self.defaultSpringArmLength`) _interpspeed (* _interpspeed 2.0))))

(fn `OnRep_Player Name`
  (bind _asuw_player_name (cast `/Game/UI/UW_PlayerName` (`WidgetComponent.GetWidget` (`self.Widget`))))
  (`/Game/UI/UW_PlayerName.SetName` _asuw_player_name (`self.Player Name`)))

(fn `RestoreStats`
  (locals (SkillsToStop :type "Array of GameplayTag Structure"))
  (bind _ac_skills (`self.AC_Skills`))
  (bind _attributeset (`/Game/Blueprints/SkillSystem/AC_SkillComponent.AttributeSet` _ac_skills))
  (bind _value (`BlueprintMapLibrary.Map_Find` _attributeset (struct :`TagName` "Attributes.Base.Health")))
  (for _array_element (`local.SkillsToStop`)
    (`/Game/Blueprints/SkillSystem/AC_SkillComponent.StopSkillByTag` (`self.AC_Skills`) _array_element))
  (`BlueprintMapLibrary.Map_Add` _attributeset (struct :`TagName` "Attributes.Base.Health") (make `/Game/Blueprints/SkillSystem/S_Attribute` (break `/Game/Blueprints/SkillSystem/S_Attribute` _value) (`.Max_24_B52313574BD363B2E33D4CBBE239C895` (break `/Game/Blueprints/SkillSystem/S_Attribute` _value)) 0.0 (`.Max_24_B52313574BD363B2E33D4CBBE239C895` (break `/Game/Blueprints/SkillSystem/S_Attribute` _value))))
  (`/Game/Blueprints/SkillSystem/AC_SkillComponent.ReCalculateAttribute` _ac_skills (struct :`TagName` "Attributes.Base.Health")))

(fn `SetupLocal`
  (if (`self.IsLocallyControlled`)
    (bind _asgi_main (cast `/Game/Player/GI_Main` (`GameplayStatics.GetGameInstance`)))
    (`self.SetPlayerNameOnServer` (`/Game/Player/GI_Main.MyPlayerName` _asgi_main))))

(fn `UserConstructionScript`
  (`self.SetReplicates` false))