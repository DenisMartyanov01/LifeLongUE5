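; Blueprint function library that converts player state to save data and restores it, with separate helpers for UI layout and camera settings.
; SavePlayer and LoadPlayer delegate to per-component functions for inventory, equipment, panels, skills and body parts, plus transform and velocity.
; Items are rebuilt by name with count, durability and gun ammo.
; Flagged effects and buffs keep remaining duration; the saved world is hard-coded to Map_Battle.
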(fn `DeSerializeItem`
  (params (Data :type "/Game/Blueprints/SaveLoad/Base/S_SAVE_DATA_ITEM Structure"))
  (returns (Result :type "/Game/Data/O_Item Object Reference"))
  (bind _result (`/Game/Blueprints/Items/BFL_Items.CreateItemByName` Data_Name_2_D2E6ADE648A9CD042F0B929C477D1194 (`local.__WorldContext`)))
  (`/Game/Data/O_Item.SetCount` _result Data_Count_8_D55806B147030119FCB453ADEFBA51CA)
  (`/Game/Data/O_Item.SetDurability` _result Data_Durability_17_B81271D14DF1FE251602AFB79AFC9A64)
  (bind _aso_weapon_gun (cast `/Game/Data/O_WeaponGun` _result)
    (:`then`
      (bind _magazine (`/Game/Data/O_WeaponGun.Magazine` _aso_weapon_gun))
      (bind _aso_bullet (cast `/Game/Data/O_Bullet` _magazine))
      (`/Game/Data/O_Item.SetByName` _aso_bullet Data_BulletName_20_5656D6B44CD5CF7DF0DD54AE4555BFE4)
      (`/Game/Data/O_Item.SetCount` _magazine Data_BulletCount_14_D3894D29424CE0D8B60D89A9FE0ECEA0))
    (:`CastFailed`
      _))
  (return _result))

(fn `LoadBodyParts`
  (params (Data :type "/Game/Blueprints/SaveLoad/Components/S_SAVE_BODY_PARTS_COMP Structure") (BodyParts :type "/Game/Blueprints/Animations/AC_BodyPart Object Reference") (__WorldContext :type "Object Object Reference"))
  (`|ExecutionSequence`
    (:`then_0`
      (set `/Game/Blueprints/Animations/AC_BodyPart.BodyType` Data_BodyType_37_CA3EFF4A4C1BCACB2C787C8D7C7CB2B7 BodyParts)
      (set `/Game/Blueprints/Animations/AC_BodyPart.HairColor` Data_HairColor_40_8A4166F64B72857572595FAB08680E9E BodyParts)
      (set `/Game/Blueprints/Animations/AC_BodyPart.BeardColor` Data_BeardColor_25_5ED3CD074DE5025A3D0C128AB8DF0F22 BodyParts)
      (set `/Game/Blueprints/Animations/AC_BodyPart.BrowsColor` Data_BrowsColor_23_D7C2AA344A41A79F423262A0942CE406 BodyParts)
      (set `/Game/Blueprints/Animations/AC_BodyPart.PuplisColor` Data_EyesColor_15_BB85BD084CEE7003ED95D0B1D6FD76E1 BodyParts)
      (set `/Game/Blueprints/Animations/AC_BodyPart.Skin Color` Data_SkinColor_27_F502B2BF4316EC9820D996A957080969 BodyParts)
      (set `/Game/Blueprints/Animations/AC_BodyPart.BrowsName` Data_BrowsType_35_416ABE6B4548BE71D3304B8B62FD1536 BodyParts)
      (set `/Game/Blueprints/Animations/AC_BodyPart.EyesName` Data_Eyes_33_1AB256804185040896AB71A7E7C98965 BodyParts)
      (set `/Game/Blueprints/Animations/AC_BodyPart.MouthName` Data_MouthType_34_E4CC2F3B4332EF729B85E0A7815CF855 BodyParts)
      (set `/Game/Blueprints/Animations/AC_BodyPart.BeardName` Data_BeardName_30_08B771FA4F384BEA1EACEF8CB70F975E BodyParts)
      (set `/Game/Blueprints/Animations/AC_BodyPart.HairName` Data_HairName_32_FE434B1A4671596BB8F6B1BDF88DFAC4 BodyParts))
    (:`then_1`
      (`/Game/Blueprints/Animations/AC_BodyPart.UpdateBodyType` BodyParts)
      (`/Game/Blueprints/Animations/AC_BodyPart.UpdateHair` BodyParts)
      (`/Game/Blueprints/Animations/AC_BodyPart.UpdateSkin` BodyParts)
      (`/Game/Blueprints/Animations/AC_BodyPart.UpdateBeard` BodyParts)
      (`/Game/Blueprints/Animations/AC_BodyPart.UpdateBrows` BodyParts)
      (`/Game/Blueprints/Animations/AC_BodyPart.UpdateEyes` BodyParts)
      (`/Game/Blueprints/Animations/AC_BodyPart.UpdateMouth` BodyParts))))

(fn `LoadControls`
  (params (Data :type "/Game/Blueprints/SaveLoad/Components/Local/S_SAVE_Controls Structure") (Character :type "/Game/Player/BP_Character Object Reference"))
  (bind _camera (`/Game/Player/BP_Character.Camera` Character))
  (bind (_relativelocation_x _relativelocation_y) (`KismetMathLibrary.BreakVector` (`SceneComponent.RelativeLocation` _camera)))
  (set `/Game/Player/BP_Character.defaultSpringArmLength` Data_CameraArmLen_18_178BE26741843C683FB829A977834384 Character)
  (`SceneComponent.K2_SetRelativeLocation` _camera (`KismetMathLibrary.MakeVector` _relativelocation_x _relativelocation_y Data_CameraArmHeight_20_369E99B449E29313734AB489867CB93C) false false))

(fn `LoadEquipment`
  (params (Data :type "/Game/Blueprints/SaveLoad/Components/S_SAVE_EQUIP_COMP Structure") (Equipment :type "/Game/Blueprints/StorageSystem/AC_Equipment Object Reference") (__WorldContext :type "Object Object Reference"))
  (bind _enumvalue (foreach `/Game/Data/Equipment/E_EquipmentSlot` false)
    (:`LoopBody`
      (bind _returnvalue (`KismetSystemLibrary.MakeLiteralByte` _enumvalue))
      (if (not (or (== _returnvalue (`KismetSystemLibrary.MakeLiteralByte` (enumliteral `/Game/Data/Equipment/E_EquipmentSlot` "NewEnumerator10"))) (== _returnvalue (`KismetSystemLibrary.MakeLiteralByte` (enumliteral `/Game/Data/Equipment/E_EquipmentSlot` "NewEnumerator9")))))
        (bind _result (`self.DeSerializeItem` (`BlueprintMapLibrary.Map_Find` Data_Items_6_1AB256804185040896AB71A7E7C98965 _enumvalue) (`local.__WorldContext`)))
        (`/Game/Blueprints/StorageSystem/AC_BaseStorage.SetSlot` Equipment (`KismetMathLibrary.Conv_ByteToInt` _enumvalue) _result false)))
    (:`then`
      (`/Game/Blueprints/StorageSystem/AC_Equipment.UpdateItemsOnBody` Equipment))))

(fn `LoadInventory`
  (params (Data :type "/Game/Blueprints/SaveLoad/Components/S_SAVE_STORAGE_COMP Structure") (Storage :type "/Game/Blueprints/StorageSystem/AC_ItemStorage Object Reference") (__WorldContext :type "Object Object Reference"))
  (`KismetArrayLibrary.Array_Resize` (`/Game/Blueprints/StorageSystem/AC_ItemStorage.Items` Storage) (`KismetArrayLibrary.Array_Length` Data_Items_3_1AB256804185040896AB71A7E7C98965))
  (for (_array_element _array_index) Data_Items_3_1AB256804185040896AB71A7E7C98965
    (bind _result (`self.DeSerializeItem` _array_element))
    (`/Game/Blueprints/StorageSystem/AC_BaseStorage.SetSlot` Storage _array_index _result false)))

(fn `LoadPanel`
  (params (Data :type "/Game/Blueprints/SaveLoad/Components/S_SAVE_PANEL_COMP Structure") (Panel :type "/Game/Blueprints/StorageSystem/Panel/AC_Panel Object Reference") (__WorldContext :type "Object Object Reference"))
  (locals (SavedPanel :type "/Game/Blueprints/SaveLoad/Base/S_SAVE_ITEM_PANEL Structure"))
  (bind _returnvalue (`KismetArrayLibrary.Array_Length` Data_Skills_7_F4B67D0A4CC32A437770948058F454D6))
  (bind _returnvalue_2 (`KismetArrayLibrary.Array_Length` Data_Items_6_1AB256804185040896AB71A7E7C98965))
  (`/Game/Blueprints/StorageSystem/Panel/AC_Panel.InitPanels` Panel (`KismetMathLibrary.Clamp` _returnvalue_2 1 _returnvalue_2) (`KismetMathLibrary.Clamp` _returnvalue 1 _returnvalue))
  (`|ExecutionSequence`
    (:`then_0`
      (for (_array_element _array_index) Data_Items_6_1AB256804185040896AB71A7E7C98965
        (bind _output (`|GetArrayItem` (`/Game/Blueprints/StorageSystem/Panel/AC_Panel.ItemPanels` (`local.Panel`)) _array_index))
        (set `/Game/Blueprints/StorageSystem/Panel/AC_ItemPanel.ActiveSlots` (break `/Game/Blueprints/SaveLoad/Base/S_SAVE_ITEM_PANEL` _array_element) _output)
        (for (_array_element_2 _array_index_2) (`.Items_6_96C621984348006F8BD5F7AD0E7C9C23` (break `/Game/Blueprints/SaveLoad/Base/S_SAVE_ITEM_PANEL` _array_element))
          (if (< _array_index_2 10)
            (bind _result (`self.DeSerializeItem` _array_element_2))
            (`/Game/Blueprints/StorageSystem/AC_BaseStorage.SetSlot` _output _array_index_2 _result false)))))
    (:`then_1`
      (for (_array_element_3 _array_index_3) Data_Skills_7_F4B67D0A4CC32A437770948058F454D6
        (bind _output_2 (`|GetArrayItem` (`/Game/Blueprints/StorageSystem/Panel/AC_Panel.SkillPanels` (`local.Panel`)) _array_index_3))
        (set `/Game/Blueprints/StorageSystem/Panel/AC_SkillsPanel.ActiveSlots` (break `/Game/Blueprints/SaveLoad/Base/S_SAVE_SKILL_PANEL` _array_element_3) _output_2)
        (for (_array_element_4 _array_index_4) (`.Items_7_96C621984348006F8BD5F7AD0E7C9C23` (break `/Game/Blueprints/SaveLoad/Base/S_SAVE_SKILL_PANEL` _array_element_3))
          (`/Game/Blueprints/StorageSystem/Panel/AC_SkillsPanel.SetSkill` _output_2 _array_element_4 _array_index_4)))
      (set `/Game/Blueprints/StorageSystem/Panel/AC_Panel.ActivePanelIndex` Data_Index_11_264C61184375C4E9149A748942BB2123 Panel))))

(fn `LoadPlayer`
  (params (Player :type "/Game/Player/BP_Character Object Reference") (Data :type "/Game/Blueprints/SaveLoad/S_SAVE_PLAYER Structure"))
  (locals (Slot :type "/Game/Blueprints/SaveLoad/SG_Player Object Reference"))
  (bind _player (`local.Player`))
  (bind _ac_equipment (`/Game/Player/BP_Character.AC_Equipment` (`local.Player`)))
  (bind _ac_skills (`/Game/Player/BP_Character.AC_Skills` _player))
  (set `/Game/Player/BP_Character.name` Data_name_2_2FAB487840E34E1449DA47A8D4F36934 Player)
  (`Actor.K2_SetActorLocation` Player Data_Pos_23_D31EBF4F45B973E46C6661A3FF34FE6F false false)
  (`Actor.K2_SetActorRotation` Player Data_R_22_18C731EE4B160D5BD4CDBF8D4058D0D9 false)
  (`Controller.SetControlRotation` (`Pawn.GetController` Player) Data_ControlR_26_5EB5688F4A86E1E98F2B13959604734A)
  (`self.LoadSkills` Data_Skill_5_71B0521B4CDAFD91DB907AAD5FD78CD6 Data_SkillTree_15_4C66B4EF492756A65BD9A4932A85F3FA _ac_skills (`/Game/Player/BP_Character.AC_SkillTrees` _player))
  (`self.LoadInventory` Data_Storage_16_A95D50C541A7DA2AC9CFF9A5323CD247 (`/Game/Player/BP_Character.AC_ItemStorage` (`local.Player`)))
  (`self.LoadPanel` Data_Panel_17_4EB1A0CC4CA9857A11DB0FB0737B9D87 (`/Game/Player/BP_Character.AC_Panel` (`local.Player`)))
  (`self.LoadEquipment` Data_Equip_14_E9B699BB4B5AEF8FFD0F65923AA6C0F5 _ac_equipment)
  (`/Game/Blueprints/StorageSystem/AC_Equipment.UpdateHands` _ac_equipment)
  (`self.LoadBodyParts` Data_BodyParts_32_8453C8994281EA703249049B26549DB2 (`/Game/Player/BP_Character.AC_BodyPart` (`local.Player`)))
  (bind _keys (`BlueprintMapLibrary.Map_Keys` (`/Game/Blueprints/SkillSystem/AC_SkillComponent.AttributeSet` _ac_skills)))
  (for _array_element _keys
    (`/Game/Blueprints/SkillSystem/AC_SkillComponent.ReCalculateAttribute` _ac_skills _array_element))
  (`Character.LaunchCharacter` Player Data_Velocity_35_9CEB51AA4E31492AC1FCD9B395AB1BCB false false))

(fn `LoadSkills`
  (params (SkillsData :type "/Game/Blueprints/SaveLoad/Components/S_SAVE_SKILL_COMP Structure") (SkillTreeData :type "/Game/Blueprints/SaveLoad/Components/S_SAVE_SKILL_TREE_COMP Structure") (Skills :type "/Game/Blueprints/SkillSystem/AC_SkillComponent Object Reference") (SkillTrees :type "/Game/Blueprints/SkillSystem/AC_SkillTrees Object Reference") (__WorldContext :type "Object Object Reference"))
  (bind (_attributes _effects _bars _buff) (break `/Game/Blueprints/SaveLoad/Components/S_SAVE_SKILL_COMP` SkillsData))
  (`|ExecutionSequence`
    (:`then_0`
      (set `/Game/Blueprints/SkillSystem/AC_SkillTrees.OwnedSkills` SkillTreeData_OwnedSkills_8_56C16FE448452F6FAEAB24A9854173FC (`local.SkillTrees`))
      (bind (_keypin _valuepin) (`|MapForEach` _attributes)
        (:`then`
          (`BlueprintMapLibrary.Map_Add` (`/Game/Blueprints/SkillSystem/AC_SkillComponent.AttributeSet` Skills) _keypin (make `/Game/Blueprints/SkillSystem/S_Attribute` 0.0 _valuepin)))
        (:`CompletedPin`
          (for _array_element _effects
            (`/Game/Blueprints/SkillSystem/AC_SkillComponent.ApplyEffect` (`local.Skills`) (break `/Game/Data/Skills/S_Effect` _array_element) (`.Data_18_F4CAC80D4078950697773C830D0E8E3E` (break `/Game/Data/Skills/S_Effect` _array_element)) (`.Duration_10_09701A1B46A9128048DFD3A7339C3312` (break `/Game/Data/Skills/S_Effect` _array_element))))
          (for _array_element_2 _buff
            (`/Game/Blueprints/SkillSystem/AC_SkillComponent.ApplyBuff` (`local.Skills`) (break `/Game/Blueprints/SaveLoad/Skill/S_SAVE_BUFF` _array_element_2) (`.Data_11_7B969E46491D473B1D8ADB88B9EB184D` (break `/Game/Blueprints/SaveLoad/Skill/S_SAVE_BUFF` _array_element_2)) (`.target_14_D55524054EDF5D7EDFBBBEAE7BD30370` (break `/Game/Blueprints/SaveLoad/Skill/S_SAVE_BUFF` _array_element_2)) (`.Duration_5_7A12DC194B43675F4F859D8142F82291` (break `/Game/Blueprints/SaveLoad/Skill/S_SAVE_BUFF` _array_element_2)) (`.Name_20_668F53304A0963C4F9D0DC8527AC8323` (break `/Game/Blueprints/SaveLoad/Skill/S_SAVE_BUFF` _array_element_2))))
          (for _array_element_3 _bars
            (`/Game/Blueprints/SkillSystem/AC_SkillComponent.ApplyBarEffect` (`local.Skills`) (break `/Game/Blueprints/SaveLoad/Skill/S_SAVE_BAR` _array_element_3) (`.Value_10_7A12DC194B43675F4F859D8142F82291` (break `/Game/Blueprints/SaveLoad/Skill/S_SAVE_BAR` _array_element_3)) (`.Data_19_BA08F5C54BD117B0D0483DA248D433FA` (break `/Game/Blueprints/SaveLoad/Skill/S_SAVE_BAR` _array_element_3)))))))
    (:`then_1`
      (set `/Game/Blueprints/SkillSystem/AC_SkillTrees.SkillPoints` SkillTreeData_SkillPoints_4_1AB256804185040896AB71A7E7C98965 SkillTrees)
      (`/Game/Blueprints/SkillSystem/AC_SkillComponent.ReCalculateAll` Skills))))

(fn `LoadUI`
  (params (Data :type "/Game/Blueprints/SaveLoad/Components/Local/S_SAVE_UI Structure") (UIManager :type "/Game/UI/AC_UIManager Object Reference") (__WorldContext :type "Object Object Reference"))
  (bind _inventory (`/Game/UI/AC_UIManager.Inventory` UIManager))
  (bind _equipment (`/Game/UI/AC_UIManager.Equipment` UIManager))
  (`/Game/UI/AC_UIManager.Init` UIManager)
  (`UserWidget.SetPositionInViewport` _inventory Data_Invent_11_BB85BD084CEE7003ED95D0B1D6FD76E1 true)
  (`/Game/UI/UW_DragableWidget.SetSize` _inventory Data_InventSize_16_61609CDB4EB2133B8348E5AAAC59BB6B)
  (set `/Game/UI/UW_DragableWidget.CurPos` Data_Invent_11_BB85BD084CEE7003ED95D0B1D6FD76E1 _inventory)
  (`UserWidget.SetPositionInViewport` _equipment Data_Equip_10_1AB256804185040896AB71A7E7C98965 true)
  (set `/Game/UI/UW_DragableWidget.CurPos` Data_Equip_10_1AB256804185040896AB71A7E7C98965 _equipment)
  (`/Game/UI/UW_DragableWidget.SetSize` _equipment Data_EquipSize_14_8725C37148E655E3E0917BAF28ADDA4A)
  (`/Game/UI/Panel/UW_PanelHolder.SetSize` (`/Game/UI/AC_UIManager.Panel` UIManager) Data_PanelSize_23_26C47B154994B99B8809D799F9F4D146))

(fn `SaveBodyParts`
  (params (BodyParts :type "/Game/Blueprints/Animations/AC_BodyPart Object Reference"))
  (returns (Data :type "/Game/Blueprints/SaveLoad/Components/S_SAVE_BODY_PARTS_COMP Structure"))
  (return (make `/Game/Blueprints/SaveLoad/Components/S_SAVE_BODY_PARTS_COMP` (`/Game/Blueprints/Animations/AC_BodyPart.BodyType` BodyParts) (`/Game/Blueprints/Animations/AC_BodyPart.BrowsName` BodyParts) (`/Game/Blueprints/Animations/AC_BodyPart.EyesName` BodyParts) (`/Game/Blueprints/Animations/AC_BodyPart.MouthName` BodyParts) (`/Game/Blueprints/Animations/AC_BodyPart.HairName` BodyParts) (`/Game/Blueprints/Animations/AC_BodyPart.BeardName` BodyParts) (`/Game/Blueprints/Animations/AC_BodyPart.PuplisColor` BodyParts) (`/Game/Blueprints/Animations/AC_BodyPart.BrowsColor` BodyParts) (`/Game/Blueprints/Animations/AC_BodyPart.BeardColor` BodyParts) (`/Game/Blueprints/Animations/AC_BodyPart.Skin Color` BodyParts) (`/Game/Blueprints/Animations/AC_BodyPart.HairColor` BodyParts))))

(fn `SaveEquipment`
  (params (Equipment :type "/Game/Blueprints/StorageSystem/AC_Equipment Object Reference"))
  (returns (Data :type "/Game/Blueprints/SaveLoad/Components/S_SAVE_EQUIP_COMP Structure"))
  (locals (Result :type "Map of /Game/Data/Equipment/E_EquipmentSlot Enum to /Game/Blueprints/SaveLoad/Base/S_SAVE_DATA_ITEM Structure"))
  (bind _result (`local.Result`))
  (bind _enumvalue (foreach `/Game/Data/Equipment/E_EquipmentSlot` false)
    (:`LoopBody`
      (bind _item (`/Game/Blueprints/StorageSystem/AC_BaseStorage.GetSlot` Equipment (`KismetMathLibrary.Conv_ByteToInt` _enumvalue)))
      (`/Engine/EditorBlueprintResources/StandardMacros.IsValid` _item
        (:`Is Valid`
          (bind _result_2 (`/Game/Data/O_Item.Serialize` _item))
          (`BlueprintMapLibrary.Map_Add` _result _enumvalue _result_2))
        (:`Is Not Valid`
          (`BlueprintMapLibrary.Map_Add` _result _enumvalue (make `/Game/Blueprints/SaveLoad/Base/S_SAVE_DATA_ITEM` "air")))))
    (:`then`
      (return (make `/Game/Blueprints/SaveLoad/Components/S_SAVE_EQUIP_COMP` _result)))))

(fn `SaveInventory`
  (params (Storage :type "/Game/Blueprints/StorageSystem/AC_ItemStorage Object Reference"))
  (returns (Data :type "/Game/Blueprints/SaveLoad/Components/S_SAVE_STORAGE_COMP Structure"))
  (locals (Result :type "Array of /Game/Blueprints/SaveLoad/Base/S_SAVE_DATA_ITEM Structure"))
  (bind _result (`local.Result`))
  (for _array_element (`/Game/Blueprints/StorageSystem/AC_ItemStorage.Items` Storage)
    (`/Engine/EditorBlueprintResources/StandardMacros.IsValid` _array_element
      (:`Is Valid`
        (bind _result_2 (`/Game/Data/O_Item.Serialize` _array_element))
        (`KismetArrayLibrary.Array_Add` _result _result_2))
      (:`Is Not Valid`
        (`KismetArrayLibrary.Array_Add` _result))))
  (return (make `/Game/Blueprints/SaveLoad/Components/S_SAVE_STORAGE_COMP` _result)))

(fn `SavePanel`
  (params (Panel :type "/Game/Blueprints/StorageSystem/Panel/AC_Panel Object Reference"))
  (returns (Data :type "/Game/Blueprints/SaveLoad/Components/S_SAVE_PANEL_COMP Structure"))
  (locals (SavedPanel :type "/Game/Blueprints/SaveLoad/Base/S_SAVE_ITEM_PANEL Structure") (SkillsAr :type "Array of GameplayTag Structure") (ItemsPanels :type "Array of /Game/Blueprints/SaveLoad/Base/S_SAVE_ITEM_PANEL Structure") (SkillsPanels :type "Array of /Game/Blueprints/SaveLoad/Base/S_SAVE_SKILL_PANEL Structure") (Items :type "Array of /Game/Blueprints/SaveLoad/Base/S_SAVE_DATA_ITEM Structure"))
  (bind _items (`local.Items`))
  (bind _skillsar (`local.SkillsAr`))
  (`|ExecutionSequence`
    (:`then_0`
      (for _array_element (`/Game/Blueprints/StorageSystem/Panel/AC_Panel.ItemPanels` Panel)
        (set `local.SavedPanel` (make `/Game/Blueprints/SaveLoad/Base/S_SAVE_ITEM_PANEL` (struct)))
        (for (_array_element_2 _array_index) (`/Game/Blueprints/StorageSystem/AC_ItemStorage.Items` _array_element)
          (if (< _array_index 10)
            (bind _result (`/Game/Data/O_Item.Serialize` _array_element_2))
            (`KismetArrayLibrary.Array_Add` _items _result)))
        (`KismetArrayLibrary.Array_Add` (`local.ItemsPanels`) (make `/Game/Blueprints/SaveLoad/Base/S_SAVE_ITEM_PANEL` (`/Game/Blueprints/StorageSystem/Panel/AC_ItemPanel.ActiveSlots` _array_element) _items))))
    (:`then_1`
      (for _array_element_3 (`/Game/Blueprints/StorageSystem/Panel/AC_Panel.SkillPanels` Panel)
        (`KismetArrayLibrary.Array_Clear` _skillsar)
        (for (_array_element_4 _array_index_2) (`/Game/Blueprints/StorageSystem/Panel/AC_SkillsPanel.Skills` _array_element_3)
          (if (< _array_index_2 10)
            (`KismetArrayLibrary.Array_Add` _skillsar (`/Game/Data/O_Skill.Tag` _array_element_4))))
        (`KismetArrayLibrary.Array_Add` (`local.SkillsPanels`) (make `/Game/Blueprints/SaveLoad/Base/S_SAVE_SKILL_PANEL` (`/Game/Blueprints/StorageSystem/Panel/AC_SkillsPanel.ActiveSlots` _array_element_3) _skillsar))))
    (:`then_2`
      (return (make `/Game/Blueprints/SaveLoad/Components/S_SAVE_PANEL_COMP` (`local.ItemsPanels`) (`local.SkillsPanels`) (`/Game/Blueprints/StorageSystem/Panel/AC_Panel.ActivePanelIndex` Panel))))))

(fn `SavePlayer`
  (params (Player :type "/Game/Player/BP_Character Object Reference"))
  (returns (Result :type "/Game/Blueprints/SaveLoad/S_SAVE_PLAYER Structure"))
  (bind _player (`local.Player`))
  (bind _data (`self.SaveInventory` (`/Game/Player/BP_Character.AC_ItemStorage` (`local.Player`))))
  (bind _data_2 (`self.SaveEquipment` (`/Game/Player/BP_Character.AC_Equipment` (`local.Player`))))
  (bind _data_3 (`self.SavePanel` (`/Game/Player/BP_Character.AC_Panel` (`local.Player`))))
  (bind (_skill _skilstrees) (`self.SaveSkills` (`/Game/Player/BP_Character.AC_Skills` _player) (`/Game/Player/BP_Character.AC_SkillTrees` _player)))
  (bind _data_4 (`self.SaveBodyParts` (`/Game/Player/BP_Character.AC_BodyPart` _player)))
  (return (make `/Game/Blueprints/SaveLoad/S_SAVE_PLAYER` (`KismetStringLibrary.Conv_StringToName` (`/Game/Player/BP_Character.Player Name` Player)) _skill _data_2 _skilstrees _data _data_3 _data_4 (`Actor.K2_GetActorLocation` Player) (`Actor.K2_GetActorRotation` Player) (`Pawn.GetControlRotation` Player) (`Actor.GetVelocity` Player))))

(fn `SaveSkills`
  (params (SkillComp :type "/Game/Blueprints/SkillSystem/AC_SkillComponent Object Reference") (SkillTreeComp :type "/Game/Blueprints/SkillSystem/AC_SkillTrees Object Reference"))
  (returns (Skill :type "/Game/Blueprints/SaveLoad/Components/S_SAVE_SKILL_COMP Structure") (SkilsTrees :type "/Game/Blueprints/SaveLoad/Components/S_SAVE_SKILL_TREE_COMP Structure"))
  (locals (SavedAttrs :type "Map of GameplayTag Structure to Float (double-precision)") (SavedEffects :type "Array of /Game/Data/Skills/S_Effect Structure") (SavedBuffs :type "Array of /Game/Blueprints/SaveLoad/Skill/S_SAVE_BUFF Structure") (SavedBars :type "Array of /Game/Blueprints/SaveLoad/Skill/S_SAVE_BAR Structure"))
  (`|ExecutionSequence`
    (:`then_0`
      (bind (_keypin _valuepin) (`|MapForEach` (`/Game/Blueprints/SkillSystem/AC_SkillComponent.AttributeSet` SkillComp))
        (:`then`
          (`BlueprintMapLibrary.Map_Add` (`local.SavedAttrs`) _keypin (`.Base_27_6D5926F0445AB5B78ECF7D85052FB2B0` (break `/Game/Blueprints/SkillSystem/S_Attribute` _valuepin))))
        (:`CompletedPin`
          (for _array_element (`/Game/Blueprints/SkillSystem/AC_SkillComponent.Effects` SkillComp)
            (if (`/Game/Blueprints/SkillSystem/A_SkillBase.save_load` _array_element)
              (bind _metadata (`/Game/Blueprints/SkillSystem/A_SkillBase.Save` _array_element))
              (bind _duration (`/Game/Blueprints/SkillSystem/Effects/_A_EffectBase.Duration` _array_element))
              (`KismetArrayLibrary.Array_Add` (`local.SavedEffects`) (make `/Game/Data/Skills/S_Effect` (`GameplayStatics.GetObjectClass` _array_element) _metadata (`KismetMathLibrary.SelectFloat` -1.0 (- _duration (- (`KismetSystemLibrary.GetGameTimeInSeconds` _array_element) (`/Game/Blueprints/SkillSystem/A_SkillBase.SkillCreated` _array_element))) (== _duration -1.0))))))
          (bind _values (`BlueprintMapLibrary.Map_Values` (`/Game/Blueprints/SkillSystem/AC_SkillComponent.Buffs` SkillComp)))
          (for _array_element_2 _values
            (bind _values_2 (`BlueprintMapLibrary.Map_Values` (break `/Game/Blueprints/SkillSystem/Buffs/S_BuffsMap` _array_element_2)))
            (for _array_element_3 _values_2
              (for _array_element_4 (break `/Game/Blueprints/SkillSystem/Buffs/S_BuffsArray` _array_element_3)
                (if (`/Game/Blueprints/SkillSystem/A_SkillBase.save_load` _array_element_4)
                  (bind _metadata_2 (`/Game/Blueprints/SkillSystem/A_SkillBase.Save` _array_element_4))
                  (bind _duration_2 (`/Game/Blueprints/SkillSystem/Buffs/_ASB_Buff.Duration` _array_element_4))
                  (`KismetArrayLibrary.Array_Add` (`local.SavedBuffs`) (make `/Game/Blueprints/SaveLoad/Skill/S_SAVE_BUFF` (`GameplayStatics.GetObjectClass` _array_element_4) _metadata_2 (`/Game/Blueprints/SkillSystem/Buffs/_ASB_Buff.PreviewTitle` _array_element_4) (`KismetMathLibrary.SelectFloat` _duration_2 (- _duration_2 (- (`KismetSystemLibrary.GetGameTimeInSeconds` null) (`/Game/Blueprints/SkillSystem/A_SkillBase.SkillCreated` _array_element_4))) (== _duration_2 -1.0)) (`/Game/Blueprints/SkillSystem/Buffs/_ASB_Buff.TargetedAttribute` _array_element_4)))))))
          (for _array_element_5 (`/Game/Blueprints/SkillSystem/AC_SkillComponent.EffectBars` SkillComp)
            (if (`/Game/Blueprints/SkillSystem/A_SkillBase.save_load` _array_element_5)
              (bind _metadata_3 (`/Game/Blueprints/SkillSystem/A_SkillBase.Save` _array_element_5))
              (`KismetArrayLibrary.Array_Add` (`local.SavedBars`) (make `/Game/Blueprints/SaveLoad/Skill/S_SAVE_BAR` (`GameplayStatics.GetObjectClass` _array_element_5) _metadata_3 (`/Game/Blueprints/SkillSystem/Bars/_AEB_EffectBarBase.CurrentPoints` _array_element_5))))))))
    (:`then_1`
      (return (make `/Game/Blueprints/SaveLoad/Components/S_SAVE_SKILL_COMP` (`local.SavedAttrs`) (`local.SavedEffects`) (`local.SavedBars`) (`local.SavedBuffs`)) (make `/Game/Blueprints/SaveLoad/Components/S_SAVE_SKILL_TREE_COMP` (`/Game/Blueprints/SkillSystem/AC_SkillTrees.SkillPoints` SkillTreeComp) (`/Game/Blueprints/SkillSystem/AC_SkillTrees.OwnedSkills` SkillTreeComp))))))

(fn `SaveUI`
  (params (UIManager :type "/Game/UI/AC_UIManager Object Reference"))
  (returns (Data :type "/Game/Blueprints/SaveLoad/Components/Local/S_SAVE_UI Structure"))
  (bind _inventory (`/Game/UI/AC_UIManager.Inventory` UIManager))
  (bind _equipment (`/Game/UI/AC_UIManager.Equipment` UIManager))
  (`/Engine/EditorBlueprintResources/StandardMacros.IsValid` UIManager
    (:`Is Valid`
      (`/Engine/EditorBlueprintResources/StandardMacros.IsValid` _equipment
        (:`Is Valid`
          (return (make `/Game/Blueprints/SaveLoad/Components/Local/S_SAVE_UI` (`/Game/UI/UW_DragableWidget.CurPos` _equipment) (`/Game/UI/UW_DragableWidget.CurPos` _inventory) (`/Game/UI/UW_DragableWidget.CurSize` _equipment) (`/Game/UI/UW_DragableWidget.CurSize` _inventory) (`/Game/UI/Panel/UW_PanelHolder.CurSize` (`/Game/UI/AC_UIManager.Panel` UIManager)))))))
    (:`Is Not Valid`
      (return (make `/Game/Blueprints/SaveLoad/Components/Local/S_SAVE_UI` (0.0 0.0))))))