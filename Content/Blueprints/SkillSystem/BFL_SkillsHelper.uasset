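; Function library for the skill system, with helpers for attribute edits, gameplay-tag damage maps and hand-string parsing.
; Damage maps pack into delimited strings (Magic tags written as Attack) and parse back by tag name.
; Armour and parry subtract per damage type, with a full-resist sentinel and diminishing chip damage on armour; magic damage comes from component buffs.
; SetSkillComp rebuilds a component's effects, buffs, attributes and bars from data, recalculating attributes.
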(fn `Add`
  (params (Attribute :type "/Game/Blueprints/SkillSystem/S_Attribute Structure") (Value :type "Float (double-precision)"))
  (returns (Result :type "/Game/Blueprints/SkillSystem/S_Attribute Structure"))
  (bind (_min _base _current _max) (break `/Game/Blueprints/SkillSystem/S_Attribute` Attribute))
  (return (make `/Game/Blueprints/SkillSystem/S_Attribute` _min (+ _base Value) _current _max)))

(fn `AddMagicDamage`
  (params (BaseDamage :type "Map of GameplayTag Structure to Float (double-precision)") (Comp :type "/Game/Blueprints/SkillSystem/AC_SkillComponent Object Reference") (Multiplyer :type "Float (double-precision)"))
  (returns (Result :type "Map of GameplayTag Structure to Float (double-precision)"))
  (locals (Dmg :type "Map of GameplayTag Structure to Float (double-precision)"))
  (bind _output_get (set `local.Dmg` BaseDamage))
  (for _array_element (`|MakeArray` (struct :`TagName` "Attributes.Magic.Clear") (struct :`TagName` "Attributes.Magic.Cutting") (struct :`TagName` "Attributes.Magic.Electrical") (struct :`TagName` "Attributes.Magic.Fire") (struct :`TagName` "Attributes.Magic.Frost") (struct :`TagName` "Attributes.Magic.Physic") (struct :`TagName` "Attributes.Magic.Piercing") (struct :`TagName` "Attributes.Magic.Poison") (struct :`TagName` "Attributes.Magic.Radiation") (struct :`TagName` "Attributes.Magic.Silver") (struct :`TagName` "Attributes.Magic.Water") :!type "GameplayTag Structure")
    (bind (_value _returnvalue) (`BlueprintMapLibrary.Map_Find` _output_get _array_element))
    (bind _result (`/Game/Blueprints/SkillSystem/AC_SkillComponent.CalculateBuff` Comp _array_element (`KismetMathLibrary.SelectFloat` _value 0.0 _returnvalue)))
    (if (not (== (`.Current_22_E11334934F74221D85B0C0AA8D87BE62` (break `/Game/Blueprints/SkillSystem/S_Attribute` _result)) 0.0))
      (`BlueprintMapLibrary.Map_Add` _output_get _array_element (* (`.Current_22_E11334934F74221D85B0C0AA8D87BE62` (break `/Game/Blueprints/SkillSystem/S_Attribute` _result)) Multiplyer))))
  (return (`local.Dmg`)))

(fn `AddWithClamp`
  (params (Attribute :type "/Game/Blueprints/SkillSystem/S_Attribute Structure") (Value :type "Float (double-precision)"))
  (returns (Result :type "/Game/Blueprints/SkillSystem/S_Attribute Structure"))
  (bind (_min _base _current _max) (break `/Game/Blueprints/SkillSystem/S_Attribute` Attribute))
  (return (make `/Game/Blueprints/SkillSystem/S_Attribute` _min (`KismetMathLibrary.FClamp` (+ _base Value) _min _max) _current _max)))

(fn `AttributeToString`
  (params (Attribute :type "/Game/Blueprints/SkillSystem/S_Attribute Structure"))
  (returns (Min :type String) (Value :type String) (Max :type String) (Full :type String))
  (bind _returnvalue (`KismetStringLibrary.Conv_DoubleToString` Attribute_Min_23_4A73B71648212DC5C33B30AD659F9A21))
  (bind _returnvalue_2 (`KismetStringLibrary.Conv_DoubleToString` Attribute_Current_22_E11334934F74221D85B0C0AA8D87BE62))
  (bind _returnvalue_3 (`KismetStringLibrary.Conv_DoubleToString` Attribute_Max_24_B52313574BD363B2E33D4CBBE239C895))
  (return _returnvalue _returnvalue_2 _returnvalue_3 (`KismetStringLibrary.Concat_StrStr` _returnvalue " " _returnvalue_2 " " _returnvalue_3)))

(fn `DamageToString`
  (params (TargetMap :type "Map of GameplayTag Structure to Float (double-precision) (by ref)"))
  (returns (ReturnValue :type String))
  (locals (Str :type String))
  (bind _keys (`BlueprintMapLibrary.Map_Keys` TargetMap))
  (for (_array_element _array_index) _keys
    (set `local.Str` (`KismetStringLibrary.Concat_StrStr` (`local.Str`) (`.RightS` (`KismetStringLibrary.Split` (`BlueprintGameplayTagLibrary.GetDebugStringFromGameplayTag` _array_element) "." "IgnoreCase" "FromEnd")) " " (`KismetStringLibrary.Split` (`KismetStringLibrary.Conv_DoubleToString` (`BlueprintMapLibrary.Map_Find` TargetMap _array_element)) ".0" "IgnoreCase" "FromEnd") (`KismetMathLibrary.SelectString` "" " \n" (== _array_index (- (`KismetArrayLibrary.Array_Length` _keys) 1))))))
  (return (`local.Str`)))

(fn `DeSerializeDamage`
  (params (Val :type String))
  (returns (ResTag :type "GameplayTag Structure") (Result :type "Map of GameplayTag Structure to Float (double-precision)"))
  (locals (Cur :type String) (Tag :type "GameplayTag Structure") (Res :type "Map of GameplayTag Structure to Float (double-precision)") (ResTag1 :type "GameplayTag Structure") (SplittedDmg :type String))
  (bind (_lefts _rights) (`KismetStringLibrary.Split` Val "|"))
  (bind _splitteddmg (`local.SplittedDmg`))
  (bind (_lefts_2 _rights_2 _returnvalue) (`KismetStringLibrary.Split` (`local.Cur`) "|"))
  (`|ExecutionSequence`
    (:`then_0`
      (switch `string` _lefts
        (:`Attributes.Base.Health`
          (set `local.ResTag1` (struct :`TagName` "Attributes.Base.Health")))
        (:`Attributes.Base.Stamina`
          (set `local.ResTag1` (struct :`TagName` "Attributes.Base.Stamina")))
        (:`Attributes.Base.Mana`
          (set `local.ResTag1` (struct :`TagName` "Attributes.Base.Mana")))))
    (:`then_1`
      (set `local.Cur` _rights)
      (while _returnvalue
        (bind _output_get (set `local.SplittedDmg` _lefts_2))
        (set `local.Cur` _rights_2)
        (`|ExecutionSequence`
          (:`then_0`
            (bind (_lefts_3 _rights_3) (`KismetStringLibrary.Split` _output_get "\\"))
            (set `local.SplittedDmg` _lefts_3)
            (switch `string` _splitteddmg
              (:`Default`
                (`KismetSystemLibrary.PrintString` null (`KismetStringLibrary.Concat_StrStr` "SKILL_HELPER - Unknown damage type - " _splitteddmg)))
              (:`Attributes.Attack.Clear`
                (set `local.Tag` (struct :`TagName` "Attributes.Attack.Clear")))
              (:`Attributes.Attack.Cutting`
                (set `local.Tag` (struct :`TagName` "Attributes.Attack.Cutting")))
              (:`Attributes.Attack.Electrical`
                (set `local.Tag` (struct :`TagName` "Attributes.Attack.Electrical")))
              (:`Attributes.Attack.FallDamage`
                (set `local.Tag` (struct :`TagName` "Attributes.Attack.FallDamage")))
              (:`Attributes.Attack.Fire`
                (set `local.Tag` (struct :`TagName` "Attributes.Attack.Fire")))
              (:`Attributes.Attack.Frost`
                (set `local.Tag` (struct :`TagName` "Attributes.Attack.Frost")))
              (:`Attributes.Attack.Physic`
                (set `local.Tag` (struct :`TagName` "Attributes.Attack.Physic")))
              (:`Attributes.Attack.Piercing`
                (set `local.Tag` (struct :`TagName` "Attributes.Attack.Piercing")))
              (:`Attributes.Attack.Water`
                (set `local.Tag` (struct :`TagName` "Attributes.Attack.Water")))
              (:`Attributes.Attack.Silver`
                (set `local.Tag` (struct :`TagName` "Attributes.Attack.Silver")))
              (:`Attributes.Attack.Radiation`
                (set `local.Tag` (struct :`TagName` "Attributes.Attack.Radiation")))
              (:`Attributes.Attack.Poison`
                (set `local.Tag` (struct :`TagName` "Attributes.Attack.Poison")))
              (:`Attributes.Magic.Clear`
                (set `local.Tag` (struct :`TagName` "Attributes.Magic.Clear")))
              (:`Attributes.Magic.Cutting`
                (set `local.Tag` (struct :`TagName` "Attributes.Magic.Cutting")))
              (:`Attributes.Magic.Electrical`
                (set `local.Tag` (struct :`TagName` "Attributes.Magic.Electrical")))
              (:`Attributes.Magic.Fire`
                (set `local.Tag` (struct :`TagName` "Attributes.Magic.Fire")))
              (:`Attributes.Magic.Frost`
                (set `local.Tag` (struct :`TagName` "Attributes.Magic.Frost")))
              (:`Attributes.Magic.Physic`
                (set `local.Tag` (struct :`TagName` "Attributes.Magic.Physic")))
              (:`Attributes.Magic.Piercing`
                (set `local.Tag` (struct :`TagName` "Attributes.Magic.Piercing")))
              (:`Attributes.Magic.Radiation`
                (set `local.Tag` (struct :`TagName` "Attributes.Magic.Radiation")))
              (:`Attributes.Magic.Silver`
                (set `local.Tag` (struct :`TagName` "Attributes.Magic.Silver")))
              (:`Attributes.Magic.Water`
                (set `local.Tag` (struct :`TagName` "Attributes.Magic.Water")))
              (:`Attributes.Magic.Poison`
                (set `local.Tag` (struct :`TagName` "Attributes.Magic.Poison")))))
          (:`then_1`
            (`BlueprintMapLibrary.Map_Add` (`local.Res`) (`local.Tag`) (`KismetStringLibrary.Conv_StringToDouble` _rights_3)))))
      (return (`local.ResTag1`) (`local.Res`)))))

(fn `DeSerializeHand`
  (params (SearchIn :type String))
  (returns (AnimSource :type Name) (Socket :type Name) (twoHands :type Boolean) (right :type Boolean))
  (bind _returnvalue (`KismetStringLibrary.Contains` SearchIn "right"))
  (bind _returnvalue_2 (`KismetStringLibrary.Contains` SearchIn "Two"))
  (return (`KismetMathLibrary.SelectName` "TwoHands" (select `bool` _returnvalue :`false` "LeftHand" :`true` "RightHand" :!type "Name") _returnvalue_2) (select `bool` (or _returnvalue_2 _returnvalue) :`false` "Left_Item_Socket" :`true` "Right_Item_Socket" :!type "Name") _returnvalue_2 _returnvalue))

(fn `GetArmour`
  (params (attributes :type "Map of GameplayTag Structure to /Game/Blueprints/SkillSystem/S_Attribute Structure"))
  (returns (Return :type "Map of GameplayTag Structure to Float (double-precision)"))
  (locals (Res :type "Map of GameplayTag Structure to Float (double-precision)"))
  (bind _res (`local.Res`))
  (bind (_keypin _valuepin) (`|MapForEach` attributes)
    (:`then`
      (`|SwitchGameplayTag` _keypin
        (:`Attributes.Armour.Cutting`
          _)
        (:`Attributes.Armour.Electrical`
          _)
        (:`Attributes.Armour.FallDamage`
          _)
        (:`Attributes.Armour.Fire`
          _)
        (:`Attributes.Armour.Frost`
          _)
        (:`Attributes.Armour.Physic`
          _)
        (:`Attributes.Armour.Piercing`
          _)
        (:`Attributes.Armour.Water`
          _)
        (:`Attributes.Armour.Poison`
          _)
        (:`Attributes.Armour.Radiation`
          _)
        (:`Attributes.Armour.Silver`
          _))
      (`BlueprintMapLibrary.Map_Add` _res _keypin (`.Current_22_E11334934F74221D85B0C0AA8D87BE62` (break `/Game/Blueprints/SkillSystem/S_Attribute` _valuepin))))
    (:`CompletedPin`
      (return _res))))

(fn `ParryDamage`
  (params (Damage :type "Map of GameplayTag Structure to Float (double-precision)") (Parry :type "Map of GameplayTag Structure to Float (double-precision)") (__WorldContext :type "Object Object Reference"))
  (returns (Result :type "Map of GameplayTag Structure to Float (double-precision)"))
  (locals (Res :type "Map of GameplayTag Structure to Float (double-precision)"))
  (bind _returnvalue (`BlueprintGameplayTagLibrary.MakeLiteralGameplayTag` (struct :`TagName` "Attributes.Parry.Frost")))
  (bind _returnvalue_2 (`BlueprintGameplayTagLibrary.MakeLiteralGameplayTag` (struct :`TagName` "Attributes.Parry.Piercing")))
  (bind _returnvalue_3 (`BlueprintGameplayTagLibrary.MakeLiteralGameplayTag` (struct :`TagName` "Attributes.Parry.Electrical")))
  (bind _returnvalue_4 (`BlueprintGameplayTagLibrary.MakeLiteralGameplayTag` (struct :`TagName` "Attributes.Parry.Cutting")))
  (bind _returnvalue_5 (`BlueprintGameplayTagLibrary.MakeLiteralGameplayTag` (struct :`TagName` "Attributes.Parry.Water")))
  (bind _returnvalue_6 (`BlueprintGameplayTagLibrary.MakeLiteralGameplayTag` (struct :`TagName` "Attributes.Parry.Fire")))
  (bind _returnvalue_7 (`BlueprintGameplayTagLibrary.MakeLiteralGameplayTag` (struct :`TagName` "Attributes.Parry.Poison")))
  (bind _returnvalue_8 (`BlueprintGameplayTagLibrary.MakeLiteralGameplayTag` (struct :`TagName` "Attributes.Parry.Silver")))
  (bind _returnvalue_9 (`BlueprintGameplayTagLibrary.MakeLiteralGameplayTag` (struct :`TagName` "Attributes.Parry.Physic")))
  (bind _parry (`local.Parry`))
  (bind _res (`local.Res`))
  (bind (_keypin _valuepin) (`|MapForEach` Damage)
    (:`then`
      (`|SwitchGameplayTag` _keypin
        (:`Attributes.Attack.Clear`
          (`BlueprintMapLibrary.Map_Add` _res _keypin _valuepin :!label _label))
        (:`Attributes.Magic.Clear`
          (goto _label))
        (:`Attributes.Attack.Cutting`
          (`BlueprintMapLibrary.Map_Add` _res _returnvalue_4 (- _valuepin (`BlueprintMapLibrary.Map_Find` _parry _returnvalue_4)) :!label _label_2))
        (:`Attributes.Magic.Cutting`
          (goto _label_2))
        (:`Attributes.Attack.Electrical`
          (`BlueprintMapLibrary.Map_Add` _res _returnvalue_3 (- _valuepin (`BlueprintMapLibrary.Map_Find` _parry _returnvalue_3)) :!label _label_3))
        (:`Attributes.Magic.Electrical`
          (goto _label_3))
        (:`Attributes.Attack.FallDamage`
          (goto _label))
        (:`Attributes.Attack.Fire`
          (`BlueprintMapLibrary.Map_Add` _res _returnvalue_6 (- _valuepin (`BlueprintMapLibrary.Map_Find` _parry _returnvalue_6)) :!label _label_4))
        (:`Attributes.Magic.Fire`
          (goto _label_4))
        (:`Attributes.Attack.Frost`
          (`BlueprintMapLibrary.Map_Add` _res _returnvalue (- _valuepin (`BlueprintMapLibrary.Map_Find` _parry _returnvalue)) :!label _label_5))
        (:`Attributes.Magic.Frost`
          (goto _label_5))
        (:`Attributes.Attack.Physic`
          (`BlueprintMapLibrary.Map_Add` _res _returnvalue_9 (- _valuepin (`BlueprintMapLibrary.Map_Find` _parry _returnvalue_9)) :!label _label_6))
        (:`Attributes.Magic.Physic`
          (goto _label_6))
        (:`Attributes.Attack.Piercing`
          (`BlueprintMapLibrary.Map_Add` _res _returnvalue_2 (- _valuepin (`BlueprintMapLibrary.Map_Find` _parry _returnvalue_2)) :!label _label_7))
        (:`Attributes.Magic.Piercing`
          (goto _label_7))
        (:`Attributes.Attack.Water`
          (`BlueprintMapLibrary.Map_Add` _res _returnvalue_5 (- _valuepin (`BlueprintMapLibrary.Map_Find` _parry _returnvalue_5)) :!label _label_8))
        (:`Attributes.Magic.Water`
          (goto _label_8))
        (:`Attributes.Attack.Poison`
          (`BlueprintMapLibrary.Map_Add` _res _returnvalue_7 (- _valuepin (`BlueprintMapLibrary.Map_Find` _parry _returnvalue_7)) :!label _label_9))
        (:`Attributes.Magic.Poison`
          (goto _label_9))
        (:`Attributes.Attack.Silver`
          (`BlueprintMapLibrary.Map_Add` _res _returnvalue_8 (- _valuepin (`BlueprintMapLibrary.Map_Find` _parry _returnvalue_8)) :!label _label_10))
        (:`Attributes.Magic.Silver`
          (goto _label_10))))
    (:`CompletedPin`
      (return (`local.Res`)))))

(fn `PRINT_DAMAGE`
  (params (Damage :type "Map of GameplayTag Structure to Float (double-precision)"))
  (bind _keys (`BlueprintMapLibrary.Map_Keys` Damage))
  (for _array_element _keys
    (`KismetSystemLibrary.PrintString` null (`KismetStringLibrary.Concat_StrStr` (`BlueprintGameplayTagLibrary.GetDebugStringFromGameplayTag` _array_element) " " (`KismetStringLibrary.Conv_DoubleToString` (`BlueprintMapLibrary.Map_Find` Damage _array_element))))))

(fn `SerializeDamage`
  (params (TargetTag :type "GameplayTag Structure" :default (struct :`TagName` "Attributes.Base.Health")) (Value :type "Map of GameplayTag Structure to Float (double-precision)") (should_draw :type Boolean) (apply_effects :type Boolean) (draw_entities_only :type Boolean))
  (returns (Result :type String))
  (locals (Res :type String))
  (set `local.Res` (`BlueprintGameplayTagLibrary.GetDebugStringFromGameplayTag` TargetTag))
  (bind (_keypin _valuepin) (`|MapForEach` Value)
    (:`then`
      (bind _returnvalue (`BlueprintGameplayTagLibrary.GetDebugStringFromGameplayTag` _keypin))
      (set `local.Res` (`KismetStringLibrary.Concat_StrStr` (`local.Res`) (`KismetStringLibrary.Concat_StrStr` "|" (`KismetMathLibrary.SelectString` (`KismetStringLibrary.Concat_StrStr` "Attributes.Attack." (`.RightS` (`KismetStringLibrary.Split` _returnvalue "." "CaseSensitive" "FromEnd"))) _returnvalue (`KismetStringLibrary.StartsWith` _returnvalue "Attributes.Magic." "CaseSensitive")) "\\" (`KismetStringLibrary.Conv_DoubleToString` _valuepin)))))
    (:`CompletedPin`
      (bind _output_get (set `local.Res` (`KismetStringLibrary.Concat_StrStr` (`local.Res`) "|")))
      (if (or should_draw apply_effects)
        (set `local.Res` (`KismetStringLibrary.Concat_StrStr` (`KismetStringLibrary.Concat_StrStr` (`KismetMathLibrary.SelectString` "" "d" should_draw) (`KismetMathLibrary.SelectString` "" "e" apply_effects) (`KismetMathLibrary.SelectString` "o" "" draw_entities_only)) "&" _output_get))
        (return (`local.Res`))
        (else
          (return (`local.Res`)))))))

(fn `Set`
  (params (Attribute :type "/Game/Blueprints/SkillSystem/S_Attribute Structure") (Value :type "Float (double-precision)"))
  (returns (Result :type "/Game/Blueprints/SkillSystem/S_Attribute Structure"))
  (bind (_min _base _current _max) (break `/Game/Blueprints/SkillSystem/S_Attribute` Attribute))
  (return (make `/Game/Blueprints/SkillSystem/S_Attribute` _min Value _current _max)))

(fn `SetSkillComp`
  (params (Data :type "/Game/Data/Enitites/S_SkillCompData Structure") (Comp :type "/Game/Blueprints/SkillSystem/AC_SkillComponent Object Reference"))
  (bind _attributeset (`/Game/Blueprints/SkillSystem/AC_SkillComponent.AttributeSet` Comp))
  (`|ExecutionSequence`
    (:`then_0`
      (for _array_element (`/Game/Blueprints/SkillSystem/AC_SkillComponent.Effects` Comp)
        (`/Game/Blueprints/SkillSystem/A_SkillBase.CallDestroySelf` _array_element))
      (for _array_element_2 Data_Effect_9_FA60C20A41CB932F3BB127845D8F9E6A
        (`/Game/Blueprints/SkillSystem/AC_SkillComponent.ApplyEffect` Comp (break `/Game/Data/Skills/S_Effect` _array_element_2) (`.Data_18_F4CAC80D4078950697773C830D0E8E3E` (break `/Game/Data/Skills/S_Effect` _array_element_2)) (`.Duration_10_09701A1B46A9128048DFD3A7339C3312` (break `/Game/Data/Skills/S_Effect` _array_element_2)))))
    (:`then_1`
      (bind (_keypin _valuepin) (`|MapForEach` (`/Game/Blueprints/SkillSystem/AC_SkillComponent.Buffs` Comp))
        (:`then`
          (bind (_keypin_2 _valuepin_2) (`|MapForEach` (break `/Game/Blueprints/SkillSystem/Buffs/S_BuffsMap` _valuepin))
            (:`then`
              (for _array_element_3 (break `/Game/Blueprints/SkillSystem/Buffs/S_BuffsArray` _valuepin_2)
                (`/Game/Blueprints/SkillSystem/A_SkillBase.CallDestroySelf` _array_element_3)))))
        (:`CompletedPin`
          (for _array_element_4 Data_Buffs_12_E745184945F56A1901C01199CF87EE8E
            (`/Game/Blueprints/SkillSystem/AC_SkillComponent.ApplyBuff` Comp (break `/Game/Blueprints/SaveLoad/Skill/S_SAVE_BUFF` _array_element_4) (`.Data_11_7B969E46491D473B1D8ADB88B9EB184D` (break `/Game/Blueprints/SaveLoad/Skill/S_SAVE_BUFF` _array_element_4)) (`.target_14_D55524054EDF5D7EDFBBBEAE7BD30370` (break `/Game/Blueprints/SaveLoad/Skill/S_SAVE_BUFF` _array_element_4)) (`.Duration_5_7A12DC194B43675F4F859D8142F82291` (break `/Game/Blueprints/SaveLoad/Skill/S_SAVE_BUFF` _array_element_4)) "")))))
    (:`then_2`
      (`BlueprintMapLibrary.Map_Clear` _attributeset)
      (bind (_keypin_3 _valuepin_3) (`|MapForEach` Data_Attributes_5_CDBA48DE424B0F103168C69C49C85650)
        (:`then`
          (`BlueprintMapLibrary.Map_Add` _attributeset _keypin_3 (make `/Game/Blueprints/SkillSystem/S_Attribute` -100.0 (`.Base_27_6D5926F0445AB5B78ECF7D85052FB2B0` (break `/Game/Blueprints/SkillSystem/S_Attribute` _valuepin_3)) 0.0 9999.0))
          (if (not (and (== (break `/Game/Blueprints/SkillSystem/S_Attribute` _valuepin_3) -100.0) (== (`.Max_24_B52313574BD363B2E33D4CBBE239C895` (break `/Game/Blueprints/SkillSystem/S_Attribute` _valuepin_3)) 9999.0)))
            (`/Game/Blueprints/SkillSystem/AC_SkillComponent.ApplyBuff` Comp "/Game/Blueprints/SkillSystem/Buffs/ASB_BaseMinMax.ASB_BaseMinMax_C" (`KismetStringLibrary.Concat_StrStr` (`KismetStringLibrary.Conv_DoubleToString` (break `/Game/Blueprints/SkillSystem/S_Attribute` _valuepin_3)) "|" (`KismetStringLibrary.Conv_DoubleToString` (`.Max_24_B52313574BD363B2E33D4CBBE239C895` (break `/Game/Blueprints/SkillSystem/S_Attribute` _valuepin_3)))) _keypin_3 -1.0 "Base Value")))))
    (:`then_3`
      (bind _keypin_4 (`|MapForEach` (`/Game/Blueprints/SkillSystem/AC_SkillComponent.AttributeSet` Comp))
        (:`then`
          (`/Game/Blueprints/SkillSystem/AC_SkillComponent.ReCalculateAttribute` Comp _keypin_4))))
    (:`then_4`
      (for _array_element_5 Data_Bars_16_726B218742F45B2D872226BA9FE6E750
        (`/Game/Blueprints/SkillSystem/AC_SkillComponent.ApplyBarEffect` Comp (break `/Game/Blueprints/SaveLoad/Skill/S_SAVE_BAR` _array_element_5) (`.Value_10_7A12DC194B43675F4F859D8142F82291` (break `/Game/Blueprints/SaveLoad/Skill/S_SAVE_BAR` _array_element_5)) (`.Data_19_BA08F5C54BD117B0D0483DA248D433FA` (break `/Game/Blueprints/SaveLoad/Skill/S_SAVE_BAR` _array_element_5)))))))

(fn `SetWithClamp`
  (params (Attribute :type "/Game/Blueprints/SkillSystem/S_Attribute Structure") (Value :type "Float (double-precision)"))
  (returns (Result :type "/Game/Blueprints/SkillSystem/S_Attribute Structure"))
  (bind (_min _base _current _max) (break `/Game/Blueprints/SkillSystem/S_Attribute` Attribute))
  (return (make `/Game/Blueprints/SkillSystem/S_Attribute` _min (`KismetMathLibrary.FClamp` Value _min _max) _current _max)))

(fn `SubtractDamageSet`
  (params (Damage :type "Map of GameplayTag Structure to Float (double-precision)") (Block :type "Map of GameplayTag Structure to Float (double-precision)"))
  (returns (Result :type "Map of GameplayTag Structure to Float (double-precision)"))
  (locals (Res :type "Map of GameplayTag Structure to Float (double-precision)"))
  (bind _block (`local.Block`))
  (bind _res (`local.Res`))
  (bind (_keypin _valuepin) (`|MapForEach` Damage)
    (:`then`
      (`|SwitchGameplayTag` _keypin
        (:`Attributes.Attack.Clear`
          (`BlueprintMapLibrary.Map_Add` _res _keypin _valuepin :!label _label))
        (:`Attributes.Magic.Clear`
          (goto _label))
        (:`Attributes.Attack.Cutting`
          (`BlueprintMapLibrary.Map_Add` _res _keypin (`self.SubtractSingleDamage` (`BlueprintMapLibrary.Map_Find` _block (`BlueprintGameplayTagLibrary.MakeLiteralGameplayTag` (struct :`TagName` "Attributes.Armour.Cutting"))) _valuepin) :!label _label_2))
        (:`Attributes.Magic.Cutting`
          (goto _label_2))
        (:`Attributes.Attack.Electrical`
          (`BlueprintMapLibrary.Map_Add` _res _keypin (`self.SubtractSingleDamage` (`BlueprintMapLibrary.Map_Find` _block (`BlueprintGameplayTagLibrary.MakeLiteralGameplayTag` (struct :`TagName` "Attributes.Armour.Electrical"))) _valuepin) :!label _label_3))
        (:`Attributes.Magic.Electrical`
          (goto _label_3))
        (:`Attributes.Attack.FallDamage`
          (`BlueprintMapLibrary.Map_Add` _res _keypin (`self.SubtractSingleDamage` (`BlueprintMapLibrary.Map_Find` _block (`BlueprintGameplayTagLibrary.MakeLiteralGameplayTag` (struct :`TagName` "Attributes.Armour.FallDamage"))) _valuepin)))
        (:`Attributes.Attack.Fire`
          (`BlueprintMapLibrary.Map_Add` _res _keypin (`self.SubtractSingleDamage` (`BlueprintMapLibrary.Map_Find` _block (`BlueprintGameplayTagLibrary.MakeLiteralGameplayTag` (struct :`TagName` "Attributes.Armour.Fire"))) _valuepin) :!label _label_4))
        (:`Attributes.Magic.Fire`
          (goto _label_4))
        (:`Attributes.Attack.Frost`
          (`BlueprintMapLibrary.Map_Add` _res _keypin (`self.SubtractSingleDamage` (`BlueprintMapLibrary.Map_Find` _block (`BlueprintGameplayTagLibrary.MakeLiteralGameplayTag` (struct :`TagName` "Attributes.Armour.Frost"))) _valuepin) :!label _label_5))
        (:`Attributes.Magic.Frost`
          (goto _label_5))
        (:`Attributes.Attack.Physic`
          (`BlueprintMapLibrary.Map_Add` _res _keypin (`self.SubtractSingleDamage` (`BlueprintMapLibrary.Map_Find` _block (`BlueprintGameplayTagLibrary.MakeLiteralGameplayTag` (struct :`TagName` "Attributes.Armour.Physic"))) _valuepin) :!label _label_6))
        (:`Attributes.Magic.Physic`
          (goto _label_6))
        (:`Attributes.Attack.Piercing`
          (`BlueprintMapLibrary.Map_Add` _res _keypin (`self.SubtractSingleDamage` (`BlueprintMapLibrary.Map_Find` _block (`BlueprintGameplayTagLibrary.MakeLiteralGameplayTag` (struct :`TagName` "Attributes.Armour.Piercing"))) _valuepin) :!label _label_7))
        (:`Attributes.Magic.Piercing`
          (goto _label_7))
        (:`Attributes.Attack.Water`
          (`BlueprintMapLibrary.Map_Add` _res _keypin (`self.SubtractSingleDamage` (`BlueprintMapLibrary.Map_Find` _block (`BlueprintGameplayTagLibrary.MakeLiteralGameplayTag` (struct :`TagName` "Attributes.Armour.Water"))) _valuepin) :!label _label_8))
        (:`Attributes.Magic.Water`
          (goto _label_8))
        (:`Attributes.Attack.Silver`
          (`BlueprintMapLibrary.Map_Add` _res _keypin (`self.SubtractSingleDamage` (`BlueprintMapLibrary.Map_Find` _block (`BlueprintGameplayTagLibrary.MakeLiteralGameplayTag` (struct :`TagName` "Attributes.Armour.Silver"))) _valuepin) :!label _label_9))
        (:`Attributes.Magic.Silver`
          (goto _label_9))
        (:`Attributes.Magic.Radiation`
          (`BlueprintMapLibrary.Map_Add` _res _keypin (`self.SubtractSingleDamage` (`BlueprintMapLibrary.Map_Find` _block (`BlueprintGameplayTagLibrary.MakeLiteralGameplayTag` (struct :`TagName` "Attributes.Armour.Radiation"))) _valuepin) :!label _label_10))
        (:`Attributes.Attack.Radiation`
          (goto _label_10))
        (:`Attributes.Attack.Poison`
          (`BlueprintMapLibrary.Map_Add` _res _keypin (`self.SubtractSingleDamage` (`BlueprintMapLibrary.Map_Find` _block (`BlueprintGameplayTagLibrary.MakeLiteralGameplayTag` (struct :`TagName` "Attributes.Armour.Poison"))) _valuepin) :!label _label_11))
        (:`Attributes.Magic.Poison`
          (goto _label_11))))
    (:`CompletedPin`
      (return (`local.Res`)))))

(fn `SubtractSingleDamage`
  (params (Armour :type "Float (double-precision)") (Damage :type "Float (double-precision)"))
  (returns (Res :type "Float (double-precision)"))
  (locals (MinPercent :type "Float (double-precision)" :default 0.15) (hardness :type "Float (double-precision)" :default 60.0))
  (bind _returnvalue (- Damage Armour))
  (if (== Armour 9999.0)
    ; FullResist
    (return 0.0)
    (elif (> _returnvalue 0.0)
      ; Armour == Damage
      (return _returnvalue)
      (else
        ; Armour > Damage
        (return (`KismetMathLibrary.FMax` 1.0 (/ (* Damage (`local.MinPercent`)) (+ (/ (- Armour Damage) (`local.hardness`)) 1.0))))))))