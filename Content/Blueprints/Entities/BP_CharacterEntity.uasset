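; Character entity Blueprint that handles landing, fall damage and hit sounds, with gameplay actions routed through ACSkillComponent.
; On landing it stops the jump skill, converts downward speed beyond a threshold into damage, and activates AS_TakeDamage with that value serialized as attribute metadata.
; Taking damage plays a random hit sound at the actor's location.
; Interact and Die events are empty; a skill-stopping, delayed destroy sequence exists but is unconnected.
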(event `self.OnLanded`
  (params (Hit :type "HitResult Structure (by ref)"))
  (bind _ac_skillcomponent (`self.AC_SkillComponent`))
  (bind _returnvalue (`KismetMathLibrary.FClamp` (/ (+ (.z (`self.GetVelocity`)) 1000.0) -20.0) 0.0 99999.0))
  (`/Game/Blueprints/SkillSystem/AC_SkillComponent.StopSkillByTag` _ac_skillcomponent (struct :`TagName` "Skills.Base.Movement.Jump"))
  (if (not (== _returnvalue 0.0))
    (`/Game/Blueprints/SkillSystem/AC_SkillComponent.ActivateSkill` _ac_skillcomponent null "/Game/Blueprints/SkillSystem/Skills/Base/AS_TakeDamage.AS_TakeDamage_C" (`/Game/Blueprints/SkillSystem/BFL_SkillsHelper.SerializeDamage` (struct :`TagName` "Attributes.Base.Health") (`|MakeMap` (struct :`TagName` "Attributes.Attack.FallDamage") _returnvalue :!type "GameplayTag Structure") true))))

(event `/Game/Blueprints/Entities/BPI_Interact.OnInteract`
  (params (Insignator :type "Actor Object Reference") (Location :type "Vector Structure") (Normal :type "Vector Structure")))

(event `/Game/Blueprints/Entities/BPI_Damage.OnTakeDamage`
  (`GameplayStatics.PlaySoundAtLocation` (`KismetArrayLibrary.Array_Random` (`self.SoundsOnHit`)) (`self.K2_GetActorLocation`) (struct) 1.0 1.0 0.0 null null null null))

(event `/Game/Blueprints/Entities/BPI_Damage.Die`)

(fn `UserConstructionScript`
  (`parent.UserConstructionScript`))