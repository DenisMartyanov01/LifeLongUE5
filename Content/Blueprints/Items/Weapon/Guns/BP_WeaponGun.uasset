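; Gun weapon item actor that can display the round from its magazine data on the weapon, with an empty Shoot event.
; Set clears the mesh for "air" data; otherwise it looks up the magazine's item row, caches bullet mesh and material, then calls UpdateBullet.
; UpdateBullet keeps a matching non-empty bullet actor, or destroys it and, if ShowBullet is on, spawns the magazine's actor class at PointBullet.
; EndPlay destroys that bullet actor.
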(event `self.ReceiveEndPlay`
  (params (EndPlayReason :type "EEndPlayReason Enum" :default "Destroyed"))
  (bind _bullet (`self.Bullet`))
  (`/Engine/EditorBlueprintResources/StandardMacros.IsValid` _bullet
    (:`Is Valid`
      (`self.K2_DestroyActor` _bullet))))

(event `Shoot`)

(fn `Set`
  (params (Data :type "/Game/Data/O_Item Object Reference") (copy :type Boolean))
  (bind _itemdata_id (break `/Game/Data/S_CompBase` (`/Game/Data/O_Item.ItemData` Data)))
  (`parent.Set` Data copy)
  (if (== _itemdata_id "air")
    (`StaticMeshComponent.SetStaticMesh` (`self.StaticMesh`) null)
    (else
      (bind _aso_weapon_gun (cast `/Game/Data/O_WeaponGun` (`self.Data`)))
      (bind _itemdata_id_2 (break `/Game/Data/S_CompBase` (`/Game/Data/O_Item.ItemData` (`/Game/Data/O_WeaponGun.Magazine` _aso_weapon_gun))))
      (bind _returnvalue (`|GetDataTableRow` "/Game/Data/BaseData/CDT_AllBaseData.CDT_AllBaseData" _itemdata_id_2)
        (:`then`
          (set `self.BulletMat` (`.Material_52_C6618F874456030E1B15CAB86F5ED5E5` (break `/Game/Data/BaseData/S_AllDataItem` _returnvalue)))
          (set `self.BulletMesh` (`.Mesh_21_E7B15A78417E9C42D369988CD7EB507C` (break `/Game/Data/BaseData/S_AllDataItem` _returnvalue)))
          (`self.UpdateBullet`))))))

(fn `UpdateBullet`
  (bind _bullet (`self.Bullet`))
  (bind (_itemdata_id _itemdata_title _itemdata_count) (break `/Game/Data/S_CompBase` (`/Game/Data/O_Item.ItemData` (`/Game/Blueprints/Items/BP_Item.Data` _bullet))))
  (bind _aso_weapon_gun (cast `/Game/Data/O_WeaponGun` (`self.Data`)))
  (bind _magazine (`/Game/Data/O_WeaponGun.Magazine` _aso_weapon_gun))
  (bind (_itemdata_id_2 _itemdata_title_2 _itemdata_count_2 _itemdata_stacksize _itemdata_objecttype _itemdata_posonbody _itemdata_tier _itemdata_hands _itemdata_actorclass) (break `/Game/Data/S_CompBase` (`/Game/Data/O_Item.ItemData` _magazine)))
  (bind _returnvalue (`|GetDataTableRow` "/Game/Data/BaseData/CDT_AllBaseData.CDT_AllBaseData" _itemdata_id_2)
    (:`then`
      (set `self.BulletMesh` (`.Mesh_21_E7B15A78417E9C42D369988CD7EB507C` (break `/Game/Data/BaseData/S_AllDataItem` _returnvalue)))
      (set `self.BulletMat` (`.Material_52_C6618F874456030E1B15CAB86F5ED5E5` (break `/Game/Data/BaseData/S_AllDataItem` _returnvalue)))
      (`|ExecutionSequence`
        (:`then_0`
          (`/Engine/EditorBlueprintResources/StandardMacros.IsValid` _bullet
            (:`Is Valid`
              (if (and (== _itemdata_id _itemdata_id_2) (!= _itemdata_count 0))
                (return)
                (else
                  (`self.K2_DestroyActor` _bullet))))))
        (:`then_1`
          (if (`self.show_bullet`)
            (if (`KismetSystemLibrary.IsValidClass` _itemdata_actorclass)
              (bind _returnvalue_2 (`|SpawnActorFromClass` _itemdata_actorclass (`KismetMathLibrary.MakeTransform` (0.0 0.0 0.0)) "Undefined" "MultiplyWithRoot" null "NewEnumerator1" true null))
              (`self.Set` _returnvalue_2 _magazine true)
              (`self.K2_AttachToComponent` _returnvalue_2 (`self.PointBullet`) "None" "KeepRelative" "KeepRelative" "KeepRelative" true)
              (set `self.Bullet` _returnvalue_2))))))))

(fn `UserConstructionScript`
  (`parent.UserConstructionScript`))