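; BP_Automat is a gun Blueprint that plays a one-shot Paper2D flipbook effect each time it shoots.
; On BeginPlay it calls its parent, disables looping, hides the flipbook and binds End to the finished-playing event.
; Shoot shows the flipbook and plays it from the start, and End hides it again when playback finishes.
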(event `self.ReceiveBeginPlay`
  (bind _paperflipbook (`self.PaperFlipbook`))
  (`parent.ReceiveBeginPlay`)
  (`PaperFlipbookComponent.SetLooping` _paperflipbook false)
  (`SceneComponent.SetVisibility` _paperflipbook false false)
  (add `PaperFlipbookComponent.OnFinishedPlaying` _paperflipbook (delegate `End`)))

(event `End`
  (`SceneComponent.SetVisibility` (`self.PaperFlipbook`) false false))

(event `self.Shoot`
  (bind _paperflipbook (`self.PaperFlipbook`))
  (`SceneComponent.SetVisibility` _paperflipbook true false)
  (`PaperFlipbookComponent.PlayFromStart` _paperflipbook))

(fn `UserConstructionScript`
  (`parent.UserConstructionScript`))