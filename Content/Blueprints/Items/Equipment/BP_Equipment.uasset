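; Equipment item Blueprint that grants armour buffs to its owner while equipped and plays handling sounds.
; OnEquip applies an endless ASB_AddArmour buff through the owner's AC_SkillComponent for each non-zero Armour entry in its O_Equipment data, storing each buff.
; Equipping, taking in hand and hiding play a random DT_BaseEquip sound by item ID.
; OnUnequip removes the buffs and spawned model actors; destruction triggers both unequip and hide.
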(event `self.ReceiveDestroyed`
  (`self.OnUnequip`)
  (`self.OnHideFromHand`))

(fn `OnEquip`
  (bind _returnvalue (`self.GetComponentByClass` (`self.GetOwner`) "/Game/Blueprints/SkillSystem/AC_SkillComponent.AC_SkillComponent_C"))
  (bind _itemdata_id (break `/Game/Data/S_CompBase` (`/Game/Data/O_Item.ItemData` (`self.Data`))))
  (bind (_itemdata_id_2 _itemdata_title) (break `/Game/Data/S_CompBase` (`/Game/Data/O_Item.ItemData` (`self.Data`))))
  (`|ExecutionSequence`
    (:`then_0`
      (bind _aso_equipment (cast `/Game/Data/O_Equipment` (`self.Data`)))
      (`/Engine/EditorBlueprintResources/StandardMacros.IsValid` _returnvalue
        (:`Is Valid`
          (bind (_equipmentdata_slot _equipmentdata_armour) (break `/Game/Data/S_CompEquipment` (`/Game/Data/O_Equipment.EquipmentData` _aso_equipment)))
          (bind (_keypin _valuepin) (`|MapForEach` _equipmentdata_armour)
            (:`then`
              (if (!= _valuepin 0.0)
                (bind _effect (`/Game/Blueprints/SkillSystem/AC_SkillComponent.ApplyBuff` _returnvalue "/Game/Blueprints/SkillSystem/Buffs/ASB_AddArmour.ASB_AddArmour_C" (`KismetStringLibrary.Concat_StrStr` "0" "|" (`KismetStringLibrary.Conv_DoubleToString` _valuepin) "|" "0") _keypin -1.0 _itemdata_title))
                (`KismetArrayLibrary.Array_Add` (`self.Buffs`) _effect)))))))
    (:`then_1`
      (bind _returnvalue_2 (`|GetDataTableRow` "/Game/Data/BaseData/DT_BaseEquip.DT_BaseEquip" _itemdata_id)
        (:`then`
          (`GameplayStatics.PlaySoundAtLocation` (`KismetArrayLibrary.Array_Random` (`.SoundsOnChoose_59_8E149F3B47035A261B0D2586441DC828` (break `/Game/Data/BaseData/S_AllDataItem` _returnvalue_2))) (`self.K2_GetActorLocation`) (struct) 1.0 1.0 0.0 "/Game/Assets/Sounds/SA_FadeOut.SA_FadeOut" null null null))))))

(fn `OnHideFromHand`
  (bind _itemdata_id (break `/Game/Data/S_CompBase` (`/Game/Data/O_Item.ItemData` (`self.Data`))))
  (bind _returnvalue (`|GetDataTableRow` "/Game/Data/BaseData/DT_BaseEquip.DT_BaseEquip" _itemdata_id)
    (:`then`
      (`GameplayStatics.PlaySoundAtLocation` (`KismetArrayLibrary.Array_Random` (`.SoundsOnChoose_59_8E149F3B47035A261B0D2586441DC828` (break `/Game/Data/BaseData/S_AllDataItem` _returnvalue))) (`self.K2_GetActorLocation`) (struct) 1.0 1.0 0.0 null null null null))))

(fn `OnTakeInHand`
  (bind _itemdata_id (break `/Game/Data/S_CompBase` (`/Game/Data/O_Item.ItemData` (`self.Data`))))
  (bind _returnvalue (`|GetDataTableRow` "/Game/Data/BaseData/DT_BaseEquip.DT_BaseEquip" _itemdata_id)
    (:`then`
      (`GameplayStatics.PlaySoundAtLocation` (`KismetArrayLibrary.Array_Random` (`.SoundsOnChoose_59_8E149F3B47035A261B0D2586441DC828` (break `/Game/Data/BaseData/S_AllDataItem` _returnvalue))) (`self.K2_GetActorLocation`) (struct) 1.0 1.0 0.0 null null null null))))

(fn `OnUnequip`
  (for _array_element (`self.Buffs`)
    (`/Engine/EditorBlueprintResources/StandardMacros.IsValid` _array_element
      (:`Is Valid`
        (`/Game/Blueprints/SkillSystem/A_SkillBase.CallDestroySelf` _array_element))))
  (for _array_element_2 (`self.Models23`)
    (`self.K2_DestroyActor` _array_element_2)))

(fn `UserConstructionScript`
  (`parent.UserConstructionScript`))