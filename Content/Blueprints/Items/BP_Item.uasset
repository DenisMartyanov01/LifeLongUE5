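; BP_Item is the world actor for an item data object, which can be picked up, held or thrown.
; Set pulls mesh, material and texture from CDT_AllBaseData, while SetPhysicMode switches between simulated, held, thrown and static states, toggling the OnFloor tag that gates pickup.
; Thrown hits apply damage and knockback through AC_SkillComponent skills, or merge matching stacks.
; Damageable items add their own skill component with health on BeginPlay.
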(event `Anim_OneHand`)

(event `Anim_TwoHandRight`)

(event `Anim_TwoHandLeft`)

(event `Anim_R`)

(event `SERVER_Interact`
  (params (Target :type "Actor Object Reference"))
  (if (`self.ActorHasTag` "OnFloor")
    (`/Game/Blueprints/SkillSystem/AC_SkillComponent.ActivateSkill` (`self.GetComponentByClass` Target "/Game/Blueprints/SkillSystem/AC_SkillComponent.AC_SkillComponent_C") self "/Game/Blueprints/SkillSystem/Skills/Base/AS_TakeItem.AS_TakeItem_C" "")
    (message `/Game/Blueprints/Entities/BPI_Interact.OnBreakInteraction` Target)))

(event `/Game/Blueprints/Entities/BPI_Interact.OnInteract`
  (params (Insignator :type "Actor Object Reference") (Location :type "Vector Structure") (Normal :type "Vector Structure"))
  (`self.SERVER_Interact` Insignator))

(event `SetPhysicMode`
  (params (State :type "/Game/Blueprints/Items/E_ItemState Enum" :default "NewEnumerator0"))
  (bind _tags (`self.Tags`))
  (bind _staticmesh (`self.StaticMesh`))
  (bind _rotatingmovement (`self.RotatingMovement`))
  (bind _staticmesh_2 (`self.StaticMesh`))
  (bind _staticmesh_3 (`self.StaticMesh`))
  (bind _staticmesh_4 (`self.StaticMesh`))
  (bind _staticmesh_5 (`self.StaticMesh`))
  (bind (_itemdata_id _itemdata_title _itemdata_count _itemdata_stacksize _itemdata_objecttype _itemdata_posonbody _itemdata_tier _itemdata_hands) (break `/Game/Data/S_CompBase` (`/Game/Data/O_Item.ItemData` (`self.Data`))))
  (bind _returnvalue (== (`KismetSystemLibrary.MakeLiteralByte` _itemdata_hands) (`KismetSystemLibrary.MakeLiteralByte` (enumliteral `/Game/Data/BaseData/E_Hands` "NewEnumerator1"))))
  (set `self.StartState` State)
  (switch `/Game/Blueprints/Items/E_ItemState` State
    (:`NewEnumerator0`
      (`PrimitiveComponent.SetCollisionEnabled` _staticmesh_5 "QueryAndPhysics")
      (`PrimitiveComponent.SetSimulatePhysics` _staticmesh_5 true)
      (`PrimitiveComponent.SetEnableGravity` _staticmesh_5 true)
      (`KismetArrayLibrary.Array_AddUnique` _tags "OnFloor")
      (`ActorComponent.Deactivate` (`self.RotatingMovement`) :!label _label)
      (`ActorComponent.Deactivate` (`self.ProjectileMovement`)))
    (:`NewEnumerator1`
      (`PrimitiveComponent.SetSimulatePhysics` _staticmesh_2 false)
      (`PrimitiveComponent.SetEnableGravity` _staticmesh_2 false)
      (`PrimitiveComponent.SetCollisionEnabled` _staticmesh_2 "NoCollision")
      (`|ExecutionSequence`
        (:`then_0`
          (switch `/Game/Data/BaseData/E_ObjectType` _itemdata_objecttype
            (:`NewEnumerator3`
              (`PrimitiveComponent.SetCollisionEnabled` _staticmesh_2 "QueryOnly")
              (`PrimitiveComponent.SetCollisionObjectType` (`self.StaticMesh`) "ECC_GameTraceChannel2")
              (`PrimitiveComponent.SetCollisionObjectType` _staticmesh_2 "ECC_GameTraceChannel2"))))
        (:`then_1`
          (`KismetArrayLibrary.Array_RemoveItem` _tags "OnFloor")
          (clear `PrimitiveComponent.OnComponentHit` (`self.StaticMesh`) :!label _label_2)
          (goto _label))))
    (:`NewEnumerator2`
      (`PrimitiveComponent.SetSimulatePhysics` _staticmesh_4 false)
      (`PrimitiveComponent.SetEnableGravity` _staticmesh_4 true)
      (`PrimitiveComponent.SetCollisionEnabled` _staticmesh_4 "NoCollision")
      (`ActorComponent.SetActive` _rotatingmovement true false)
      (`ActorComponent.SetActive` (`self.ProjectileMovement`) true false)
      (set `ProjectileMovementComponent.bSimulationEnabled` true (`self.ProjectileMovement`))
      (`ActorComponent.SetAutoActivate` _rotatingmovement true)
      (`self.SetFlyingStats` 1000.0)
      (`KismetArrayLibrary.Array_AddUnique` (`self.Tags`) "OnFloor")
      (cast `/Game/Data/O_Weapon` (`self.Data`)
        (:`then`
          (set `RotatingMovementComponent.RotationRate` (`KismetMathLibrary.MakeRotator` 0.0 (`KismetMathLibrary.SelectFloat` 0.0 -360.0 _returnvalue)) (`self.RotatingMovement`))
          (set `ProjectileMovementComponent.bRotationFollowsVelocity` _returnvalue (`self.ProjectileMovement`)))
        (:`CastFailed`
          (set `RotatingMovementComponent.RotationRate` (`KismetMathLibrary.MakeRotator` 0.0) (`self.RotatingMovement`))))
      (clear `PrimitiveComponent.OnComponentHit` (`self.StaticMesh`))
      (`KismetSystemLibrary.Delay` 0.3)
      (`PrimitiveComponent.SetCollisionEnabled` _staticmesh "QueryAndPhysics")
      (add `PrimitiveComponent.OnComponentHit` _staticmesh (`|CreateDelegate` :!event `OnHit`))
      (`self.OnThrow`))
    (:`NewEnumerator3`
      (`PrimitiveComponent.SetSimulatePhysics` _staticmesh_3 false)
      (`PrimitiveComponent.SetEnableGravity` _staticmesh_3 false)
      (`PrimitiveComponent.SetCollisionEnabled` _staticmesh_3 "QueryAndPhysics")
      (`KismetArrayLibrary.Array_AddUnique` (`self.Tags`) "OnFloor")
      (goto _label_2))))

(event `OnThrow`)

(event `OnHit`
  (params (HitComponent :type "PrimitiveComponent Object Reference") (OtherActor :type "Actor Object Reference") (OtherComp :type "PrimitiveComponent Object Reference") (NormalImpulse :type "Vector Structure") (Hit :type "HitResult Structure (by ref)"))
  (bind _returnvalue (`self.GetComponentByClass` OtherActor "/Game/Blueprints/SkillSystem/AC_SkillComponent.AC_SkillComponent_C"))
  (bind _returnvalue_2 (`KismetMathLibrary.Normal` (- (`self.K2_GetActorLocation`) Hit_ImpactPoint)))
  (`/Engine/EditorBlueprintResources/StandardMacros.IsValid` OtherActor
    (:`Is Valid`
      (set `self.Speed` (`KismetMathLibrary.VSize` (`self.GetVelocity`)))
      (`|ExecutionSequence`
        (:`then_0`
          (`/Engine/EditorBlueprintResources/StandardMacros.IsValid` _returnvalue
            (:`Is Valid`
              (`self.SetPhysicMode` "NewEnumerator0")
              (if (and (> (`self.Speed`) 300.0) (`self.deal_damage`))
                (bind _aso_weapon (cast `/Game/Data/O_Weapon` (`self.Data`))
                  (:`then`
                    (bind _weapondata_damage (break `/Game/Data/S_CompWeapon` (`/Game/Data/O_Weapon.WeaponData` _aso_weapon)))
                    (`/Game/Blueprints/SkillSystem/AC_SkillComponent.ActivateSkill` _returnvalue null "/Game/Blueprints/SkillSystem/Skills/Base/AS_TakeDamage.AS_TakeDamage_C" (`/Game/Blueprints/SkillSystem/BFL_SkillsHelper.SerializeDamage` (struct :`TagName` "Attributes.Base.Health") _weapondata_damage true true))
                    (`/Engine/EditorBlueprintResources/StandardMacros.IsValid` OtherActor
                      (:`Is Valid`
                        (`/Game/Blueprints/SkillSystem/AC_SkillComponent.ActivateSkillBase` _returnvalue "/Game/Blueprints/SkillSystem/Skills/Attack/_Other/AS_KnockBack.AS_KnockBack_C" (`KismetStringLibrary.Conv_VectorToString` (* _returnvalue_2 (+ (`BlueprintMapLibrary.Map_Find` _weapondata_damage (struct :`TagName` "Attributes.Attack.Physic")) 100.0)))))))
                  (:`CastFailed`
                    (`/Game/Blueprints/SkillSystem/AC_SkillComponent.ActivateSkill` _returnvalue null "/Game/Blueprints/SkillSystem/Skills/Base/AS_TakeDamage.AS_TakeDamage_C" (`/Game/Blueprints/SkillSystem/BFL_SkillsHelper.SerializeDamage` (struct :`TagName` "Attributes.Base.Health") (`|MakeMap` (struct :`TagName` "Attributes.Attack.Physic") 3.0 :!type "GameplayTag Structure") true true))
                    (`/Game/Blueprints/SkillSystem/AC_SkillComponent.ActivateSkillBase` _returnvalue "/Game/Blueprints/SkillSystem/Skills/Attack/_Other/AS_KnockBack.AS_KnockBack_C" (`KismetStringLibrary.Conv_VectorToString` (* _returnvalue_2 100.0)))))))
            (:`Is Not Valid`
              (if (`self.can_merge`)
                (bind _asbp_item (cast `/Game/Blueprints/Items/BP_Item` OtherActor)
                  (:`then`
                    (bind _stay_self (`self.TryToConnect` _asbp_item))
                    (if _stay_self
                      (`self.SetPhysicMode` "NewEnumerator0")))
                  (:`CastFailed`
                    (cast `/Game/Data/O_Weapon` (`self.Data`) :!label _label_3
                      (:`then`
                        (if (== (`GameplayStatics.GetObjectClass` OtherActor) null)
                          (`self.SetPhysicMode` "NewEnumerator0" :!label _label_4)
                          (else
                            (`self.SetPhysicMode` "NewEnumerator3"))))
                      (:`CastFailed`
                        (goto _label_4)))))
                (else
                  (goto _label_3))))))
        (:`then_1`
          (`self.OnHitLogic` Hit_Normal Hit_ImpactPoint (`self.Speed`)))))))

(event `OnHitLogic`
  (params (Normal :type "Vector Structure") (HitLocation :type "Vector Structure") (Speed :type "Float (double-precision)")))

(event `self.ReceiveDestroyed`
  (`self.OnHideFromHand`)
  (`/Engine/EditorBlueprintResources/StandardMacros.IsValid` (stale `self.ReceiveBeginPlay` _returnvalue)
    (:`Is Valid`
      (`/Game/Blueprints/SkillSystem/AC_SkillComponent.StopAll` (stale `self.ReceiveBeginPlay` _returnvalue))
      (`KismetSystemLibrary.DelayUntilNextTick`))))

(event `self.ReceiveBeginPlay`
  (if (`self.can_be_damaged`)
    (bind _returnvalue (`AddComponent|NODE_AddAC_SkillComponent-0`))
    (bind _attributeset (`/Game/Blueprints/SkillSystem/AC_SkillComponent.AttributeSet` _returnvalue))
    (`BlueprintMapLibrary.Map_Add` _attributeset (struct :`TagName` "Attributes.Base.Health") (make `/Game/Blueprints/SkillSystem/S_Attribute` 0.0 5.0 5.0 5.0))
    (`BlueprintMapLibrary.Map_Add` _attributeset (struct :`TagName` "Attributes.Armour.Water") (make `/Game/Blueprints/SkillSystem/S_Attribute` 0.0 9999.0 9999.0 9999.0))))

(fn `OnHideFromHand`
  (bind _itemdata_id (break `/Game/Data/S_CompBase` (`/Game/Data/O_Item.ItemData` (`self.Data`))))
  (bind _returnvalue (`|GetDataTableRow` "/Game/Data/BaseData/CDT_AllBaseData.CDT_AllBaseData" _itemdata_id)
    (:`then`
      (`GameplayStatics.PlaySoundAtLocation` (`KismetArrayLibrary.Array_Random` (`.SoundsOnChoose_59_8E149F3B47035A261B0D2586441DC828` (break `/Game/Data/BaseData/S_AllDataItem` _returnvalue))) (`self.K2_GetActorLocation`) (struct) 1.0 1.0 0.0 null null null null))))

(fn `OnTakeInHand`
  (bind _itemdata_id (break `/Game/Data/S_CompBase` (`/Game/Data/O_Item.ItemData` (`self.Data`))))
  (bind _returnvalue (`|GetDataTableRow` "/Game/Data/BaseData/CDT_AllBaseData.CDT_AllBaseData" _itemdata_id)
    (:`then`
      (`GameplayStatics.PlaySoundAtLocation` (`KismetArrayLibrary.Array_Random` (`.SoundsOnChoose_59_8E149F3B47035A261B0D2586441DC828` (break `/Game/Data/BaseData/S_AllDataItem` _returnvalue))) (`self.K2_GetActorLocation`) (struct) 1.0 1.0 0.0 null null null null))))

(fn `Set`
  (params (Data :type "/Game/Data/O_Item Object Reference") (copy :type Boolean :default true))
  (bind _data (`self.Data`))
  (bind _staticmesh (`self.StaticMesh`))
  (bind _itemdata_id (break `/Game/Data/S_CompBase` (`/Game/Data/O_Item.ItemData` _data)))
  (if copy
    (bind _returnvalue (`|GenericCreateObject` (`GameplayStatics.GetObjectClass` Data)))
    (bind _output_get (set `self.Data` _returnvalue))
    (`/Game/Data/O_Item.Copy` _data Data)
    (`/Game/Data/O_Item.Copy` _output_get Data)
    (set `/Game/Data/O_Item.ItemActor` self _data)
    (else
      (set `self.Data` Data)
      (set `/Game/Data/O_Item.ItemActor` self _data)))
  (if (or (== _itemdata_id "None") (== _itemdata_id "air"))
    (`StaticMeshComponent.SetStaticMesh` _staticmesh null :!label _label)
    (else
      (bind _returnvalue_2 (`|GetDataTableRow` "/Game/Data/BaseData/CDT_AllBaseData.CDT_AllBaseData" _itemdata_id)
        (:`then`
          (`StaticMeshComponent.SetStaticMesh` _staticmesh (`.Mesh_21_E7B15A78417E9C42D369988CD7EB507C` (break `/Game/Data/BaseData/S_AllDataItem` _returnvalue_2)))
          (bind _returnvalue_3 (`KismetMaterialLibrary.CreateDynamicMaterialInstance` (`.Material_52_C6618F874456030E1B15CAB86F5ED5E5` (break `/Game/Data/BaseData/S_AllDataItem` _returnvalue_2))))
          (`MaterialInstanceDynamic.SetTextureParameterValue` _returnvalue_3 "Texture" (`.Texture_92_852A257A41DCA6BA2F62BB89B87126B8` (break `/Game/Data/BaseData/S_AllDataItem` _returnvalue_2)))
          (`PrimitiveComponent.SetMaterial` _staticmesh 0 _returnvalue_3)
          (`self.SetPhysicMode` (`self.StartState`)))
        (:`RowNotFound`
          (goto _label))))))

(fn `SetFlyingStats`
  (params (Speed :type "Float (double-precision)") (Weight :type "Float (double-precision)"))
  (bind _projectilemovement (`self.ProjectileMovement`))
  (set `ProjectileMovementComponent.InitialSpeed` Speed _projectilemovement)
  (set `ProjectileMovementComponent.MaxSpeed` Speed _projectilemovement)
  (set `MovementComponent.Velocity` (* (`self.GetActorForwardVector`) Speed) _projectilemovement)
  (`ActorComponent.Activate` _projectilemovement true))

(fn `TryToConnect`
  (params (Other :type "/Game/Blueprints/Items/BP_Item Object Reference"))
  (returns (stay_self :type Boolean))
  (locals (Sum :type Integer) (lastCount :type Integer))
  (bind _data (`self.Data`))
  (bind _data_2 (`/Game/Blueprints/Items/BP_Item.Data` Other))
  (bind (_itemdata_id _itemdata_title _itemdata_count _itemdata_stacksize) (break `/Game/Data/S_CompBase` (`/Game/Data/O_Item.ItemData` _data)))
  (bind (_itemdata_id_2 _itemdata_title_2 _itemdata_count_2) (break `/Game/Data/S_CompBase` (`/Game/Data/O_Item.ItemData` _data_2)))
  (bind _returnvalue (+ _itemdata_count_2 _itemdata_count))
  (if (== _itemdata_id _itemdata_id_2)
    (bind _output_get (set `local.Sum` _returnvalue))
    (set `local.lastCount` (mod _returnvalue _itemdata_stacksize))
    (if (<= _output_get _itemdata_stacksize)
      (`/Game/Data/O_Item.SetCount` _data_2 _output_get)
      (`self.K2_DestroyActor`)
      (return false)
      (else
        (`/Game/Data/O_Item.SetCount` _data_2 _itemdata_stacksize)
        (`/Game/Data/O_Item.SetCount` _data (- _output_get _itemdata_stacksize))
        (return true)))
    (else
      (return true))))

(fn `UserConstructionScript`)