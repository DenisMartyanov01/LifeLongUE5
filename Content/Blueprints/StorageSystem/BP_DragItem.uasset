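; Drag-and-drop operation for the storage system that broadcasts the pointer's screen position while an item is dragged.
; The Dragged event passes that position through CallPointerChangedPosition, and the Return event is empty.
; Unconnected leftover logic would respond to visibility changes by returning the item to equipment or storage, dropping any remainder, then removing the drag visual and cancelling the drag.
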(event `self.Dragged`
  (params (PointerEvent :type "PointerEvent Structure (by ref)"))
  (`self.Pointer Changed Position` (`KismetInputLibrary.PointerEvent_GetScreenSpacePosition` PointerEvent)))

(event `Return`
  (params (InVisibility :type "ESlateVisibility Enum" :default "Visible")))