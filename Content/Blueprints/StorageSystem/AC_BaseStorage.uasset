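; Base actor component for the storage system, defining a common slot interface with stub get, set, drop-to-slot, clear and replication hooks.
; Swap exchanges slots between two storages, rolling back if the second write fails, and refreshes equipped hands when an item panel is involved.
; DropItem throws a stack through the owner's skill component; drops and successful swaps update weight.
; ReplicatedData's OnRep forwards to overridable client update and logic hooks.
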(event `CLIENT_UpdateData`
  (params (ReplicatedData :type "Array of /Game/Blueprints/SaveLoad/Base/S_SAVE_DATA_ITEM Structure")))

(fn `Clear`)

(fn `DropItem`
  (params (SStack :type "/Game/Data/O_Item Object Reference"))
  (bind _scaleeffect (`/Game/Blueprints/SkillSystem/AC_SkillComponent.ApplyBarEffect` (`Actor.GetComponentByClass` (`self.GetOwner`) "/Game/Blueprints/SkillSystem/AC_SkillComponent.AC_SkillComponent_C") "/Game/Blueprints/SkillSystem/Skills/Attack/Throw/AS_ThrowBase.AS_ThrowBase_C" 1.0 ""))
  (bind _asas_throw_base (cast `/Game/Blueprints/SkillSystem/Skills/Attack/Throw/AS_ThrowBase` _scaleeffect))
  (set `/Game/Blueprints/SkillSystem/Skills/Attack/Throw/AS_ThrowBase.throw_full` true _asas_throw_base)
  (set `/Game/Blueprints/SkillSystem/Skills/Attack/Throw/AS_ThrowBase.Item` SStack _asas_throw_base)
  (`self.ChangeWeight`)
  (`/Game/Blueprints/SkillSystem/Skills/Attack/Throw/AS_ThrowBase.Throw` _asas_throw_base))

(fn `DropToSlot`
  (params (Drag :type "/Game/Blueprints/StorageSystem/S_DragData Structure") (Index :type Integer))
  (returns (result :type Boolean))
  (return true))

(fn `EqualSlots`
  (params (A :type "/Game/Data/O_Item Object Reference") (B :type "/Game/Data/O_Item Object Reference"))
  (returns (result :type Boolean))
  (bind (_itemdata_id _itemdata_title) (break `/Game/Data/S_CompBase` (`/Game/Data/O_Item.ItemData` B)))
  (bind (_itemdata_id_2 _itemdata_title_2) (break `/Game/Data/S_CompBase` (`/Game/Data/O_Item.ItemData` A)))
  (return (and (== _itemdata_id _itemdata_id_2) (`KismetStringLibrary.EqualEqual_StrStr` _itemdata_title _itemdata_title_2))))

(fn `GetSlot`
  (params (Index :type Integer))
  (returns (Item :type "/Game/Data/O_Item Object Reference"))
  (return null))

(fn `GetStackFromDrag`
  (params (Drag :type "/Game/Blueprints/StorageSystem/BP_DragItem Object Reference"))
  (returns (Stack :type "/Game/Data/O_Item Object Reference"))
  (bind (_data_aindex _data_data _data_infinite _data_baseactor _data_type) (break `/Game/Blueprints/StorageSystem/S_DragData` (`/Game/Blueprints/StorageSystem/BP_DragItem.Data` Drag)))
  (bind _item (`self.GetSlot` (`/Game/Blueprints/StorageSystem/BFL_Storage.GetStorageByType` _data_baseactor _data_type) _data_aindex))
  (return _item))

(fn `OnRep_ReplicatedData`
  (`self.CLIENT_UpdateData` (`self.ReplicatedData`))
  (`self.OnRepLogic`))

(fn `OnRepLogic`)

(fn `SERVER_UpdateData`)

(fn `SetSlot`
  (params (Index :type Integer) (Item :type "/Game/Data/O_Item Object Reference") (copy :type Boolean))
  (returns (success :type Boolean))
  (return false))

(fn `Swap`
  (params (BaseStorage :type "/Game/Blueprints/StorageSystem/AC_BaseStorage Object Reference") (a :type Integer) (b :type Integer))
  (returns (success :type Boolean))
  (locals (ASlot :type "/Game/Data/O_Item Object Reference") (BSlot :type "/Game/Data/O_Item Object Reference"))
  (bind _basestorage (`local.BaseStorage`))
  (bind _returnvalue (`Actor.GetComponentByClass` (`self.GetOwner`) "/Game/Blueprints/StorageSystem/AC_Equipment.AC_Equipment_C"))
  (bind _item (`self.GetSlot` BaseStorage a))
  (set `local.ASlot` _item)
  (bind _item_2 (`self.GetSlot` (`local.b`)))
  (set `local.BSlot` _item_2)
  (bind _success (`self.SetSlot` _basestorage (`local.a`) (`local.BSlot`) false))
  (if _success
    (bind _success_2 (`self.SetSlot` (`local.b`) (`local.ASlot`)))
    (if _success_2
      (`|ExecutionSequence`
        (:`then_0`
          (if (== (`GameplayStatics.GetObjectClass` _basestorage) "/Game/Blueprints/StorageSystem/Panel/AC_ItemPanel.AC_ItemPanel_C")
            (`/Engine/EditorBlueprintResources/StandardMacros.IsValid` _returnvalue :!label _label
              (:`Is Valid`
                (`/Game/Blueprints/StorageSystem/AC_Equipment.UpdateHands` _returnvalue)))))
        (:`then_1`
          (if (== (`GameplayStatics.GetObjectClass` self) "/Game/Blueprints/StorageSystem/Panel/AC_ItemPanel.AC_ItemPanel_C")
            (goto _label)))
        (:`then_2`
          (`self.ChangeWeight`)
          (return true)))
      (else
        (`self.SetSlot` (`local.BaseStorage`) (`local.a`) (`local.ASlot`) false)
        (`self.SetSlot` (`local.b`) (`local.BSlot`))
        (return false)))
    (else
      (return false))))