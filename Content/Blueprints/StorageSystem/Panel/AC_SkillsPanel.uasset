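; AC_SkillsPanel is a component that holds a ten-slot skill panel with active slot selections for left and right buttons.
; On BeginPlay it fills the Skills array with freshly constructed O_Skill objects.
; GetSkill and SetSkill access slots with bounds checks, updating existing objects in place, and PRINT shows each skill's gameplay tag.
; ChangeActiveSlot shifts either button's selected index, wrapping it with modulo arithmetic.
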(event `self.ReceiveBeginPlay`
  (bind _skills (`self.Skills`))
  (`KismetArrayLibrary.Array_Clear` _skills)
  (for _ (range 10)
    (bind _returnvalue (`|GenericCreateObject` "/Game/Data/O_Skill.O_Skill_C"))
    (`/Game/Data/O_Skill.Set` :`self` _returnvalue)
    (`KismetArrayLibrary.Array_Add` _skills _returnvalue)))

(fn `ChangeActiveSlot`
  (params (Val :type Integer) (RButton :type Boolean))
  (bind (_activeslots_rbutton _activeslots_lbutton) (break `/Game/Blueprints/StorageSystem/Panel/S_SlotsOnPanel` (`self.ActiveSlots`)))
  (if RButton
    (`|VariableSetRef` _activeslots_rbutton (mod (+ _activeslots_rbutton Val 10) 10))
    (else
      (`|VariableSetRef` _activeslots_lbutton (mod (+ _activeslots_lbutton Val 10) 10)))))

(fn `GetSkill`
  (params (Index :type Integer))
  (returns (Output :type "/Game/Data/O_Skill Object Reference"))
  (if (and (> Index -1) (< Index (`KismetArrayLibrary.Array_Length` (`self.Skills`))))
    (return (`|GetArrayItem` (`self.Skills`) Index))))

(fn `PRINT`
  (for _array_element (`self.Skills`)
    (`KismetSystemLibrary.PrintString` (`BlueprintGameplayTagLibrary.GetDebugStringFromGameplayTag` (`/Game/Data/O_Skill.Tag` _array_element)))))

(fn `SetSkill`
  (params (Value :type "GameplayTag Structure") (Index :type Integer))
  (returns (success :type Boolean))
  (bind _skills (`self.Skills`))
  (if (and (> Index -1) (< Index (`KismetArrayLibrary.Array_Length` _skills)))
    (`/Game/Data/O_Skill.Set` (`|GetArrayItem` _skills Index) Value)
    (return true)
    (else
      (return false))))