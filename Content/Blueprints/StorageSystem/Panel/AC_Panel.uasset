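; Actor component that manages a character's item and skill panels, with active left and right hand slots.
; It cycles the active panel and blocks slot changes under a CantSwitchHandItem tag.
; GetSkillInHand resolves each hand's one- or two-handed skill from the active slot, with punch fallbacks.
; For replication, the active panel is serialized and a Notifyer counter bumped, so its OnRep rebuilds slots and refreshes the UI.
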(event `self.ReceiveBeginPlay`
  (`/Engine/EditorBlueprintResources/ActorComponentMacros.Switch Has Authority`
    (:`Remote`
      (`self.InitPanels` 1 1))))

(event `InitPanels`
  (params (ItemPanels :type Integer) (SkillPanels :type Integer))
  (bind _returnvalue (`self.GetOwner`))
  (`KismetArrayLibrary.Array_Clear` (`self.ItemPanels`))
  (`KismetArrayLibrary.Array_Clear` (`self.SkillPanels`))
  (`|ExecutionSequence`
    (:`then_1`
      (for _ (range 1 (+ ItemPanels 1))
        (bind _returnvalue_2 (`|AddComponentByClass` :`self` _returnvalue :`Class` "/Game/Blueprints/StorageSystem/Panel/AC_ItemPanel.AC_ItemPanel_C"))
        (`KismetArrayLibrary.Array_Add` (`self.ItemPanels`) _returnvalue_2)
        (add `/Game/Blueprints/StorageSystem/AC_ItemStorage.UpdateData` _returnvalue_2 (delegate `Serialize`)))
      (for _ (range 1 (+ SkillPanels 1))
        (bind _returnvalue_3 (`|AddComponentByClass` _returnvalue "/Game/Blueprints/StorageSystem/Panel/AC_SkillsPanel.AC_SkillsPanel_C"))
        (`KismetArrayLibrary.Array_Add` (`self.SkillPanels`) _returnvalue_3)))))

(event `Serialize`
  (`self.SERVER_UpdatePanel`))

(event `UpdatePanel`
  (params (items :type Boolean) (Slots :type "/Game/Blueprints/StorageSystem/Panel/S_SlotsOnPanel Structure (by ref)"))
  (bind (_serializedskills_activeslots _serializedskills_items) (break `/Game/Blueprints/SaveLoad/Base/S_SAVE_SKILL_PANEL` (`self.SerializedSkills`)))
  (bind (_serializeditems_activeslots _serializeditems_items) (break `/Game/Blueprints/SaveLoad/Base/S_SAVE_ITEM_PANEL` (`self.SerializedItems`)))
  (bind _output (`|GetArrayItem` (`self.ItemPanels`)))
  (bind _output_2 (`|GetArrayItem` (`self.SkillPanels`)))
  (if items
    (`/Engine/EditorBlueprintResources/StandardMacros.IsValid` _output
      (:`Is Valid`
        _)
      (:`Is Not Valid`
        (`self.InitPanels` 1 1)))
    (for (_array_element _array_index) _serializeditems_items
      (bind _result (`/Game/Blueprints/SaveLoad/BFL_SaveLoad.DeSerializeItem` _array_element))
      (`/Game/Blueprints/StorageSystem/AC_BaseStorage.SetSlot` _output _array_index _result false))
    (set `/Game/Blueprints/StorageSystem/Panel/AC_ItemPanel.ActiveSlots` Slots _output)
    (else
      (for (_array_element_2 _array_index_2) _serializedskills_items
        (`/Game/Blueprints/StorageSystem/Panel/AC_SkillsPanel.SetSkill` _output_2 _array_element_2 _array_index_2))
      (set `/Game/Blueprints/StorageSystem/Panel/AC_SkillsPanel.ActiveSlots` Slots _output_2))))

(event `CLIENT_UpdatePanel`
  (params (items :type Boolean) (Slots :type "/Game/Blueprints/StorageSystem/Panel/S_SlotsOnPanel Structure (by ref)"))
  (bind _returnvalue (`Actor.GetComponentByClass` (`self.GetOwner`) "/Game/UI/AC_UIManager.AC_UIManager_C"))
  (`self.UpdatePanel` items Slots)
  (`/Game/UI/AC_UIManager.UpdateUI` _returnvalue "NewEnumerator2")
  (`/Game/UI/AC_UIManager.UpdateActiveSlots` _returnvalue))

(fn `ChangeActiveSlot`
  (params (Val :type Integer) (RButton :type Boolean))
  (returns (Result :type "/Game/Blueprints/StorageSystem/Panel/S_SlotsOnPanel Structure"))
  (bind _returnvalue (`KismetArrayLibrary.Array_Contains` (`/Game/Blueprints/SkillSystem/AC_SkillComponent.Tags` (`Actor.GetComponentByClass` (`self.GetOwner`) "/Game/Blueprints/SkillSystem/AC_SkillComponent.AC_SkillComponent_C")) (struct :`TagName` "Effects.Negative.Hands.CantSwitchHandItem")))
  (bind _result (`self.GetActivePanel`))
  (bind _asac_skills_panel (cast `/Game/Blueprints/StorageSystem/Panel/AC_SkillsPanel` _result)
    (:`then`
      (if (not _returnvalue)
        (`/Game/Blueprints/StorageSystem/Panel/AC_SkillsPanel.ChangeActiveSlot` _asac_skills_panel Val RButton))
      (return (`/Game/Blueprints/StorageSystem/Panel/AC_SkillsPanel.ActiveSlots` _asac_skills_panel)))
    (:`CastFailed`
      (bind _asac_item_panel (cast `/Game/Blueprints/StorageSystem/Panel/AC_ItemPanel` _result))
      (if (not _returnvalue)
        (`/Game/Blueprints/StorageSystem/Panel/AC_ItemPanel.ChangeActiveSlot` _asac_item_panel Val RButton))
      (return (`/Game/Blueprints/StorageSystem/Panel/AC_ItemPanel.ActiveSlots` _asac_item_panel)))))

(fn `GetActivePanel`
  (returns (Result :type "ActorComponent Object Reference"))
  (bind _activepanelindex (`self.ActivePanelIndex`))
  (bind _returnvalue (`KismetArrayLibrary.Array_Length` (`self.ItemPanels`)))
  (if (< _activepanelindex _returnvalue)
    (return (`|GetArrayItem` (`self.ItemPanels`) _activepanelindex))
    (else
      (return (`|GetArrayItem` (`self.SkillPanels`) (- _activepanelindex _returnvalue))))))

(fn `GetActiveSlots`
  (returns (Result :type "/Game/Blueprints/StorageSystem/Panel/S_SlotsOnPanel Structure"))
  (bind _activepanelindex (`self.ActivePanelIndex`))
  (bind _returnvalue (`KismetArrayLibrary.Array_Length` (`self.ItemPanels`)))
  (if (< _activepanelindex _returnvalue)
    (return (`/Game/Blueprints/StorageSystem/Panel/AC_ItemPanel.ActiveSlots` (`|GetArrayItem` (`self.ItemPanels`) _activepanelindex)))
    (else
      (return (`/Game/Blueprints/StorageSystem/Panel/AC_SkillsPanel.ActiveSlots` (`|GetArrayItem` (`self.SkillPanels`) (- _activepanelindex _returnvalue)))))))

(fn `GetHandItem`
  (params (RightHand :type Boolean))
  (returns (index :type Integer) (Item :type "/Game/Data/O_Item Object Reference") (is_valid_panel :type Boolean))
  (bind _result (`self.GetActivePanel`))
  (bind _asac_item_panel (cast `/Game/Blueprints/StorageSystem/Panel/AC_ItemPanel` _result)
    (:`then`
      (bind (_activeslots_rbutton _activeslots_lbutton) (break `/Game/Blueprints/StorageSystem/Panel/S_SlotsOnPanel` (`/Game/Blueprints/StorageSystem/Panel/AC_ItemPanel.ActiveSlots` _asac_item_panel)))
      (bind _returnvalue (`KismetMathLibrary.SelectInt` _activeslots_rbutton _activeslots_lbutton RightHand))
      (bind _item (`/Game/Blueprints/StorageSystem/AC_BaseStorage.GetSlot` _asac_item_panel _returnvalue))
      (return _returnvalue _item true))
    (:`CastFailed`
      (bind _result_2 (`/Game/Blueprints/Items/BFL_Items.CreateItemByName` "air"))
      (bind (_itemdata_id _itemdata_title _itemdata_count _itemdata_stacksize _itemdata_objecttype _itemdata_posonbody _itemdata_tier _itemdata_hands _itemdata_actorclass _itemdata_weight _itemdata_durability _itemdata_maxdurability _itemdata_skillr _itemdata_skilll _itemdata_skill2r _itemdata_skill2l) (break `/Game/Data/S_CompBase` (`/Game/Data/O_Item.ItemData` _result_2)))
      (set `/Game/Data/O_Item.ItemData` (make `/Game/Data/S_CompBase` _itemdata_id _itemdata_title _itemdata_count _itemdata_stacksize _itemdata_objecttype _itemdata_posonbody _itemdata_tier "NewEnumerator7" _itemdata_actorclass _itemdata_weight _itemdata_durability _itemdata_maxdurability _itemdata_skillr _itemdata_skilll _itemdata_skill2r _itemdata_skill2l) _result_2)
      (return 0 _result_2 false))))

(fn `GetHandSkill`
  (params (RightHand :type Boolean))
  (returns (index :type Integer) (Output :type "/Game/Data/O_Skill Object Reference") (is_valid_panel :type Boolean))
  (bind _result (`self.GetActivePanel`))
  (bind _asac_skills_panel (cast `/Game/Blueprints/StorageSystem/Panel/AC_SkillsPanel` _result)
    (:`then`
      (bind (_activeslots_rbutton _activeslots_lbutton) (break `/Game/Blueprints/StorageSystem/Panel/S_SlotsOnPanel` (`/Game/Blueprints/StorageSystem/Panel/AC_SkillsPanel.ActiveSlots` _asac_skills_panel)))
      (bind _returnvalue (`KismetMathLibrary.SelectInt` _activeslots_rbutton _activeslots_lbutton RightHand))
      (bind _output (`/Game/Blueprints/StorageSystem/Panel/AC_SkillsPanel.GetSkill` _asac_skills_panel _returnvalue))
      (return _returnvalue _output true))
    (:`CastFailed`
      (return -1 null false))))

(fn `GetSkillInHand`
  (params (`Right btn` :type Boolean))
  (returns (Source :type "/Game/Blueprints/SkillSystem/E_SkillSource Enum") (Holder :type "/Game/Blueprints/Items/BP_Item Object Reference") (Skill :type "/Game/Blueprints/SkillSystem/Skills/A_Skill Class Reference"))
  (locals (IsTwoHanded :type Boolean) (Src :type "/Game/Blueprints/SkillSystem/E_SkillSource Enum"))
  (bind _returnvalue (not `Right btn`))
  (bind _right_btn (`local.Right btn`))
  (bind _src (`local.Src`))
  (bind _src_2 (`local.Src`))
  (bind _right_btn_2 (`local.Right btn`))
  (bind _returnvalue_2 (`KismetMathLibrary.Conv_ByteToInt` (enumliteral `/Game/Data/Equipment/E_EquipmentSlot` "NewEnumerator9")))
  (bind _returnvalue_3 (select `/Game/Blueprints/SkillSystem/E_SkillSource` _src_2 :`NewEnumerator1` "/Game/Blueprints/SkillSystem/Skills/Attack/Punch/AS_PunchR.AS_PunchR_C" :`NewEnumerator2` "/Game/Blueprints/SkillSystem/Skills/Attack/Punch/AS_PunchL.AS_PunchL_C" :`NewEnumerator3` "/Game/Blueprints/SkillSystem/Skills/Attack/Punch/AS_Punch2R.AS_Punch2R_C" :`NewEnumerator4` "/Game/Blueprints/SkillSystem/Skills/Attack/Punch/AS_Punch2L.AS_Punch2L_C" :!type "/Game/Blueprints/SkillSystem/Skills/A_Skill Class Reference"))
  (bind (_index _item _is_valid_panel) (`self.GetHandItem` `Right btn`))
  (if _is_valid_panel
    (bind (_index_2 _item_2) (`self.GetHandItem` _returnvalue))
    (bind _output_get (set `local.IsTwoHanded` (== _index_2 _index)))
    (bind _itemdata_id (break `/Game/Data/S_CompBase` (`/Game/Data/O_Item.ItemData` _item_2)))
    (bind _itemdata_id_2 (break `/Game/Data/S_CompBase` (`/Game/Data/O_Item.ItemData` _item)))
    (set `local.Src` (select `bool` (or (and (== _itemdata_id _itemdata_id_2) (== _itemdata_id_2 "air")) (`local.IsTwoHanded`)) :`false` (select `bool` _right_btn :`false` "NewEnumerator2" :`true` "NewEnumerator1" :!type "/Game/Blueprints/SkillSystem/E_SkillSource Enum") :`true` (select `bool` _right_btn :`false` "NewEnumerator4" :`true` "NewEnumerator3" :!type "/Game/Blueprints/SkillSystem/E_SkillSource Enum")))
    (bind (_itemdata_id_3 _itemdata_title _itemdata_count _itemdata_stacksize _itemdata_objecttype _itemdata_posonbody _itemdata_tier _itemdata_hands _itemdata_actorclass _itemdata_weight _itemdata_durability _itemdata_maxdurability _itemdata_skillr _itemdata_skilll _itemdata_skill2r _itemdata_skill2l) (break `/Game/Data/S_CompBase` (`/Game/Data/O_Item.ItemData` _item)))
    (if (== _itemdata_id_3 "air")
      (return _src null _returnvalue_3)
      (else
        (return _src (`BlueprintMapLibrary.Map_Find` (`/Game/Blueprints/StorageSystem/AC_Equipment.Items` (`Actor.GetComponentByClass` (`self.GetOwner`) "/Game/Blueprints/StorageSystem/AC_Equipment.AC_Equipment_C")) (cast `/Game/Data/Equipment/E_EquipmentSlot` (`KismetMathLibrary.Conv_IntToByte` (`KismetMathLibrary.SelectInt` _returnvalue_2 (`KismetMathLibrary.SelectInt` _returnvalue_2 (`KismetMathLibrary.Conv_ByteToInt` (enumliteral `/Game/Data/Equipment/E_EquipmentSlot` "NewEnumerator10")) `Right btn`) _output_get)))) (select `bool` (== (`KismetSystemLibrary.MakeLiteralByte` _itemdata_objecttype) (`KismetSystemLibrary.MakeLiteralByte` (enumliteral `/Game/Data/BaseData/E_ObjectType` "NewEnumerator5"))) :`false` (select `bool` (== (`KismetSystemLibrary.MakeLiteralByte` _itemdata_objecttype) (`KismetSystemLibrary.MakeLiteralByte` (enumliteral `/Game/Data/BaseData/E_ObjectType` "NewEnumerator2"))) :`false` (select `/Game/Blueprints/SkillSystem/E_SkillSource` (`local.Src`) :`NewEnumerator1` _itemdata_skillr :`NewEnumerator2` _itemdata_skilll :`NewEnumerator3` _itemdata_skill2r :`NewEnumerator4` _itemdata_skill2l) :`true` "/Game/Blueprints/SkillSystem/Skills/Base/AS_EquipItem.AS_EquipItem_C")))))
    (else
      (bind (_index_3 _output) (`self.GetHandSkill` `Right btn`))
      (bind _index_4 (`self.GetHandSkill` _returnvalue))
      (bind _output_get_2 (set `local.IsTwoHanded` (== _index_4 _index_3)))
      (set `local.Src` (select `bool` _output_get_2 :`false` (select `bool` _right_btn_2 :`false` "NewEnumerator2" :`true` "NewEnumerator1" :!type "/Game/Blueprints/SkillSystem/E_SkillSource Enum") :`true` (select `bool` _right_btn_2 :`false` "NewEnumerator4" :`true` "NewEnumerator3" :!type "/Game/Blueprints/SkillSystem/E_SkillSource Enum")))
      (bind _returnvalue_4 (select `/Game/Blueprints/SkillSystem/E_SkillSource` _src_2 :`NewEnumerator1` (`/Game/Data/O_Skill.SkillR` _output) :`NewEnumerator2` (`/Game/Data/O_Skill.SkillL` _output) :`NewEnumerator3` (`/Game/Data/O_Skill.Skill2R` _output) :`NewEnumerator4` (`/Game/Data/O_Skill.Skill2L` _output)))
      (return _src_2 null (select `bool` (== _returnvalue_4 null) :`false` _returnvalue_4 :`true` _returnvalue_3)))))

(fn `OnRep_Notifyer`
  (bind _items_panel_active (`self.Items_panel_active`))
  (bind _serializeditems_activeslots (break `/Game/Blueprints/SaveLoad/Base/S_SAVE_ITEM_PANEL` (`self.SerializedItems`)))
  (bind _serializedskills_activeslots (break `/Game/Blueprints/SaveLoad/Base/S_SAVE_SKILL_PANEL` (`self.SerializedSkills`)))
  (bind _returnvalue (select `bool` _items_panel_active :`false` _serializedskills_activeslots :`true` _serializeditems_activeslots))
  (`self.UpdatePanel` _items_panel_active _returnvalue)
  (`self.CLIENT_UpdatePanel` (`self.Items_panel_active`) _returnvalue))

(fn `PRINT_ITEMS`
  (for _array_element (`self.ItemPanels`)
    (`/Game/Blueprints/StorageSystem/AC_ItemStorage.PRINT` _array_element)
    (`KismetSystemLibrary.PrintString` "------")))

(fn `PRINT_SKILLS`
  (for _array_element (`self.SkillPanels`)
    (`/Game/Blueprints/StorageSystem/Panel/AC_SkillsPanel.PRINT` _array_element)
    (`KismetSystemLibrary.PrintString` "------")))

(fn `SERVER_UpdatePanel`
  (locals (Items :type "Array of /Game/Blueprints/SaveLoad/Base/S_SAVE_DATA_ITEM Structure") (Skills :type "Array of GameplayTag Structure") (NewLocalVar :type "/Game/Blueprints/StorageSystem/Panel/S_SlotsOnPanel Structure"))
  (bind _items (`local.Items`))
  (`|ExecutionSequence`
    (:`then_0`
      (bind _result (`self.GetActivePanel`))
      (bind _asac_item_panel (cast `/Game/Blueprints/StorageSystem/Panel/AC_ItemPanel` _result)
        (:`then`
          (set `self.Items_panel_active` true)
          (set `self.SerializedItems` (struct))
          (for _array_element (`/Game/Blueprints/StorageSystem/AC_ItemStorage.Items` _asac_item_panel)
            (bind _result_2 (`/Game/Data/O_Item.Serialize` _array_element))
            (`KismetArrayLibrary.Array_Add` _items _result_2))
          (bind _activeslots (`/Game/Blueprints/StorageSystem/Panel/AC_ItemPanel.ActiveSlots` _asac_item_panel))
          (set `local.NewLocalVar` _activeslots)
          (set `self.SerializedItems` (make `/Game/Blueprints/SaveLoad/Base/S_SAVE_ITEM_PANEL` _activeslots _items)))
        (:`CastFailed`
          (bind _asac_skills_panel (cast `/Game/Blueprints/StorageSystem/Panel/AC_SkillsPanel` _result))
          (set `self.Items_panel_active` false)
          (set `self.SerializedSkills` (struct))
          (for _array_element_2 (`/Game/Blueprints/StorageSystem/Panel/AC_SkillsPanel.Skills` _asac_skills_panel)
            (`KismetArrayLibrary.Array_Add` (`local.Skills`) (`/Game/Data/O_Skill.Tag` _array_element_2)))
          (bind _activeslots_2 (`/Game/Blueprints/StorageSystem/Panel/AC_SkillsPanel.ActiveSlots` _asac_skills_panel))
          (set `local.NewLocalVar` _activeslots_2)
          (set `self.SerializedSkills` (make `/Game/Blueprints/SaveLoad/Base/S_SAVE_SKILL_PANEL` _activeslots_2 (`local.Skills`))))))
    (:`then_1`
      (set `self.Notifyer` (+ (`self.Notifyer`) 1)))))

(fn `SetActiveSlots`
  (params (Val :type Integer) (RButton :type Boolean))
  (returns (Result :type "/Game/Blueprints/StorageSystem/Panel/S_SlotsOnPanel Structure") (has_changes :type Boolean))
  (bind _returnvalue (`KismetArrayLibrary.Array_Contains` (`/Game/Blueprints/SkillSystem/AC_SkillComponent.Tags` (`Actor.GetComponentByClass` (`self.GetOwner`) "/Game/Blueprints/SkillSystem/AC_SkillComponent.AC_SkillComponent_C")) (struct :`TagName` "Effects.Negative.Hands.CantSwitchHandItem")))
  (bind _result (`self.GetActivePanel`))
  (bind _asac_skills_panel (cast `/Game/Blueprints/StorageSystem/Panel/AC_SkillsPanel` _result)
    (:`then`
      (if (not _returnvalue)
        (bind (_activeslots_rbutton _activeslots_lbutton) (break `/Game/Blueprints/StorageSystem/Panel/S_SlotsOnPanel` (`/Game/Blueprints/StorageSystem/Panel/AC_SkillsPanel.ActiveSlots` _asac_skills_panel)))
        (if (== Val (`KismetMathLibrary.SelectInt` _activeslots_rbutton _activeslots_lbutton RButton))
          _
          (else
            (bind _output_get (set `/Game/Blueprints/StorageSystem/Panel/AC_SkillsPanel.ActiveSlots` (select `bool` RButton :`false` (make `/Game/Blueprints/StorageSystem/Panel/S_SlotsOnPanel` _activeslots_rbutton Val) :`true` (make `/Game/Blueprints/StorageSystem/Panel/S_SlotsOnPanel` Val _activeslots_lbutton) :!type "/Game/Blueprints/StorageSystem/Panel/S_SlotsOnPanel Structure") _asac_skills_panel))
            (return _output_get true))))
      (return (make `/Game/Blueprints/StorageSystem/Panel/S_SlotsOnPanel` _activeslots_rbutton _activeslots_lbutton) false))
    (:`CastFailed`
      (bind _asac_item_panel (cast `/Game/Blueprints/StorageSystem/Panel/AC_ItemPanel` _result))
      (if (not _returnvalue)
        (bind (_activeslots_rbutton_2 _activeslots_lbutton_2) (break `/Game/Blueprints/StorageSystem/Panel/S_SlotsOnPanel` (`/Game/Blueprints/StorageSystem/Panel/AC_ItemPanel.ActiveSlots` _asac_item_panel)))
        (if (== Val (`KismetMathLibrary.SelectInt` _activeslots_rbutton_2 _activeslots_lbutton_2 RButton))
          _
          (else
            (bind _output_get_2 (set `/Game/Blueprints/StorageSystem/Panel/AC_ItemPanel.ActiveSlots` (select `bool` RButton :`false` (make `/Game/Blueprints/StorageSystem/Panel/S_SlotsOnPanel` _activeslots_rbutton_2 Val) :`true` (make `/Game/Blueprints/StorageSystem/Panel/S_SlotsOnPanel` Val _activeslots_lbutton_2) :!type "/Game/Blueprints/StorageSystem/Panel/S_SlotsOnPanel Structure") _asac_item_panel))
            (return _output_get_2 true))))
      (return (make `/Game/Blueprints/StorageSystem/Panel/S_SlotsOnPanel` _activeslots_rbutton_2 _activeslots_lbutton_2) false))))

(fn `SwapPanel`
  (returns (Return :type Integer))
  (bind _output_get (set `self.ActivePanelIndex` (mod (+ (`self.ActivePanelIndex`) 1) (+ (`KismetArrayLibrary.Array_Length` (`self.ItemPanels`)) (`KismetArrayLibrary.Array_Length` (`self.SkillPanels`))))))
  (return _output_get))