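; AC_ItemPanel is a storage component for a ten-slot item panel with separate active slots for the left and right buttons.
; On BeginPlay it fills Items with "air" O_Item placeholders.
; SetSlot bounds-checks, then stores a fresh copy, copies into a matching-ID item, or replaces the reference.
; ChangeActiveSlot wraps either selection around the ten slots, PRINT shows both, and CLIENTUpdateData is empty.
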(event `self.ReceiveBeginPlay`
  (bind _items (`self.Items`))
  (`parent.ReceiveBeginPlay`)
  (`KismetArrayLibrary.Array_Clear` _items)
  (for _ (range 10)
    (bind _returnvalue (`|GenericCreateObject` "/Game/Data/O_Item.O_Item_C"))
    (`/Game/Data/O_Item.SetByName` _returnvalue "air")
    (`KismetArrayLibrary.Array_Add` _items _returnvalue)))

(event `self.CLIENT_UpdateData`
  (params (ReplicatedData :type "Array of /Game/Blueprints/SaveLoad/Base/S_SAVE_DATA_ITEM Structure (by ref)")))

(fn `ChangeActiveSlot`
  (params (Val :type Integer) (RButton :type Boolean))
  (bind (_activeslots_rbutton _activeslots_lbutton) (break `/Game/Blueprints/StorageSystem/Panel/S_SlotsOnPanel` (`self.ActiveSlots`)))
  (if RButton
    (`|VariableSetRef` _activeslots_rbutton (mod (+ _activeslots_rbutton Val 10) 10))
    (else
      (`|VariableSetRef` _activeslots_lbutton (mod (+ _activeslots_lbutton Val 10) 10)))))

(fn `GetSlot`
  (params (Index :type Integer))
  (returns (Item :type "/Game/Data/O_Item Object Reference"))
  (if (and (> Index -1) (< Index (`KismetArrayLibrary.Array_Length` (`self.Items`))))
    (return (`|GetArrayItem` (`self.Items`) Index))
    (else
      (return null))))

(fn `PRINT`
  (bind (_activeslots_rbutton _activeslots_lbutton) (break `/Game/Blueprints/StorageSystem/Panel/S_SlotsOnPanel` (`self.ActiveSlots`)))
  (`parent.PRINT`)
  (`KismetSystemLibrary.PrintString` (`KismetStringLibrary.Concat_StrStr` "R " (`KismetStringLibrary.Conv_IntToString` _activeslots_rbutton) "   " "L " (`KismetStringLibrary.Conv_IntToString` _activeslots_lbutton))))

(fn `SetSlot`
  (params (Index :type Integer) (Item :type "/Game/Data/O_Item Object Reference") (copy :type Boolean))
  (returns (success :type Boolean))
  (bind _itemdata_id (break `/Game/Data/S_CompBase` (`/Game/Data/O_Item.ItemData` Item)))
  (if (and (> Index -1) (< Index (`KismetArrayLibrary.Array_Length` (`self.Items`))))
    (if copy
      (bind _result (`/Game/Blueprints/Items/BFL_Items.CreateItemByName` _itemdata_id))
      (`/Game/Data/O_Item.Copy` _result Item)
      (`KismetArrayLibrary.Array_Set` (`self.Items`) Index _result)
      (return true)
      (else
        (bind _item (`self.GetSlot` Index))
        (bind _itemdata_id_2 (break `/Game/Data/S_CompBase` (`/Game/Data/O_Item.ItemData` _item)))
        (if (== _itemdata_id _itemdata_id_2)
          (`/Game/Data/O_Item.Copy` _item Item)
          (else
            (`KismetArrayLibrary.Array_Set` (`self.Items`) Index Item)))
        (return true)))
    (else
      (return false))))