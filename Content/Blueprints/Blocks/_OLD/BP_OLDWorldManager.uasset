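; Legacy world manager for a chunked block world, which loads a small grid of chunks on BeginPlay.
; Saved ChunkData becomes spawned BP_ChunkMesh actors of 16x16 blocks in two Z layers, and converts back for saving.
; SetBlock finds chunks by scanning all chunk actors, loading missing ones.
; Layer helpers generate through WorldGen, save, build meshes or export PNG maps colored from DT_DataBlocks, but their event-graph calls are disconnected.
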(event `self.ReceiveBeginPlay`
  (bind _chunk (`self.CreateChunks` -2 2 0 2)))

(fn `_LAYER`
  (params (Name :type "E_Layer Enum" :default "test") (SaveToFile :type Boolean) (SaveToPNG :type Boolean) (Split :type Boolean) (Create :type Boolean) (Gen :type "WorldGen Object Reference") (Size :type Integer))
  (bind (_returnvalue_x _returnvalue_y) (`KismetMathLibrary.BreakVector2D` (`WorldGen.getSector` Gen)))
  (bind _returnvalue (`WorldGen.GenLayer` Gen Size Name))
  (`/Engine/EditorBlueprintResources/StandardMacros.IsValid` _returnvalue
    (:`Is Valid`
      (`|ExecutionSequence`
        (:`then_0`
          (if SaveToFile
            (`SaveLoad.SaveGameLayer` _returnvalue Name (`WorldGen.getSector` Gen))))
        (:`then_1`
          (if SaveToPNG
            (`self.SaveToPNG` _returnvalue (`KismetStringLibrary.Concat_StrStr` (`KismetStringLibrary.Concat_StrStr` (`|GetEnumeratorNameAsString` Name) " ") (`KismetStringLibrary.Concat_StrStr` (`KismetStringLibrary.Conv_DoubleToString` _returnvalue_x) (`KismetStringLibrary.Conv_DoubleToString` _returnvalue_y))) Split)))
        (:`then_2`
          (if Create
            (`self.CreateLayerMesh` _returnvalue)))))
    (:`Is Not Valid`
      (`KismetSystemLibrary.PrintString` "ERROR: Layer is not valid"))))

(fn `ChunkDataToChunkMesh`
  (params (Data :type "ChunkData Object Reference"))
  (returns (Mesh :type "/Game/Blueprints/Blocks/_OLD/BP_ChunkMesh Object Reference"))
  (bind _data (`local.Data`))
  (bind _data_2 (`local.Data`))
  (`/Engine/EditorBlueprintResources/StandardMacros.IsValid` Data
    (:`Is Valid`
      (bind _returnvalue (`|SpawnActorFromClass` "/Game/Blueprints/Blocks/_OLD/BP_ChunkMesh.BP_ChunkMesh_C" (`KismetMathLibrary.Conv_VectorToTransform` (* (`KismetMathLibrary.Conv_Vector2DToVector` (`ChunkData.getPosition` Data)) 100)) "Undefined" "MultiplyWithRoot" null null))
      (for _index (range 16)
        (for _index_2 (range 16)
          (`/Game/Blueprints/Blocks/_OLD/BP_ChunkMesh.CreateBlock` _returnvalue _index _index_2 false (`ChunkData.getBlock` _data _index _index_2 false))
          (`/Game/Blueprints/Blocks/_OLD/BP_ChunkMesh.CreateBlock` _returnvalue _index _index_2 true (`ChunkData.getBlock` _data _index _index_2 true))))
      (set `/Game/Blueprints/Blocks/_OLD/BP_ChunkMesh.Position` (`KismetMathLibrary.Conv_Vector2DToVector` (`ChunkData.getPosition` _data_2)) _returnvalue)
      (set `/Game/Blueprints/Blocks/_OLD/BP_ChunkMesh.Type` (`ChunkData.getType` _data_2) _returnvalue)
      (set `/Game/Blueprints/Blocks/_OLD/BP_ChunkMesh.Biome` (`ChunkData.getBiome` _data_2) _returnvalue)
      (return _returnvalue))
    (:`Is Not Valid`
      (`KismetSystemLibrary.PrintString` "ERROR: ChunkData is not valid")
      (return null))))

(fn `ChunkMeshToChunkData`
  (params (Mesh :type "/Game/Blueprints/Blocks/_OLD/BP_ChunkMesh Object Reference"))
  (returns (Data :type "ChunkData Object Reference"))
  (locals (nums :type "Array of Integer"))
  (bind _mesh (`local.Mesh`))
  (bind _mesh_2 (`local.Mesh`))
  (`/Engine/EditorBlueprintResources/StandardMacros.IsValid` Mesh
    (:`Is Valid`
      (bind _returnvalue (`|GenericCreateObject` "/Script/Test.ChunkData"))
      (`ChunkData.setPosition` _returnvalue (`KismetMathLibrary.Conv_VectorToVector2D` (`/Game/Blueprints/Blocks/_OLD/BP_ChunkMesh.Position` _mesh)))
      (`ChunkData.setType` _returnvalue (`/Game/Blueprints/Blocks/_OLD/BP_ChunkMesh.Type` _mesh))
      (`ChunkData.setBiome` _returnvalue (`/Game/Blueprints/Blocks/_OLD/BP_ChunkMesh.Biome` _mesh))
      (for _index (range 16)
        (for _index_2 (range 16)
          (`ChunkData.setBlock` _returnvalue _index _index_2 false (`KismetStringLibrary.Conv_StringToName` (`/Game/Blueprints/Blocks/_OLD/BP_ChunkMesh.GetBlock` _mesh_2 _index _index_2 false)))
          (`ChunkData.setBlock` _returnvalue 0 0 true (`KismetStringLibrary.Conv_StringToName` (`/Game/Blueprints/Blocks/_OLD/BP_ChunkMesh.GetBlock` _mesh_2 _index _index_2 true)))))
      (return _returnvalue))
    (:`Is Not Valid`
      (`KismetSystemLibrary.PrintString` "ERROR: ChunkMesh is not valid")
      (return null))))

(fn `CreateChunks`
  (params (Xstart :type Integer) (Xend :type Integer) (Ystart :type Integer) (Yend :type Integer))
  (returns (chunk :type "Set of /Game/Blueprints/Blocks/_OLD/BP_ChunkMesh Object Reference"))
  (locals (ChunksReturn :type "Set of /Game/Blueprints/Blocks/_OLD/BP_ChunkMesh Object Reference") (Positions :type "Array of Vector2D Structure"))
  (for _index (range (`KismetMathLibrary.Min` Xstart Xend) (+ (`KismetMathLibrary.Max` Xstart Xend) 1))
    (for _index_2 (range (`KismetMathLibrary.Min` Ystart Yend) (+ (`KismetMathLibrary.Max` Yend Yend) 1))
      (`KismetArrayLibrary.Array_Add` (`local.Positions`) (`KismetMathLibrary.MakeVector2D` (`KismetMathLibrary.Conv_IntToDouble` _index) (`KismetMathLibrary.Conv_IntToDouble` _index_2)))))
  (bind (_bsuccess _message _returnvalue) (`SaveLoad.LoadChunks` (`local.Positions`) (`self.name`)))
  (if _bsuccess
    (for _array_element _returnvalue
      (bind _mesh (`self.ChunkDataToChunkMesh` _array_element))
      (`self.K2_SetActorLocation` _mesh (* (`/Game/Blueprints/Blocks/_OLD/BP_ChunkMesh.Position` _mesh) 1600) false false)
      (`BlueprintSetLibrary.Set_Add` (`local.ChunksReturn`) _mesh))
    (return (`local.ChunksReturn`))
    (else
      (`KismetSystemLibrary.PrintString` (`KismetStringLibrary.Concat_StrStr` "ERROR: " _message))
      (return))))

(fn `CreateLayerMesh`
  (params (Layer :type "LayerData Object Reference"))
  (bind _returnvalue (- (`LayerData.getChunkCount` Layer) 1))
  (`/Engine/EditorBlueprintResources/StandardMacros.IsValid` Layer
    (:`Is Valid`
      (for _index (range (+ _returnvalue 1))
        (for _index_2 (range (+ _returnvalue 1))
          (bind _returnvalue_2 (`LayerData.getChunk` Layer _index _index_2))
          (`/Engine/EditorBlueprintResources/StandardMacros.IsValid` _returnvalue_2
            (:`Is Valid`
              (bind _mesh (`self.ChunkDataToChunkMesh` _returnvalue_2))
              (bind (_returnvalue_x _returnvalue_y _returnvalue_z) (`KismetMathLibrary.BreakVector` (* (`/Game/Blueprints/Blocks/_OLD/BP_ChunkMesh.Position` _mesh) 1600)))
              (`self.K2_SetActorLocation` _mesh (`KismetMathLibrary.MakeVector` _returnvalue_x _returnvalue_y _returnvalue_z) false false))
            (:`Is Not Valid`
              (`KismetSystemLibrary.PrintString` (`KismetStringLibrary.Concat_StrStr` (`KismetStringLibrary.Concat_StrStr` (`KismetStringLibrary.Concat_StrStr` (`KismetStringLibrary.Concat_StrStr` "ERROR: chunk " (`KismetStringLibrary.Conv_IntToString` _index))) (`KismetStringLibrary.Conv_IntToString` _index_2)) " is not valid")))))))
    (:`Is Not Valid`
      (`KismetSystemLibrary.PrintString` "ERROR: Layer is not valid"))))

(fn `DeleteChunks`
  (params (XStart :type Integer) (XEnd :type Integer) (YStart :type Integer) (YEnd :type Integer))
  (for _index (range XStart (+ XEnd 1))
    (for _index_2 (range YStart (+ YEnd 1))
      (bind _chunk (`self.FindChunk` (`KismetMathLibrary.MakeVector` (`KismetMathLibrary.Conv_IntToDouble` _index) (`KismetMathLibrary.Conv_IntToDouble` _index_2))))
      (`/Engine/EditorBlueprintResources/StandardMacros.IsValid` _chunk
        (:`Is Valid`
          (`/Game/Blueprints/Blocks/_OLD/BP_ChunkMesh.DeleteChunk` _chunk)
          (`self.K2_DestroyActor` _chunk))))))

(fn `FindChunk`
  (params (Position :type "Vector Structure"))
  (returns (Chunk :type "/Game/Blueprints/Blocks/_OLD/BP_ChunkMesh Object Reference"))
  (bind _outactors (`GameplayStatics.GetAllActorsOfClass` "/Game/Blueprints/Blocks/_OLD/BP_ChunkMesh.BP_ChunkMesh_C"))
  (for _array_element _outactors
    (bind (_position_x _position_y) (`KismetMathLibrary.BreakVector` (`/Game/Blueprints/Blocks/_OLD/BP_ChunkMesh.Position` _array_element)))
    (if (and (== _position_x Position_X) (== _position_y Position_Y))
      (return _array_element)))
  (return null))

(fn `Save Chunks`
  (params (ChunksToSave :type "Array of /Game/Blueprints/Blocks/_OLD/BP_ChunkMesh Object Reference"))
  (locals (Data :type "Array of ChunkData Object Reference"))
  (bind _data (`local.Data`))
  (for _array_element ChunksToSave
    (bind _data_2 (`self.ChunkMeshToChunkData` _array_element))
    (`KismetArrayLibrary.Array_Add` _data _data_2))
  (bind (_bsuccess _message) (`SaveLoad.SaveChunks` _data (`self.name`)))
  (`KismetSystemLibrary.PrintString` _message))

(fn `SaveToPNG`
  (params (Layer :type "LayerData Object Reference") (Name :type String) (split :type Boolean))
  (locals (Pixels1 :type "Array of Color Structure") (Pixels2 :type "Array of Color Structure") (CurBlock :type String))
  (bind _returnvalue (`LayerData.getChunkCount` Layer))
  (bind _pixels1 (`local.Pixels1`))
  (bind _name (`local.Name`))
  (bind _pixels2 (`local.Pixels2`))
  (bind _pixels1_2 (`local.Pixels1`))
  (bind _returnvalue_2 (- (* _returnvalue 16) 1))
  (bind _returnvalue_3 (* (`LayerData.getChunkCount` (`local.Layer`)) 16))
  (`/Engine/EditorBlueprintResources/StandardMacros.IsValid` Layer
    (:`Is Valid`
      (if (not split)
        (`LayerData.connectLayers` Layer))
      (for _index (range (+ _returnvalue_2 1))
        (for _index_2 (range (+ _returnvalue_2 1))
          (bind _returnvalue_4 (`|GetDataTableRow` "/Game/Data/Voxel/DT_DataBlocks.DT_DataBlocks" (`KismetStringLibrary.Conv_StringToName` (`KismetStringLibrary.Conv_NameToString` (`LayerData.getBlock` Layer (- (- (* _returnvalue 16) 1) _index_2) _index false))))
            (:`then`
              (`KismetArrayLibrary.Array_Add` _pixels1 (`.Color_8_D4A5B4A34F6F531BCBEAF8B1F34499AB` (break `/Game/Data/Voxel/S_AssetBlock` _returnvalue_4))))
            (:`RowNotFound`
              (`KismetArrayLibrary.Array_Add` _pixels1 (make `Color` 0))))))
      (if split
        (for _index_3 (range (+ _returnvalue_2 1))
          (for _index_4 (range (+ _returnvalue_2 1))
            (bind _returnvalue_5 (`|GetDataTableRow` "/Game/Data/Voxel/DT_DataBlocks.DT_DataBlocks" (`KismetStringLibrary.Conv_StringToName` (`KismetStringLibrary.Conv_NameToString` (`LayerData.getBlock` Layer (- (- (* _returnvalue 16) 1) _index_4) _index_3 true))))
              (:`then`
                (`KismetArrayLibrary.Array_Add` _pixels2 (`.Color_8_D4A5B4A34F6F531BCBEAF8B1F34499AB` (break `/Game/Data/Voxel/S_AssetBlock` _returnvalue_5))))
              (:`RowNotFound`
                (`KismetArrayLibrary.Array_Add` _pixels2 (make `Color` 0))))))
        (`KismetArrayLibrary.Array_Reverse` (`local.Pixels1`))
        (`KismetArrayLibrary.Array_Reverse` (`local.Pixels2`))
        (`SaveLoad.SaveArrayToPNG` (`local.Pixels1`) (`KismetStringLibrary.Concat_StrStr` _name "_0") _returnvalue_3)
        (`SaveLoad.SaveArrayToPNG` (`local.Pixels2`) (`KismetStringLibrary.Concat_StrStr` _name "_1") _returnvalue_3)
        (else
          (`KismetArrayLibrary.Array_Reverse` _pixels1_2)
          (`SaveLoad.SaveArrayToPNG` _pixels1_2 (`local.Name`) _returnvalue_3))))
    (:`Is Not Valid`
      (`KismetSystemLibrary.PrintString` "ERROR: Layer is not valid"))))

(fn `SetBlock`
  (params (X :type Integer) (Y :type Integer) (Z :type Boolean) (Block :type Name))
  (bind _block (`local.Block`))
  (bind _z (`local.Z`))
  (bind _returnvalue (mod (`local.X`) 16))
  (bind _returnvalue_2 (`CoordsConvert.BlockToChunk` (`KismetMathLibrary.Conv_IntToDouble` X) (`KismetMathLibrary.Conv_IntToDouble` Y) Z))
  (bind _returnvalue_3 (mod (`local.Y`) 16))
  (bind _returnvalue_4 (`KismetMathLibrary.FTrunc` (.x _returnvalue_2)))
  (bind _returnvalue_5 (`KismetMathLibrary.FTrunc` (.y _returnvalue_2)))
  (bind _chunk (`self.FindChunk` _returnvalue_2))
  (`/Engine/EditorBlueprintResources/StandardMacros.IsValid` _chunk
    (:`Is Valid`
      (`/Game/Blueprints/Blocks/_OLD/BP_ChunkMesh.SetBlock` _chunk _returnvalue _returnvalue_3 _z _block))
    (:`Is Not Valid`
      (bind _chunk_2 (`self.CreateChunks` _returnvalue_4 _returnvalue_4 _returnvalue_5 _returnvalue_5))
      (bind _result (`BlueprintSetLibrary.Set_ToArray` _chunk_2))
      (bind _output (`|GetArrayItem` _result))
      (`/Engine/EditorBlueprintResources/StandardMacros.IsValid` _output
        (:`Is Valid`
          (`/Game/Blueprints/Blocks/_OLD/BP_ChunkMesh.SetBlock` _output _returnvalue _returnvalue_3 _z _block))))))

(fn `UserConstructionScript`)