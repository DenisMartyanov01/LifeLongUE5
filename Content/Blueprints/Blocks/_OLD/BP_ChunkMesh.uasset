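; Older chunk mesh Blueprint that renders a 16x16, two-layer grid of blocks as instanced static meshes at 100-unit spacing.
; CreateBlock skips air and adds instances to ISM block components stored in a map by block name.
; GetBlock linearly searches instance transforms to find a cell, which DeleteBlock and SetBlock use for edits.
; SetChunk destroys all components and rebuilds every cell from the given chunk.
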(fn `CreateBlock`
  (params (X :type Integer) (Y :type Integer) (Z :type Boolean) (Block :type Name))
  (returns (Index :type Integer))
  (locals (pos :type "Transform Structure"))
  (bind _pos (`local.pos`))
  (bind _block (`local.Block`))
  (bind (_value _returnvalue) (`BlueprintMapLibrary.Map_Find` (`self.data`)))
  (bind (_returnvalue_location _returnvalue_rotation _returnvalue_scale) (`KismetMathLibrary.BreakTransform` (`KismetMathLibrary.MakeTransform` (`KismetMathLibrary.MakeVector` (`KismetMathLibrary.Conv_IntToDouble` (* Y 100)) (`KismetMathLibrary.Conv_IntToDouble` (* X 100)) (`KismetMathLibrary.Conv_IntToDouble` (* (`KismetMathLibrary.Conv_BoolToInt` Z) 100))))))
  (if (!= Block "air")
    (set `local.pos` (`KismetMathLibrary.MakeTransform` _returnvalue_location _returnvalue_rotation _returnvalue_scale))
    (if _returnvalue
      (bind _returnvalue_2 (`InstancedStaticMeshComponent.AddInstance` _value _pos false))
      (return _returnvalue_2)
      (else
        (bind _returnvalue_3 (`AddComponent|NODE_AddISM_Block-0`))
        (`/Game/Blueprints/Blocks/_OLD/ISM_Block.SetBlock` _returnvalue_3 _block)
        (`BlueprintMapLibrary.Map_Add` (`self.data`) (`KismetStringLibrary.Conv_NameToString` _block) _returnvalue_3)
        (bind _returnvalue_4 (`InstancedStaticMeshComponent.AddInstance` _returnvalue_3 _pos false))
        (return _returnvalue_4)))))

(fn `DeleteBlock`
  (params (X :type Integer) (Y :type Integer) (Z :type Boolean))
  (bind (_block _index) (`self.GetBlock` X Y Z))
  (bind (_value _returnvalue) (`BlueprintMapLibrary.Map_Find` (`self.data`) _block))
  (if (and _returnvalue (!= _index -1))
    (`InstancedStaticMeshComponent.RemoveInstance` _value _index)
    (return)))

(fn `DeleteChunk`
  (bind _data (`self.data`))
  (bind _keys (`BlueprintMapLibrary.Map_Keys` _data))
  (for _array_element _keys
    (`ActorComponent.K2_DestroyComponent` (`BlueprintMapLibrary.Map_Find` _data _array_element)))
  (`BlueprintMapLibrary.Map_Clear` _data))

(fn `GetBlock`
  (params (X :type Integer) (Y :type Integer) (Z :type Boolean))
  (returns (Block :type String) (Index :type Integer))
  (bind _keys (`BlueprintMapLibrary.Map_Keys` (`self.data`)))
  (for _array_element _keys
    (bind _value (`BlueprintMapLibrary.Map_Find` (`self.data`) _array_element))
    (for _index (range (`InstancedStaticMeshComponent.GetInstanceCount` _value))
      (bind _outinstancetransform (`InstancedStaticMeshComponent.GetInstanceTransform` _value _index false))
      (if (and (and (== (/ (.x (.location _outinstancetransform)) 100.0) (`local.X`)) (== (/ (.y (.location _outinstancetransform)) 100.0) (`local.Y`))) (== (!= (.z (.location _outinstancetransform)) 0.0) (`local.Z`)))
        (return _array_element _index))))
  (return "" -1))

(fn `SetBlock`
  (params (x :type Integer) (y :type Integer) (z :type Boolean) (Asset :type Name))
  (`self.DeleteBlock` x y z)
  (`self.CreateBlock` x y z Asset))

(fn `SetChunk`
  (params (Chunk :type "ChunkData Object Reference"))
  (`self.DeleteChunk`)
  (for _index (range 2)
    (for _index_2 (range 16)
      (for _index_3 (range 16)
        (bind _returnvalue (!= _index 0))
        (`self.CreateBlock` _index_2 _index_3 _returnvalue (`ChunkData.getBlock` Chunk _index_2 _index_3 _returnvalue))))))

(fn `UserConstructionScript`
  (`|GenericCreateObject` "/Script/Test.ChunkData"))