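; BP_Barell is a placeable barrel block that acts as an interactable storage container.
; BeginPlay and Set read its DT_Chests row to resize and clear BPItemStorage and pick the UI texture, with Set also taking the sounds.
; Interacting creates a UW_RectangleChest widget over that storage and shows it through the initiator's AC_UIManager.
; Closing or breaking interaction switches the storage UI visibility and plays a random sound, as opening does.
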(event `self.OnInteract`
  (params (Insignator :type "Actor Object Reference") (Location :type "Vector Structure") (Normal :type "Vector Structure"))
  (bind _output_get (set `self.Initiator` Insignator))
  (bind _returnvalue (`self.GetComponentByClass` _output_get "/Game/UI/AC_UIManager.AC_UIManager_C"))
  (`/Engine/EditorBlueprintResources/StandardMacros.IsValid` _returnvalue
    (:`Is Valid`
      (bind _ascharacter (cast `Character` _output_get))
      (bind _asplayer_controller (cast `PlayerController` (`Pawn.GetController` _ascharacter)))
      (bind _returnvalue_2 (`|CreateWidget` "/Game/UI/Storage/UW_RectangleChest.UW_RectangleChest_C" _asplayer_controller (`self.BP_ItemStorage`) (-0.0 -0.0)))
      (`UserWidget.SetPositionInViewport` _returnvalue_2 (600.0 80.0) true)
      (bind _output_get_2 (set `self.Widget` _returnvalue_2))
      (`Image.SetBrushFromTexture` (`/Game/UI/Storage/UW_RectangleChest.Texture` _returnvalue_2) (`self.Texture`) false)
      (`/Game/UI/AC_UIManager.AddTempUI` _returnvalue _output_get_2 0)
      (`/Game/UI/AC_UIManager.UpdateUI` _returnvalue "NewEnumerator6")
      (add `/Game/UI/UW_DragableWidget.BtnCloseTriggered` _returnvalue_2 (delegate `Close`))
      (`GameplayStatics.PlaySoundAtLocation` (`KismetArrayLibrary.Array_Random` (`self.Sounds`)) (`self.K2_GetActorLocation`) (struct) 1.0 1.0 0.0 null null null null))))

(event `Close`
  (`/Game/Blueprints/Entities/BPI_Interact.OnBreakInteraction`)
  (message `/Game/Blueprints/Entities/BPI_Interact.OnBreakInteraction` (stale `self.OnInteract` Insignator)))

(event `self.OnBreakInteraction`
  (bind _returnvalue (`self.GetComponentByClass` (`self.Initiator`) "/Game/UI/AC_UIManager.AC_UIManager_C"))
  (`|ExecutionSequence`
    (:`then_0`
      (`/Engine/EditorBlueprintResources/StandardMacros.IsValid` _returnvalue
        (:`Is Valid`
          (`/Game/UI/AC_UIManager.SwitchStorageUIVisibility` _returnvalue (`self.Widget`)))))
    (:`then_1`
      (`GameplayStatics.PlaySoundAtLocation` (`KismetArrayLibrary.Array_Random` (`self.Sounds`)) (`self.K2_GetActorLocation`) (struct) 1.0 1.0 0.0 null null null null))))

(event `self.ReceiveBeginPlay`
  (bind _bp_itemstorage (`self.BP_ItemStorage`))
  (bind _returnvalue (`|GetDataTableRow` "/Game/Data/Placeable/_DT_Chests._DT_Chests" (`self.name`))
    (:`then`
      (`KismetArrayLibrary.Array_Resize` (`/Game/Blueprints/StorageSystem/AC_ItemStorage.Items` _bp_itemstorage) (break `/Game/Data/Placeable/S_DataChest` _returnvalue))
      (`/Game/Blueprints/StorageSystem/AC_BaseStorage.Clear` _bp_itemstorage)
      (set `self.Texture` (`.UITexture_8_6EFBFB244524ED478D81308C9B206254` (break `/Game/Data/Placeable/S_DataChest` _returnvalue))))))

(fn `Set`
  (params (Data :type "/Game/Data/Placeable/S_DataPlaceable Structure") (index :type Integer))
  (bind _bp_itemstorage (`self.BP_ItemStorage`))
  (`parent.Set` Data index)
  (bind _returnvalue (`|GetDataTableRow` "/Game/Data/Placeable/_DT_Chests._DT_Chests" (`.name_28_89D610374A8CB6D76F6FA9A74D3086DB` (break `/Game/Data/Placeable/S_DataPlaceable` Data)))
    (:`then`
      (`KismetArrayLibrary.Array_Resize` (`/Game/Blueprints/StorageSystem/AC_ItemStorage.Items` _bp_itemstorage) (break `/Game/Data/Placeable/S_DataChest` _returnvalue))
      (`/Game/Blueprints/StorageSystem/AC_BaseStorage.Clear` _bp_itemstorage)
      (set `self.Texture` (`.UITexture_8_6EFBFB244524ED478D81308C9B206254` (break `/Game/Data/Placeable/S_DataChest` _returnvalue)))
      (set `self.Sounds` (`.Sounds_23_D1C56A8F426021BD6C4929A1D2EC438F` (break `/Game/Data/Placeable/S_DataChest` _returnvalue))))))

(fn `UserConstructionScript`
  (set `/Game/Blueprints/StorageSystem/AC_BaseStorage.Type` "NewEnumerator6" (`self.BP_ItemStorage`)))