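; BP_Chest is a placeable chest block that players interact with to open an item storage UI.
; Set applies a dynamic textured material, then pulls mesh, capacity, UI texture, sounds and animation names from the DT_Chests row.
; Interaction plays an open animation and shows a horizontal chest widget through the initiator's AC_UIManager.
; Breaking interaction, also triggered by the close button, plays the close animation and toggles the UI, with separate first-time animations.
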(event `SERVER_Interact`)

(event `/Game/Blueprints/Entities/BPI_Interact.OnInteract`
  (params (Insignator :type "Actor Object Reference") (Location :type "Vector Structure") (Normal :type "Vector Structure"))
  (`/Game/Blueprints/Animations/AC_AnimationManager.PlayAnimation` (`self.AC_AnimChest`) (`KismetMathLibrary.SelectName` (`self.OpenAnimationFirstTime`) (`self.OpenAnimation`) (`self.first_time`)) "None" 0 1.0 false)
  (bind _output_get (set `self.Initiator` Insignator))
  (bind _returnvalue (`self.GetComponentByClass` _output_get "/Game/UI/AC_UIManager.AC_UIManager_C"))
  (`/Engine/EditorBlueprintResources/StandardMacros.IsValid` _returnvalue
    (:`Is Valid`
      (bind _ascharacter (cast `Character` _output_get))
      (bind _asplayer_controller (cast `PlayerController` (`Pawn.GetController` _ascharacter)))
      (bind _returnvalue_2 (`|CreateWidget` "/Game/UI/Storage/UW_HorizontalChest.UW_HorizontalChest_C" _asplayer_controller (`self.BP_ItemStorage`) (-0.0 -0.0)))
      (`UserWidget.SetPositionInViewport` _returnvalue_2 (600.0 80.0) true)
      (bind _output_get_2 (set `self.Widget` _returnvalue_2))
      (`Image.SetBrushFromTexture` (`/Game/UI/Storage/UW_HorizontalChest.Texture` _returnvalue_2) (`self.Texture`) false)
      (`/Game/UI/AC_UIManager.AddTempUI` _returnvalue _output_get_2 0)
      (`/Game/UI/AC_UIManager.UpdateUI` _returnvalue "NewEnumerator6")
      (add `/Game/UI/UW_DragableWidget.BtnCloseTriggered` _returnvalue_2 (delegate `Close`)))))

(event `Close`
  (`/Game/Blueprints/Entities/BPI_Interact.OnBreakInteraction`)
  (message `/Game/Blueprints/Entities/BPI_Interact.OnBreakInteraction` (stale `/Game/Blueprints/Entities/BPI_Interact.OnInteract` Insignator)))

(event `/Game/Blueprints/Entities/BPI_Interact.OnBreakInteraction`
  (bind _returnvalue (`self.GetComponentByClass` (`self.Initiator`) "/Game/UI/AC_UIManager.AC_UIManager_C"))
  (`|ExecutionSequence`
    (:`then_0`
      (`/Game/Blueprints/Animations/AC_AnimationManager.PlayAnimation` (`self.AC_AnimChest`) (`KismetMathLibrary.SelectName` (`self.CloseAnimationFirstTime`) (`self.CloseAnimation`) (`self.first_time`)) "None" 0 1.0 false)
      (set `self.first_time` false))
    (:`then_1`
      (`/Engine/EditorBlueprintResources/StandardMacros.IsValid` _returnvalue
        (:`Is Valid`
          (`/Game/UI/AC_UIManager.SwitchStorageUIVisibility` _returnvalue (`self.Widget`)))))))

(event `self.ReceiveBeginPlay`)

(fn `Set`
  (params (Data :type "/Game/Data/Placeable/S_DataPlaceable Structure") (index :type Integer))
  (bind (_name _mesh _attributes _material _class _drop _texture) (break `/Game/Data/Placeable/S_DataPlaceable` Data))
  (bind _bp_itemstorage (`self.BP_ItemStorage`))
  (`parent.Set` Data index)
  (bind _returnvalue (`KismetMaterialLibrary.CreateDynamicMaterialInstance` (`|GetArrayItem` _material (mod index (`KismetArrayLibrary.Array_Length` _material)))))
  (`MaterialInstanceDynamic.SetTextureParameterValue` _returnvalue "Texture" (`|GetArrayItem` _texture (mod index (`KismetArrayLibrary.Array_Length` _texture))))
  (`PrimitiveComponent.SetMaterial` (`self.SkeletalMesh_0`) 0 _returnvalue)
  (bind _returnvalue_2 (`|GetDataTableRow` "/Game/Data/Placeable/_DT_Chests._DT_Chests" _name)
    (:`then`
      (`KismetArrayLibrary.Array_Resize` (`/Game/Blueprints/StorageSystem/AC_ItemStorage.Items` _bp_itemstorage) (break `/Game/Data/Placeable/S_DataChest` _returnvalue_2))
      (`/Game/Blueprints/StorageSystem/AC_BaseStorage.Clear` _bp_itemstorage)
      (set `self.Texture` (`.UITexture_8_6EFBFB244524ED478D81308C9B206254` (break `/Game/Data/Placeable/S_DataChest` _returnvalue_2)))
      (set `SkeletalMeshComponent.SkeletalMeshAsset` (`.Mesh_9_84090D49440C12EF10D26A8B217D6D56` (break `/Game/Data/Placeable/S_DataChest` _returnvalue_2)) (`self.SkeletalMesh_0`))
      (set `self.OpenAnimation` (`.open_12_CB165E5441020DCC1A42E9B0C65697D8` (break `/Game/Data/Placeable/S_DataChest` _returnvalue_2)))
      (set `self.CloseAnimation` (`.close_14_02D62B81420787935884B192064448CC` (break `/Game/Data/Placeable/S_DataChest` _returnvalue_2)))
      (set `self.OpenAnimationFirstTime` (`.open1_16_331DEFE041D65069D10799BE64E59535` (break `/Game/Data/Placeable/S_DataChest` _returnvalue_2)))
      (set `self.CloseAnimationFirstTime` (`.close1_18_52B47C854A0AB4AE97C14488E358BFDA` (break `/Game/Data/Placeable/S_DataChest` _returnvalue_2)))
      (set `self.Sounds` (`.Sounds_23_D1C56A8F426021BD6C4929A1D2EC438F` (break `/Game/Data/Placeable/S_DataChest` _returnvalue_2))))))

(fn `UserConstructionScript`
  (`parent.UserConstructionScript`)
  (set `/Game/Blueprints/StorageSystem/AC_BaseStorage.Type` "NewEnumerator6" (`self.BP_ItemStorage`)))