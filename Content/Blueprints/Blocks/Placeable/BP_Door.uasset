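; BP_Door is a placeable, interactable door that swings open or closed.
; Opening turns the door 90 degrees in a direction chosen by the dot product of the actor's right vector and the direction to the interactor.
; Closing targets a world yaw of zero rather than a stored starting rotation.
; A timeline interpolates the rotation, then toggles the open state and calls OnBreakInteractionMessage on the interactor.
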(event `/Game/Blueprints/Entities/BPI_Interact.OnInteract`
  (params (Insignator :type "Actor Object Reference") (Location :type "Vector Structure") (Normal :type "Vector Structure"))
  (bind _door (`self.Door`))
  (bind _returnvalue (`SceneComponent.K2_GetComponentRotation` _door))
  (bind _yaw (.yaw _returnvalue))
  (bind _output_get (set `self.CurR` _returnvalue))
  (bind _output_get_2 (set `self.NeededR` (`KismetMathLibrary.MakeRotator` (.roll _returnvalue) (.pitch _returnvalue) (`KismetMathLibrary.SelectFloat` 0.0 (`KismetMathLibrary.SelectFloat` (+ _yaw 90.0) (+ _yaw -90.0) (<= (`KismetMathLibrary.Dot_VectorVector` (`KismetMathLibrary.GetDirectionUnitVector` (`self.K2_GetActorLocation`) (`self.K2_GetActorLocation` Insignator)) (`self.GetActorRightVector`)) 0.0)) (`self.is_opened`)))))
  (bind (_direction _newtrack_0) (`Timeline|Timeline` :!via `PlayFromStart`)
    (:`Update`
      (`SceneComponent.K2_SetWorldRotation` _door (`KismetMathLibrary.RLerp` _output_get _output_get_2 _newtrack_0) false false))
    (:`Finished`
      (set `self.is_opened` (not (`self.is_opened`)))
      (message `/Game/Blueprints/Entities/BPI_Interact.OnBreakInteraction` Insignator))))

(fn `UserConstructionScript`)