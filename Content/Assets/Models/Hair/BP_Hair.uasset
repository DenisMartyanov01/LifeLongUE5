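; BP_Hair is an actor that displays a hair or beard piece on a skeletal mesh.
; SetHair looks the name up in DT_Hair, falls back to DT_Beard, then applies that row's mesh and anim blueprint.
; It builds a dynamic instance of MI_Hair for slot 0, setting the row's texture and the supplied color.
; Visibility follows IsHidden, applied on BeginPlay and through its OnRep function.
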(event `SetHair`
  (params (Name :type Name) (Color :type "Color Structure"))
  (bind _skeletalmesh (`self.SkeletalMesh`))
  (bind _skeletalmesh_2 (`self.SkeletalMesh`))
  (bind _returnvalue (`|GetDataTableRow` "/Game/Data/BodyParts/DT_Hair.DT_Hair" Name)
    (:`then`
      (set `SkeletalMeshComponent.SkeletalMeshAsset` (`.Mesh_5_347B02E74B55E96B086FA0B874220EE3` (break `/Game/Data/BodyParts/S_Hair` _returnvalue)) _skeletalmesh_2)
      (`SkeletalMeshComponent.SetAnimInstanceClass` _skeletalmesh_2 (`.AnimBp_10_B5F16E734AE121B4ECC7FDAF8A3E8652` (break `/Game/Data/BodyParts/S_Hair` _returnvalue)))
      (bind _returnvalue_2 (`KismetMaterialLibrary.CreateDynamicMaterialInstance` "/Game/Assets/Materials/Emotions/MI_Hair.MI_Hair"))
      (`PrimitiveComponent.SetMaterial` (`self.SkeletalMesh`) 0 _returnvalue_2)
      (`MaterialInstanceDynamic.SetTextureParameterValue` _returnvalue_2 "Texture" (`.Texture_13_ABAD2002480F4EEFA01CED8E0659E83E` (break `/Game/Data/BodyParts/S_Hair` _returnvalue)))
      (`MaterialInstanceDynamic.SetVectorParameterValue` _returnvalue_2 "Color" (`KismetMathLibrary.Conv_ColorToLinearColor` Color)))
    (:`RowNotFound`
      (bind _returnvalue_3 (`|GetDataTableRow` "/Game/Data/BodyParts/DT_Beard.DT_Beard" Name)
        (:`then`
          (set `SkeletalMeshComponent.SkeletalMeshAsset` (`.Mesh_5_347B02E74B55E96B086FA0B874220EE3` (break `/Game/Data/BodyParts/S_Hair` _returnvalue_3)) _skeletalmesh)
          (`SkeletalMeshComponent.SetAnimInstanceClass` _skeletalmesh (`.AnimBp_10_B5F16E734AE121B4ECC7FDAF8A3E8652` (break `/Game/Data/BodyParts/S_Hair` _returnvalue_3)))
          (bind _returnvalue_4 (`KismetMaterialLibrary.CreateDynamicMaterialInstance` "/Game/Assets/Materials/Emotions/MI_Hair.MI_Hair"))
          (`PrimitiveComponent.SetMaterial` (`self.SkeletalMesh`) 0 _returnvalue_4)
          (`MaterialInstanceDynamic.SetTextureParameterValue` _returnvalue_4 "Texture" (`.Texture_13_ABAD2002480F4EEFA01CED8E0659E83E` (break `/Game/Data/BodyParts/S_Hair` _returnvalue_3)))
          (`MaterialInstanceDynamic.SetVectorParameterValue` _returnvalue_4 "Color" (`KismetMathLibrary.Conv_ColorToLinearColor` Color)))))))

(event `self.ReceiveBeginPlay`
  (`self.SetActorHiddenInGame` (`self.is_hidden`)))

(fn `OnRep_is_hidden`
  (`self.SetActorHiddenInGame` (`self.is_hidden`)))

(fn `UserConstructionScript`)